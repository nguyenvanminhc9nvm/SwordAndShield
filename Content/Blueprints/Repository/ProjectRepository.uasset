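; Data repository Blueprint serving weapon catalogs, character lookups and save games.
; Sword, axe and shield struct lists become Weapon_Obj objects through a shared converter, with a reverse converter back to structs.
; Character names map to character classes and per-character SaveGame classes, which are loaded from name-keyed slots or created when absent.
; Game settings load from a constant-named slot, and only this path saves a newly created object immediately.
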(fn ConvertListSwordtoObject
  (params (ListStructure :type Array%20of%20Weapon%20Structure%20Structures))
  (for _array_element ListStructure
    (bind _weaponobj (CallFunction|ConvertWeaponStructtoObject _array_element))
    (Utilities|Array|Add (LocalVariables|GetListWeapon) _weaponobj))
  (return (LocalVariables|GetListWeapon)))

(fn GetListSwords
  (bind _listobject (CallFunction|ConvertListSwordtoObject (Variables|Default|GetListSwords)))
  (return _listobject))

(fn GetListAxe
  (bind _listobject (CallFunction|ConvertListSwordtoObject (Variables|Default|GetListAxe)))
  (return _listobject))

(fn GetListShield
  (bind _listobject (CallFunction|ConvertListSwordtoObject (Variables|Default|GetListShield)))
  (return _listobject))

(fn GetCharacterDatabyName
  (params (NameCharacter :type String))
  (switch string NameCharacter
    (:Thunderstorm
      (return "/Game/Blueprints/GameSaver/SG_Player/SG_Thunderstorm.SG_Thunderstorm_C"))
    (:Blazeheart
      (return "/Game/Blueprints/GameSaver/SG_Player/SG_Blazeheart.SG_Blazeheart_C"))
    (:Frostbite
      (return "/Game/Blueprints/GameSaver/SG_Player/SG_Fostbite.SG_Fostbite_C"))
    (:Dawnbreaker
      (return "/Game/Blueprints/GameSaver/SG_Player/SG_Dawnbreaker.SG_Dawnbreaker_C"))
    (:Bloodfang
      (return "/Game/Blueprints/GameSaver/SG_Player/SG_Bloodfang.SG_Bloodfang_C"))
    (:Nightshade
      (return "/Game/Blueprints/GameSaver/SG_Player/SG_Nightshade.SG_Nightshade_C"))
    (:Ironclad
      (return "/Game/Blueprints/GameSaver/SG_Player/SG_Ironclad.SG_Ironclad_C"))
    (:Emberblade
      (return "/Game/Blueprints/GameSaver/SG_Player/SG_Emberblade.SG_Emberblade_C"))
    (:Darkthorn
      (return "/Game/Blueprints/GameSaver/SG_Player/SG_Darkthorn.SG_Darkthorn_C"))
    (:Drake
      (return "/Game/Blueprints/GameSaver/SG_Player/SG_Drake.SG_Drake_C"))
    (:Lunarstrike
      (return "/Game/Blueprints/GameSaver/SG_Player/SG_Lunarstrike.SG_Lunarstrike_C"))
    (:Voidwalker
      (return "/Game/Blueprints/GameSaver/SG_Player/SG_Voidwalker.SG_Voidwalker_C"))
    (:KingAuthur
      (return "/Game/Blueprints/GameSaver/SG_Player/SG_KingAuthur.SG_KingAuthur_C"))))

(fn GetorInitbyCharacterName
  (params (CharacterName :type String))
  (bind _sg_gamedata_player (CallFunction|GetCharacterDatabyName CharacterName))
  (return (CallFunction|GetorCreateSaveGame CharacterName _sg_gamedata_player)))

(fn GetGameSetting
  (bind _returnvalue (Game|ConstructObjectfromClass "/Game/Blueprints/Constant/BP_Constant.BP_Constant_C"))
  (bind _returnvalue_2 (SaveGame|DoesSaveGameExist (Variables|/Game/Blueprints/Constant/BP_Constant.BP_Constant_C|GetSG_SettingGame _returnvalue) (Variables|Default|GetSaveGameIndex)))
  (if _returnvalue_2
    (bind _returnvalue_3 (SaveGame|LoadGamefromSlot (Variables|/Game/Blueprints/Constant/BP_Constant.BP_Constant_C|GetSG_SettingGame _returnvalue) (Variables|Default|GetSaveGameIndex)))
    (bind _assg_setting_game (Utilities|Casting|CastToSG_SettingGame _returnvalue_3))
    (return _assg_setting_game)
    (else
      (bind _returnvalue_4 (SaveGame|CreateSaveGameObject "/Game/Blueprints/GameSaver/SG_SettingGame.SG_SettingGame_C"))
      (SaveGame|SaveGametoSlot _returnvalue_4 (Variables|/Game/Blueprints/Constant/BP_Constant.BP_Constant_C|GetSG_SettingGame _returnvalue) (Variables|Default|GetSaveGameIndex))
      (return _returnvalue_4))))

(fn ConvertWeaponStructtoObject
  (params (WeaponStruct :type Weapon%20Structure%20Structure))
  (bind (_name _texture _staticmesh _credit _licensing _price _weapontype _increasedamage _decreasespeed _armorial _magicskill _star _description) (Utilities|Struct|BreakWeapon_Structure WeaponStruct))
  (bind _returnvalue (Game|ConstructObjectfromClass "/Game/Blueprints/Structure/Weapon_Obj.Weapon_Obj_C"))
  (Utilities|FlowControl|Sequence
    (:then_0
      (Variables|/Game/Blueprints/Structure/Weapon_Obj.Weapon_Obj_C|SetTexture _returnvalue _texture))
    (:then_1
      (Variables|/Game/Blueprints/Structure/Weapon_Obj.Weapon_Obj_C|SetStaticMesh _returnvalue _staticmesh))
    (:then_2
      (Variables|/Game/Blueprints/Structure/Weapon_Obj.Weapon_Obj_C|SetName _returnvalue _name))
    (:then_3
      (Variables|/Game/Blueprints/Structure/Weapon_Obj.Weapon_Obj_C|SetCredit _returnvalue _credit))
    (:then_4
      (Variables|/Game/Blueprints/Structure/Weapon_Obj.Weapon_Obj_C|SetLicense _returnvalue _licensing))
    (:then_5
      (Variables|/Game/Blueprints/Structure/Weapon_Obj.Weapon_Obj_C|SetPrice _returnvalue _price))
    (:then_6
      (Variables|/Game/Blueprints/Structure/Weapon_Obj.Weapon_Obj_C|SetWeaponType _returnvalue _weapontype))
    (:then_7
      (Variables|/Game/Blueprints/Structure/Weapon_Obj.Weapon_Obj_C|SetIncreaseDamage _returnvalue _increasedamage))
    (:then_8
      (Variables|/Game/Blueprints/Structure/Weapon_Obj.Weapon_Obj_C|SetDecreaseSpeed _returnvalue _decreasespeed))
    (:then_9
      (Variables|/Game/Blueprints/Structure/Weapon_Obj.Weapon_Obj_C|SetArmorial _returnvalue _armorial))
    (:then_10
      (Variables|/Game/Blueprints/Structure/Weapon_Obj.Weapon_Obj_C|SetMagicSkill _returnvalue _magicskill))
    (:then_11
      (Variables|/Game/Blueprints/Structure/Weapon_Obj.Weapon_Obj_C|SetStar _returnvalue _star))
    (:then_12
      (Variables|/Game/Blueprints/Structure/Weapon_Obj.Weapon_Obj_C|SetDescription _returnvalue _description))
    (:then_20
      (return _returnvalue))))

(fn GetorCreateSaveGame
  (params (CharacterName :type String) (SG_Class :type SG%20Game%20Data%20Player%20Class%20Reference))
  (bind _returnvalue (SaveGame|DoesSaveGameExist CharacterName (Variables|Default|GetSaveGameIndex)))
  (if _returnvalue
    (bind _returnvalue_2 (SaveGame|LoadGamefromSlot CharacterName (Variables|Default|GetSaveGameIndex)))
    (bind _assg_game_data_player (Utilities|Casting|CastToSG_GameData_Player _returnvalue_2))
    (return _assg_game_data_player)
    (else
      (bind _returnvalue_3 (SaveGame|CreateSaveGameObject SG_Class))
      (return _returnvalue_3))))

(fn GetCharacterClassbyName
  (params (String :type String))
  (switch string String
    (:Thunderstorm
      (return "/Game/Blueprints/Characters/PlayerCharacter/Thunderstorm.Thunderstorm_C"))
    (:Blazeheart
      (return "/Game/Blueprints/Characters/PlayerCharacter/Blazeheart.Blazeheart_C"))
    (:Frostbite
      (return "/Game/Blueprints/Characters/PlayerCharacter/Fostbite.Fostbite_C"))
    (:Dawnbreaker
      (return "/Game/Blueprints/Characters/EnemyCharacter/Dawnbreaker.Dawnbreaker_C"))
    (:Bloodfang
      (return "/Game/Blueprints/Characters/EnemyCharacter/Bloodfang.Bloodfang_C"))
    (:Nightshade
      (return "/Game/Blueprints/Characters/EnemyCharacter/Nightshade.Nightshade_C"))
    (:Ironclad
      (return "/Game/Blueprints/Characters/EnemyCharacter/Ironclad.Ironclad_C"))
    (:Emberblade
      (return "/Game/Blueprints/Characters/EnemyCharacter/Emberblade.Emberblade_C"))
    (:Darkthorn
      (return "/Game/Blueprints/Characters/EnemyCharacter/Darkthon.Darkthon_C"))
    (:Drake
      (return "/Game/Blueprints/Characters/EnemyCharacter/Drake.Drake_C"))
    (:Lunarstrike
      (return "/Game/Blueprints/Characters/EnemyCharacter/Lunarstrike.Lunarstrike_C"))
    (:Voidwalker
      (return "/Game/Blueprints/Characters/EnemyCharacter/VoidWalker.VoidWalker_C"))
    (:KingAuthur
      (return "/Game/Blueprints/Characters/EnemyCharacter/KingAuthur.KingAuthur_C"))))

(fn ConvertWeaponObjtoWeaponStructure
  (params (WeaponObj :type Weapon%20Obj%20Object%20Reference))
  (return (Utilities|Struct|MakeWeapon_Structure (Variables|/Game/Blueprints/Structure/Weapon_Obj.Weapon_Obj_C|GetName WeaponObj) (Variables|/Game/Blueprints/Structure/Weapon_Obj.Weapon_Obj_C|GetTexture WeaponObj) (Variables|/Game/Blueprints/Structure/Weapon_Obj.Weapon_Obj_C|GetStaticMesh WeaponObj) (Variables|/Game/Blueprints/Structure/Weapon_Obj.Weapon_Obj_C|GetCredit WeaponObj) (Variables|/Game/Blueprints/Structure/Weapon_Obj.Weapon_Obj_C|GetLicense WeaponObj) (Variables|/Game/Blueprints/Structure/Weapon_Obj.Weapon_Obj_C|GetPrice WeaponObj) (Variables|/Game/Blueprints/Structure/Weapon_Obj.Weapon_Obj_C|GetWeaponType WeaponObj) (Variables|/Game/Blueprints/Structure/Weapon_Obj.Weapon_Obj_C|GetIncreaseDamage WeaponObj) (Variables|/Game/Blueprints/Structure/Weapon_Obj.Weapon_Obj_C|GetDecreaseSpeed WeaponObj) (Variables|/Game/Blueprints/Structure/Weapon_Obj.Weapon_Obj_C|GetArmorial WeaponObj) (Variables|/Game/Blueprints/Structure/Weapon_Obj.Weapon_Obj_C|GetMagicSkill WeaponObj) (Variables|/Game/Blueprints/Structure/Weapon_Obj.Weapon_Obj_C|GetStar WeaponObj) (Variables|/Game/Blueprints/Structure/Weapon_Obj.Weapon_Obj_C|GetDescription WeaponObj))))