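; Base melee-and-magic character for players, enemies and bots, handling input, movement, weapon equipping, healing and target lock.
; Health, stamina, attack, hit and sound components process combat, with stamina gating attacks and heals and updates broadcast outward.
; Stats and gear load from SG_GameData by PlayerType; milestone functions save player character and weapon level-ups.
; Attach socket names derive from mesh names, and Tick turns control rotation toward the sphere-traced target.
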(event Custom|Welcome
  ;[1 0 0.02818] Base Event
  ;;[1 1 1] Welcome
)

(event Custom|PerformSpecialAbilities
  ;[1 0 0.02818] Base Event
  ;;[1 1 1] Perform special abilities
)

(event EventBeginPlay
  ;[1 0 0.02818] Base Event
  ;;[1 1 1] Init Enhanced Input
  (Data|SetDataPlayer)
  (bind _asbp_play_player_controller (Utilities|Casting|CastToBP_Play_PlayerController (Pawn|GetController)))
  (bind _output_get (Variables|Default|SetPlay_PlayerController _asbp_play_player_controller))
  (Variables|/Game/Blueprints/Core/PlayerController/BP_Play_PlayerController.BP_Play_PlayerController_C|SetCameraSpringArm _output_get 0)
  (Input|AddMappingContext (PlayerController|LocalPlayerSubsystems|GetEnhancedInputLocalPlayerSubsystem _output_get) "/Game/Input/IMC_Player.IMC_Player" 0 "(bIgnoreAllPressedKeysUntilRelease=True,bForceImmediately=False,bNotifyUserSettings=False)")
  (Game|ConstructObjectfromClass "/Game/Blueprints/Constant/BP_Language.BP_Language_C"))

(event EventTick
  (params (DeltaSeconds :type Float%20%28single-precision%29))
  ;[1 0 0.02818] Base Event
  ;;[1 1 1] HandleAutoRun
  (if (Variables|CharacterProperties|GetIsAutoRun)
    (Movement|MoveActorForward)
    (Default|DecreaseStaminawhenMoving (Variables|Default|GetBP_StaminaComponent))
    (elif (Variables|CharacterProperties|GetIsMoving)
      _
      (else
        (Default|RecoverStaminawhenIdle (Variables|Default|GetBP_StaminaComponent)))))
  (Data|CallCharacterUpdate)
  (bind _enemytarget (Variables|TargetLock|GetEnemyTarget)
    (:then
      (Pawn|SetControlRotation (Pawn|GetController) (Math|Rotator|FindLookatRotation (Transformation|GetActorLocation) (Transformation|GetActorLocation _enemytarget))))
    (:else)))

(event Custom|IAutoRun_1
  ;[1 0.8444 0] Enhanced Input
  ;;[1 1 1] Auto Run
  (Variables|CharacterProperties|SetIsAutoRun true))

(event Input|EnhancedActionEvents|EnhancedInputActionIA_Move
  (params (ActionValue :type Vector%202D%20Structure) (ElapsedSeconds :type Float%20%28double-precision%29) (TriggeredSeconds :type Float%20%28double-precision%29) (InputAction :type Input%20Action%20Object%20Reference :default "/Game/Input/Action/IA_Move.IA_Move"))
  (bind _returnvalue (Pawn|GetControlRotation :!class /Script/Engine.Pawn))
  ;[1 0.8444 0] Enhanced Input
  ;;[1 1 1] IA_Move
  (:Triggered
    (Variables|CharacterProperties|SetIsMoving true)
    (Variables|CharacterProperties|SetIsAutoRun false)
    (Pawn|Input|AddMovementInput (Math|Vector|GetRightVector (Math|Rotator|MakeRotator 0.0 0.0 (.yaw _returnvalue))) (.y ActionValue) false)
    (Pawn|Input|AddMovementInput (Math|Vector|GetForwardVector (Math|Rotator|MakeRotator 0.0 0.0 (.yaw _returnvalue))) (.x ActionValue) false)
    (Default|DecreaseStamina (Variables|Default|GetBP_StaminaComponent) 0.1)
    (Class|Actor|MakeNoise 1.0 self (Transformation|GetActorLocation) 0.0 "None"))
  (:Completed
    (Variables|CharacterProperties|SetIsMoving false)))

(event Input|EnhancedActionEvents|EnhancedInputActionIA_Look
  (params (ActionValue :type Vector%202D%20Structure) (ElapsedSeconds :type Float%20%28double-precision%29) (TriggeredSeconds :type Float%20%28double-precision%29) (InputAction :type Input%20Action%20Object%20Reference :default "/Game/Input/Action/IA_Look.IA_Look"))
  ;[1 0.8444 0] Enhanced Input
  ;;[1 1 1] IA_Look
  (Pawn|Input|AddControllerYawInput (.x ActionValue))
  (Pawn|Input|AddControllerPitchInput (.y ActionValue)))

(event Game|Damage|EventPointDamage
  (params (Damage :type Float%20%28single-precision%29) (DamageType :type Damage%20Type%20Object%20Reference) (HitLocation :type Vector :default "0, 0, 0") (HitNormal :type Vector :default "0, 0, 0") (HitComponent :type Primitive%20Component%20Object%20Reference) (BoneName :type Name :default "None") (ShotFromDirection :type Vector :default "0, 0, 0") (InstigatedBy :type Controller%20Object%20Reference) (DamageCauser :type Actor%20Object%20Reference) (HitInfo :type Hit%20Result%20Structure%20%28by%20ref%29))
  ;[0 1 0.005929] Character Event
  ;;[1 1 1] Handle Point Damage
  (CallFunction|ISetTargetLock1)
  (Equipment|CanculatorPushActorBack ShotFromDirection 1.5e+02)
  (Default|PlaySoundbyAction (Variables|Default|GetBP_SoundComponent) DamageCauser false)
  (Default|HandleHitImpact (Variables|Default|GetBP_HitComponent) ShotFromDirection HitLocation Damage)
  (Default|DecreaseHealth (Variables|Default|GetBP_HealthComponent) Damage)
  (Default|DecreaseStamina (Variables|Default|GetBP_StaminaComponent) Damage)
  (Data|CallCharacterUpdate (Utilities|String|Append "-" (Utilities|String|ToString(Integer) (Math|Float|Truncate Damage)) " "))
  (bind _stillalive (Default|DoesStillAlive (Variables|Default|GetBP_HealthComponent)))
  (if (not _stillalive)
    (Default|CallOnDeath)
    (CallFunction|IHandleEndAttack)
    (Animation|PlayAnimMontage (Variables|/Game/Blueprints/Component/BP_HealthComponent.BP_HealthComponent_C|GetAM_Death (Variables|Default|GetBP_HealthComponent)) 1.0 "None")
    (Actor|SetLifeSpan 1.5)
    (Variables|/Game/Blueprints/Component/BP_AttackComponent.BP_AttackComponent_C|SetCombatState (Variables|Default|GetBP_AttackComponent) "NewEnumerator1")
    (Collision|SetCollisionEnabled (Variables|Character|GetMesh) "NoCollision")
    (Collision|SetCollisionEnabled (Variables|Collision|GetCapsuleComponent) "NoCollision")
    (Components|Movement|StopMovementImmediately (Variables|Character|GetCharacterMovement))))

(event Custom|TriggerJump
  ;[1 1 1] Trigger Jump
  (Character|UnCrouch)
  (if (Character|CanJump)
    (Character|Jump)))

(event Custom|TriggerCrouch
  ;[1 1 1] TriggerCrouch
  (if (Variables|Default|GetbIsCrouched)
    (Character|UnCrouch)
    (else
      (Character|Crouch))))

(event Custom|IDraw
  ;[1 1 1] Draw
  (Default|PlaySoundwhenDraworSheath (Variables|Default|GetBP_SoundComponent) true)
  (Transformation|AttachComponentToComponent (Variables|Default|GetPrimaryWeapon) (Variables|Character|GetMesh) (.PrimaryWeaponDraw (Equipment|GetCorrectPrimaryWeaponSocketName)) "SnapToTarget" "SnapToTarget" "SnapToTarget" true)
  (Transformation|AttachComponentToComponent (Variables|Default|GetSecondaryWeapon) (Variables|Character|GetMesh) (.SecondaryWeaponDraw (Equipment|GetCorrectSecondaryWeaponSocketName)) "SnapToTarget" "SnapToTarget" "SnapToTarget" true)
  (Variables|Equipment|SetIsEquip true))

(event Custom|IShealth
  ;[1 1 1] Sheath
  (Default|PlaySoundwhenDraworSheath (Variables|Default|GetBP_SoundComponent) false)
  (Transformation|AttachComponentToComponent (Variables|Default|GetPrimaryWeapon) (Variables|Character|GetMesh) (.PrimaryWeaponSheath (Equipment|GetCorrectPrimaryWeaponSocketName)) "SnapToTarget" "SnapToTarget" "SnapToTarget" true)
  (Transformation|AttachComponentToComponent (Variables|Default|GetSecondaryWeapon) (Variables|Character|GetMesh) (.SecondaryWeaponSheath (Equipment|GetCorrectSecondaryWeaponSocketName)) "SnapToTarget" "SnapToTarget" "SnapToTarget" true)
  (Variables|Equipment|SetIsEquip false))

(event Custom|TriggerEquip
  ;[1 1 1] Trigger Equip
  (if (Variables|Equipment|GetIsEquip)
    (Animation|PlayAnimMontage (Equipment|GetCorrectAnimSheathbyEquipType) 1.0 "None")
    (else
      (Animation|PlayAnimMontage (Equipment|GetCorrectAnimDrawbyEquipType) 1.0 "None"))))

(event Custom|TriggerChangeEquipType
  (params (EquipType :type E_EquipType%20Enum :default "NewEnumerator0"))
  ;[1 1 1] Change Equip Type
  (Variables|Equipment|SetEquipType EquipType))

(event Custom|TriggerPowerUp
  ;[1 1 1] Trigger Heal
  (Default|PlaySoundwhenPowerUp (Variables|Default|GetBP_SoundComponent))
  (Animation|PlayAnimMontage (Variables|Montage|GetAM_PowerUp) 1.0 "None")
  (if (>= (Default|GetStaminaPercent (Variables|Default|GetBP_StaminaComponent)) 0.15)
    (Default|RecoverFull (Variables|Default|GetBP_HealthComponent))
    (Default|RecoverFull (Variables|Default|GetBP_StaminaComponent))
    ;;[1 1 1] Reset Damage Taken
    (Variables|/Game/Blueprints/Component/BP_HitComponent.BP_HitComponent_C|SetTotalDamageTaken (Variables|Default|GetBP_HitComponent) 0.0)
    (else
      (bind _returnvalue (Game|ConstructObjectfromClass "/Game/Blueprints/Constant/BP_Language.BP_Language_C"))
      (Data|CallCharacterUpdate (Default|GetTextNotEnoughStamina _returnvalue)))))

(event Custom|ISpawnMagicBeam
  (params (ProjectileClass :type Actor%20Class%20Reference) (Speed :type Float%20%28double-precision%29) (NewRelativeScale :type Vector))
  (bind _self self)
  ;[0 0.9178 1] Interface Event
  ;;[1 1 1] Spawn Magic Beam
  (Default|PlaySoundwhenSpawnMagic (Variables|Default|GetBP_SoundComponent))
  (bind _asbp_base_magic (Utilities|Casting|CastToBP_Base_MagicClass ProjectileClass))
  (bind _returnvalue (Game|SpawnActorfromClass _asbp_base_magic (Transformation|GetWorldTransform (Variables|Default|GetShotPoint)) "AlwaysSpawn" "MultiplyWithRoot" _self Speed 0.0 0 _self))
  (Variables|/Game/Blueprints/Actors/Projectile/BP_Base_Magic.BP_Base_Magic_C|SetDamage _returnvalue (/ (Variables|/Game/Blueprints/Component/BP_AttackComponent.BP_AttackComponent_C|GetAttackDamage (Variables|Default|GetBP_AttackComponent)) 2.0))
  (Transformation|SetActorRelativeScale3D _returnvalue NewRelativeScale))

(event Custom|IHandleTickDoDamage
  (params (Side :type E_SideAttack%20Enum :default "NewEnumerator0"))
  ;[0 0.9178 1] Interface Event
  ;;[1 1 1] Handle Tick Do Damage
  (Default|HandleTickDoDamage (Variables|Default|GetBP_AttackComponent) Side))

(event Custom|IHandleBeginDoDamage
  ;[0 0.9178 1] Interface Event
  ;;[1 1 1] Handle Begin Do Damage
  (Default|HandleBeginDoDamage (Variables|Default|GetBP_AttackComponent)))

(event Custom|IHandleEndAttack
  ;[0 0.9178 1] Interface Event
  ;;[1 1 1] Handle End Attack
  (Default|HandleEndAttack (Variables|Default|GetBP_AttackComponent))
  (Default|DecreaseStaminawhenAttack (Variables|Default|GetBP_StaminaComponent))
  (Data|CallCharacterUpdate))

(event Custom|IResetCombat
  ;[0 0.9178 1] Interface Event
  ;;[1 1 1] Handle Reset Combat
  (Default|HandleEndAttack (Variables|Default|GetBP_AttackComponent))
  (Variables|/Game/Blueprints/Component/BP_AttackComponent.BP_AttackComponent_C|SetCombatState (Variables|Default|GetBP_AttackComponent) "NewEnumerator0")
  (CallFunction|IResetWeaponStatus))

(event Custom|IContinueAttack
  (params (Action :type E_Action%20Enum :default "NewEnumerator0"))
  ;[0 0.9178 1] Interface Event
  ;;[1 1 1] Handle Continue Attack
  (Default|ContinueAttack (Variables|Default|GetBP_AttackComponent) Action))

(event Custom|IRequestAttack
  (params (Action :type E_Action%20Enum :default "NewEnumerator0"))
  ;[0 0.9178 1] Interface Event
  ;;[1 1 1] Handle Request Attack
  (if (Utilities|Enum|Equal(Enum) (Variables|/Game/Blueprints/Component/BP_AttackComponent.BP_AttackComponent_C|GetCombatState (Variables|Default|GetBP_AttackComponent)) "NewEnumerator0")
    (if (>= (Default|GetStaminaPercent (Variables|Default|GetBP_StaminaComponent)) 0.15)
      (bind _length (Default|RequestAttack (Variables|Default|GetBP_AttackComponent) Action))
      (Utilities|FlowControl|Delay _length)
      (else
        (bind _returnvalue (Game|ConstructObjectfromClass "/Game/Blueprints/Constant/BP_Language.BP_Language_C"))
        (Data|CallCharacterUpdate (Default|GetTextNotEnoughStamina _returnvalue))))))

(event Custom|IResetWeaponStatus
  ;[0 0.9178 1] Interface Event
  ;;[1 1 1] Reset Weapon Status
  (Variables|/Game/Blueprints/Component/BP_SoundComponent.BP_SoundComponent_C|SetShouldPlaySound (Variables|Default|GetBP_SoundComponent) false)
  (if (Variables|Equipment|GetIsEquip)
    (CallFunction|IDraw)
    (else
      (CallFunction|IShealth)))
  (Variables|/Game/Blueprints/Component/BP_SoundComponent.BP_SoundComponent_C|SetShouldPlaySound (Variables|Default|GetBP_SoundComponent) true))

(event Custom|ICancelTargetLock
  ;[0 0.9178 1] Interface Event
  ;;[1 1 1] Handle End Power Up
  (Variables|TargetLock|SetIsTargetLock false))

(event Custom|ISetTargetLock_1
  (bind _returnvalue (Transformation|GetActorLocation))
  ;[0 0.9178 1] Interface Event
  ;;[1 1 1] Set Target Lock
  (if (not (Variables|TargetLock|GetIsTargetLock))
    (Variables|TargetLock|SetIsTargetLock true)
    (bind (_outhit _returnvalue_2) (Collision|SphereTraceForObjects _returnvalue (+ (* (Math|Vector|GetForwardVector (Transformation|GetWorldRotation (Variables|Default|GetCamera))) 5e+02) _returnvalue) 2e+03 (Utilities|Array|MakeArray "ObjectTypeQuery8") false 0 "ForOneFrame"))
    (if _returnvalue_2
      (bind _asbase_character (Utilities|Casting|CastToBase_Character (.HitActor (Collision|BreakHitResult _outhit))))
      (bind _output_get (Variables|TargetLock|SetEnemyTarget _asbase_character))
      (Default|CallOnDetectTargetLock _output_get))))

(fn ConstructionScript)

(fn MoveActorForward
  (Pawn|Input|AddMovementInput (Transformation|GetActorForwardVector) 1.0 false))

(fn SetDataPlayer
  (switch Utilities|FlowControl|Switch|SwitchonE_PlayerType (Variables|Equipment|GetPlayerType)
    (:NewEnumerator0
      (bind _playerdata1 (Data|LoadPlayerData))
      (return _playerdata1))
    (:NewEnumerator1
      _)
    (:NewEnumerator2
      _))
  (bind _outputpin (Data|LoadEnemyData))
  (return _outputpin))

(fn GetCorrectPrimaryWeaponSocketName
  (bind _staticmesh (Variables|/Script/Engine.StaticMeshComponent|GetStaticMesh (Variables|Default|GetPrimaryWeapon))
    (:then
      (return (Utilities|String|StringToName (Utilities|String|Append "Primary" (Utilities|GetDisplayName _staticmesh) "Draw")) (Utilities|String|StringToName (Utilities|String|Append "Primary" (Utilities|GetDisplayName _staticmesh) "Sheath"))))
    (:else
      (return "None" "None"))))

(fn GetCorrectSecondaryWeaponSocketName
  (bind _staticmesh (Variables|/Script/Engine.StaticMeshComponent|GetStaticMesh (Variables|Default|GetSecondaryWeapon))
    (:then
      (return (Utilities|String|StringToName (Utilities|String|Append "Secondary" (Utilities|GetObjectName _staticmesh) "Draw")) (Utilities|String|StringToName (Utilities|String|Append "Secondary" (Utilities|GetObjectName _staticmesh) "Sheath"))))
    (:else)))

(fn GetCorrectShieldSocketName
  (bind _staticmesh (Variables|/Script/Engine.StaticMeshComponent|GetStaticMesh (Variables|Default|GetShield))
    (:then
      (return (Utilities|String|StringToName (Utilities|GetObjectName _staticmesh))))
    (:else
      (return "None"))))

(fn SetEquipPrimaryWeaponPreview
  (params (Weapon :type BP%20ST%20Weapon%20Structure))
  (bind _returnvalue (Game|ConstructObjectfromClass "/Game/Blueprints/Utils/BP_StaticMeshExtension.BP_StaticMeshExtension_C"))
  (bind _staticmesh (Default|GetStaticMeshbyName _returnvalue (.WeaponName (Utilities|Struct|BreakBP_ST_Weapon Weapon))))
  (Components|StaticMesh|SetStaticMesh (Variables|Default|GetPrimaryWeapon) _staticmesh)
  (Transformation|AttachComponentToComponent (Variables|Default|GetPrimaryWeapon) (Variables|Character|GetMesh) (.PrimaryWeaponDraw (Equipment|GetCorrectPrimaryWeaponSocketName)) "KeepRelative" "KeepRelative" "KeepRelative" true))

(fn SetEquipShieldWeaponPreview
  (params (Weapon :type BP%20ST%20Weapon%20Structure))
  (bind _returnvalue (Game|ConstructObjectfromClass "/Game/Blueprints/Utils/BP_StaticMeshExtension.BP_StaticMeshExtension_C"))
  (Components|StaticMesh|SetStaticMesh (Variables|Default|GetShield) (Default|GetShieldStaticMeshbyName _returnvalue (.WeaponName (Utilities|Struct|BreakBP_ST_Weapon Weapon))))
  (Transformation|AttachComponentToComponent (Variables|Default|GetShield) (Variables|Character|GetMesh) (Equipment|GetCorrectShieldSocketName) "KeepRelative" "KeepRelative" "KeepRelative" true))

(fn GetCorrectAnimSheathbyEquipType
  (bind _equiptype (Variables|Equipment|GetEquipType))
  (Development|PrintString (Utilities|String|EnumtoString _equiptype))
  (switch Utilities|FlowControl|Switch|SwitchonE_EquipType _equiptype
    (:NewEnumerator0
      (return (Variables|Montage|GetAM_Sheath_TypeAxe)))
    (:NewEnumerator1
      (return (Variables|Montage|GetAM_Sheath_TypeSword)))))

(fn GetCorrectAnimDrawbyEquipType
  (switch Utilities|FlowControl|Switch|SwitchonE_EquipType (Variables|Equipment|GetEquipType)
    (:NewEnumerator0
      (return (Variables|Montage|GetAM_Draw_TypeAxe)))
    (:NewEnumerator1
      (return (Variables|Montage|GetAM_Draw_TypeSword)))))

(fn CanculatorPushActorBack
  (params (HitDirection :type Vector) (Damage :type Float%20%28double-precision%29))
  (bind _returnvalue (Transformation|GetActorLocation))
  (bind _returnvalue_2 (Transformation|GetActorLocation))
  (bind _returnvalue_3 (Transformation|GetActorLocation))
  (bind _returnvalue_4 (Transformation|GetActorTransform))
  (bind _returnvalue_5 (- HitDirection _returnvalue_3))
  (bind _returnvalue_6 (Math|Transform|InverseTransformDirection _returnvalue_4 _returnvalue_5))
  (Development|PrintString (Utilities|String|Append "X: " (Utilities|String|ToString(Float) (.x _returnvalue_6)) " Y: " (Utilities|String|ToString(Float) (.y _returnvalue_6))))
  (Utilities|FlowControl|Sequence
    (:then_0
      (if (> (.x _returnvalue_6) 0.0)
        (Transformation|SetActorRelativeLocation (Math|Vector|MakeVector (- (.x _returnvalue) Damage) (.y _returnvalue) (.z _returnvalue)) true)
        (else
          (Transformation|SetActorRelativeLocation (Math|Vector|MakeVector (+ (.x _returnvalue_2) Damage) (.y _returnvalue_2) (.z _returnvalue_2)) true))))))

(fn CallCharacterUpdate
  (params (Message :type String))
  (Default|CallOnCharacterUpdate (Default|GetStaminaPercent (Variables|Default|GetBP_StaminaComponent)) (Default|GetHealthPercent (Variables|Default|GetBP_HealthComponent)) Message))

(fn LoadPlayerData
  ;[1 1 1] Find Charcater Active
  (bind _returnvalue (Game|ConstructObjectfromClass "/Game/Blueprints/Data/SaveGame/SG_GameData.SG_GameData_C"))
  (bind _sg_gamedata (Default|LoadLocalGameData _returnvalue))
  (Development|PrintString (.email (Variables|/Game/Blueprints/Data/SaveGame/SG_GameData.SG_GameData_C|GetUser _sg_gamedata)))
  (for _array_element (.characterpurchased (Variables|/Game/Blueprints/Data/SaveGame/SG_GameData.SG_GameData_C|GetUser _sg_gamedata))
    (if (.IsActive (Utilities|Struct|BreakBP_ST_PlayerCharacter _array_element))
      (LocalVariables|SetPlayerData _array_element)))
  (Data|LoadCharacterData (LocalVariables|GetPlayerData))
  (return (LocalVariables|GetPlayerData)))

(fn LoadEnemyData
  (bind _returnvalue (Game|ConstructObjectfromClass "/Game/Blueprints/Data/SaveGame/SG_GameData.SG_GameData_C"))
  (bind _sg_gamedata (Default|LoadLocalGameData _returnvalue))
  (bind _player (Default|GetEnemyDatabyName _sg_gamedata (Variables|CharacterProperties|GetCharacterName)))
  (Data|LoadCharacterData _player)
  (return _player))

(fn LoadCharacterData
  (params (PlayerCharacter :type BP%20ST%20Player%20Character%20Structure))
  ;[1 1 1] Set Data
  (bind _output_get (Variables|Data|SetCurrentPlayerCharacter PlayerCharacter))
  (Variables|CharacterProperties|SetCharacterName (.CharacterName (Utilities|Struct|BreakBP_ST_PlayerCharacter _output_get)))
  (Default|InitHealth (Variables|Default|GetBP_HealthComponent) (.Health (Utilities|Struct|BreakBP_ST_PlayerCharacter _output_get)))
  (Default|InitStamina (Variables|Default|GetBP_StaminaComponent) (.StaminaReduceWhenAttackPercent (Utilities|Struct|BreakBP_ST_PlayerCharacter _output_get)) (.Stamina (Utilities|Struct|BreakBP_ST_PlayerCharacter _output_get)))
  (Data|SetPrimaryWeapon (.ActivateSword (Utilities|Struct|BreakBP_ST_PlayerCharacter _output_get)) (.ActivateAxe (Utilities|Struct|BreakBP_ST_PlayerCharacter _output_get)))
  (Data|SetShieldEquip (.ActivateShield (Utilities|Struct|BreakBP_ST_PlayerCharacter _output_get)))
  (if (Variables|Equipment|GetIsEquip)
    (CallFunction|IDraw)
    (else
      (CallFunction|IShealth))))

(fn SetEquipWeaponPreview
  (params (Weapon :type BP%20ST%20Weapon%20Structure))
  (if (Utilities|String|Contains (.WeaponName (Utilities|Struct|BreakBP_ST_Weapon Weapon)) "shield")
    (Equipment|SetEquipShieldWeaponPreview Weapon)
    (else
      (Equipment|SetEquipPrimaryWeaponPreview Weapon)))
  (CallFunction|TriggerEquip))

(fn CalculatorUpLevelCharacter
  (bind _currentplayercharacter (Variables|Data|GetCurrentPlayerCharacter))
  (bind _bp_healthcomponent (Variables|Default|GetBP_HealthComponent))
  (bind _returnvalue (- (.maxlevel _currentplayercharacter) (.level _currentplayercharacter)))
  (bind _returnvalue_2 (- (.maxhealth _currentplayercharacter) (.health _currentplayercharacter)))
  (bind _returnvalue_3 (Math|Conversions|ToFloat(Integer) _returnvalue))
  (bind _returnvalue_4 (/ _returnvalue_2 _returnvalue_3))
  (bind _returnvalue_5 (+ (.health _currentplayercharacter) _returnvalue_4))
  (switch Utilities|FlowControl|Switch|SwitchonE_PlayerType (Variables|Equipment|GetPlayerType)
    (:NewEnumerator0
      (LocalVariables|SetCurrentHealthBeforeUpdate (Variables|/Game/Blueprints/Component/BP_HealthComponent.BP_HealthComponent_C|GetCurrentHealth _bp_healthcomponent))
      (LocalVariables|SetCurrentStaminaBeforeUpdate (Variables|/Game/Blueprints/Component/BP_StaminaComponent.BP_StaminaComponent_C|GetCurrentStamina (Variables|Default|GetBP_StaminaComponent)))
      (if (and (> (Variables|/Game/Blueprints/Component/BP_HealthComponent.BP_HealthComponent_C|GetCurrentHealth _bp_healthcomponent) (Variables|Data|GetMilestoneUpCharacterLevel)) (> (Variables|/Game/Blueprints/Component/BP_StaminaComponent.BP_StaminaComponent_C|GetCurrentStamina (Variables|Default|GetBP_StaminaComponent)) (Variables|Data|GetMilestoneUpCharacterLevel)))
        (Variables|Data|SetMilestoneUpCharacterLevel (/ (Variables|/Game/Blueprints/Component/BP_HealthComponent.BP_HealthComponent_C|GetMaxHealth _bp_healthcomponent) 2.0)))
      (if (> (Variables|/Game/Blueprints/Component/BP_HitComponent.BP_HitComponent_C|GetTotalDamageTaken (Variables|Default|GetBP_HitComponent)) (Variables|Data|GetMilestoneUpCharacterLevel))
        (Variables|Data|SetMilestoneUpCharacterLevel (* (Variables|Data|GetMilestoneUpCharacterLevel) 5.0))
        (bind _returnvalue_6 (Game|ConstructObjectfromClass "/Game/Blueprints/Data/SaveGame/SG_GameData.SG_GameData_C"))
        (Default|UpdatePlayerData _returnvalue_6 (Utilities|Struct|MakeBP_ST_PlayerCharacter (.charactername _currentplayercharacter) (+ (.level _currentplayercharacter) 1) _returnvalue_5 (.staminareducewhenattackpercent _currentplayercharacter) _returnvalue_5 (.activatesword _currentplayercharacter) (.activateaxe _currentplayercharacter) (.activateshield _currentplayercharacter) (.credit _currentplayercharacter) (.license _currentplayercharacter) (.matchanalytics _currentplayercharacter) (.isactive _currentplayercharacter) (.maxlevel _currentplayercharacter) (.maxhealth _currentplayercharacter) (.maxstamina _currentplayercharacter)))
        (Data|SetDataPlayer)
        (Variables|/Game/Blueprints/Component/BP_HealthComponent.BP_HealthComponent_C|SetCurrentHealth (Variables|Default|GetBP_HealthComponent) (LocalVariables|GetCurrentHealthBeforeUpdate))
        (Variables|/Game/Blueprints/Component/BP_StaminaComponent.BP_StaminaComponent_C|SetCurrentStamina (Variables|Default|GetBP_StaminaComponent) (LocalVariables|GetCurrentStaminaBeforeUpdate))))))

(fn CalculatorUpLevelWeapon
  (bind _bp_attackcomponent (Variables|Default|GetBP_AttackComponent))
  (bind _bp_attackcomponent_2 (Variables|Default|GetBP_AttackComponent))
  (bind _swordequip (Variables|Data|GetSwordEquip))
  (bind _axeequip (Variables|Data|GetAxeEquip))
  (bind _returnvalue (+ (.level _swordequip) 1))
  (bind _totaldamagedealt (Variables|/Game/Blueprints/Component/BP_AttackComponent.BP_AttackComponent_C|GetTotalDamageDealt _bp_attackcomponent))
  (bind _attackdamage (Variables|/Game/Blueprints/Component/BP_AttackComponent.BP_AttackComponent_C|GetAttackDamage _bp_attackcomponent_2))
  (switch Utilities|FlowControl|Switch|SwitchonE_PlayerType (Variables|Equipment|GetPlayerType)
    (:NewEnumerator0
      (LocalVariables|SetCurrentHealthBeforeUpdate (Variables|/Game/Blueprints/Component/BP_HealthComponent.BP_HealthComponent_C|GetCurrentHealth (Variables|Default|GetBP_HealthComponent)))
      (LocalVariables|SetCurrentStaminaBeforeUpdate (Variables|/Game/Blueprints/Component/BP_StaminaComponent.BP_StaminaComponent_C|GetCurrentStamina (Variables|Default|GetBP_StaminaComponent)))
      (if (> _attackdamage (Variables|Data|GetMilestoneUpWeaponLevel))
        (Variables|Data|SetMilestoneUpWeaponLevel (* (+ _attackdamage (Variables|Data|GetMilestoneUpWeaponLevel)) 3.0)))
      (Development|PrintString (Utilities|String|Append "UpLevelWeapon: " "  TotalDamageDealt:  " (Utilities|String|ToString(Float) _totaldamagedealt) " Milestone:  " (Utilities|String|ToString(Float) (Variables|Data|GetMilestoneUpWeaponLevel)) " AttackDamage:  " (Utilities|String|ToString(Float) _attackdamage)))
      (if (> _totaldamagedealt (Variables|Data|GetMilestoneUpWeaponLevel))
        (bind _output_get (Variables|Data|SetMilestoneUpWeaponLevel (* (Variables|Data|GetMilestoneUpWeaponLevel) 3.0)))
        (Development|PrintString (Utilities|String|Append "UpLevelWeapon: newMaxMilestone:  " (Utilities|String|ToString(Float) _output_get)) true true "(R=1.000000,G=0.000000,B=0.006920,A=1.000000)")
        (bind _returnvalue_2 (Game|ConstructObjectfromClass "/Game/Blueprints/Data/SaveGame/SG_GameData.SG_GameData_C"))
        (if (Utilities|Array|IsEmpty (.weaponname _swordequip))
          (Default|UpdateWeaponData _returnvalue_2 (Utilities|Struct|MakeBP_ST_Weapon (.weaponname _axeequip) (.credit _axeequip) (.license _axeequip) (* (.damage _axeequip) (+ (/ 0.0 (Math|Conversions|ToFloat(Integer) (.levelmax _axeequip))) 1.0)) (+ (.level _axeequip) 1) (.isactive _axeequip) (.levelmax _axeequip)))
          (else
            (Default|UpdateWeaponData _returnvalue_2 (Utilities|Struct|MakeBP_ST_Weapon (.weaponname _swordequip) (.credit _swordequip) (.license _swordequip) (+ (.damage _swordequip) (/ (- (.maxdamage _swordequip) (.damage _swordequip)) (Math|Conversions|ToFloat(Integer) (- (.levelmax _swordequip) _returnvalue)))) _returnvalue (.isactive _swordequip) (.levelmax _swordequip) (.maxdamage _swordequip)))))
        (Data|SetDataPlayer)
        (Variables|/Game/Blueprints/Component/BP_HealthComponent.BP_HealthComponent_C|SetCurrentHealth (Variables|Default|GetBP_HealthComponent) (LocalVariables|GetCurrentHealthBeforeUpdate))
        (Variables|/Game/Blueprints/Component/BP_StaminaComponent.BP_StaminaComponent_C|SetCurrentStamina (Variables|Default|GetBP_StaminaComponent) (LocalVariables|GetCurrentStaminaBeforeUpdate))))))

(fn SetPrimaryWeapon
  (params (SwordActive :type BP%20ST%20Weapon%20Structure) (AxeActive :type BP%20ST%20Weapon%20Structure))
  (bind (_weaponname _credit _license _damage) (Utilities|Struct|BreakBP_ST_Weapon SwordActive))
  (if (Utilities|Array|IsEmpty _weaponname)
    (Data|SetAxeEquip AxeActive)
    (else
      (Variables|Data|SetSwordEquip SwordActive)
      (bind _returnvalue (Game|ConstructObjectfromClass "/Game/Blueprints/Utils/BP_StaticMeshExtension.BP_StaticMeshExtension_C"))
      (Components|StaticMesh|SetStaticMesh (Variables|Default|GetPrimaryWeapon) (Default|GetSwordStaticMeshbyName _returnvalue _weaponname))
      (Variables|/Game/Blueprints/Component/BP_AttackComponent.BP_AttackComponent_C|SetAttackDamage (Variables|Default|GetBP_AttackComponent) _damage))))

(fn SetAxeEquip
  (params (Weapon :type BP%20ST%20Weapon%20Structure))
  (bind (_weaponname _credit _license _damage) (Utilities|Struct|BreakBP_ST_Weapon Weapon))
  (if (not (Utilities|Array|IsEmpty _weaponname))
    (Variables|Data|SetAxeEquip Weapon)
    (bind _returnvalue (Game|ConstructObjectfromClass "/Game/Blueprints/Utils/BP_StaticMeshExtension.BP_StaticMeshExtension_C"))
    (Components|StaticMesh|SetStaticMesh (Variables|Default|GetPrimaryWeapon) (Default|GetAxeStaticMeshbyName _returnvalue _weaponname))
    (Variables|/Game/Blueprints/Component/BP_AttackComponent.BP_AttackComponent_C|SetAttackDamage (Variables|Default|GetBP_AttackComponent) _damage)))

(fn SetShieldEquip
  (params (Weapon :type BP%20ST%20Weapon%20Structure))
  (bind _weaponname (Utilities|Struct|BreakBP_ST_Weapon Weapon))
  (if (not (Utilities|Array|IsEmpty _weaponname))
    (bind _returnvalue (Game|ConstructObjectfromClass "/Game/Blueprints/Utils/BP_StaticMeshExtension.BP_StaticMeshExtension_C"))
    (Components|StaticMesh|SetStaticMesh (Variables|Default|GetShield) (Default|GetShieldStaticMeshbyName _returnvalue _weaponname))
    (Transformation|AttachComponentToComponent (Variables|Default|GetShield) (Variables|Character|GetMesh) (Equipment|GetCorrectShieldSocketName) "SnapToTarget" "SnapToTarget" "SnapToTarget" true)))