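; Intro level column actor that displays a randomly chosen character at the position of its Plane component.
; RespawnCharacter destroys the previously spawned actor, then spawns a random class from ListActor with a fixed rotation and stores it for the next swap.
; BeginPlay triggers the first spawn, then plays the Intro_download 2D sound after a short delay.
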(event Custom|RespawnCharacter
  (Utilities|IsValid (Variables|Default|GetOldCharacter)
    (:Is%20Valid
      (Actor|DestroyActor (Variables|Default|GetOldCharacter)))
    (:Is%20Not%20Valid
      _))
  (bind _returnvalue (Game|SpawnActorfromClass (.OutItem (Utilities|Array|Random (Variables|Default|GetListActor))) (Math|Transform|MakeTransform (Transformation|GetWorldLocation (Variables|Default|GetPlane)) "0.000000,90.000000,0.000000" "1.000000,1.000000,1.000000") "Undefined" "MultiplyWithRoot" 0 0))
  (Variables|Default|SetOldCharacter _returnvalue))

(event EventBeginPlay
  (CallFunction|RespawnCharacter)
  (Utilities|FlowControl|Delay 0.2)
  (Audio|PlaySound2D "/Game/Assets/Sound/Intro/intro_download.intro_download" 1.0 1.0 0.0 0 0))

(event EventTick
  (params (DeltaSeconds :type Float%20%28single-precision%29)))

(fn ConstructionScript)