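; String utility Blueprint that formats timestamps and looks up player character descriptions.
; FormatTimestamp converts a Unix timestamp into an hours, minutes and seconds string, substituting dashes when all three are zero.
; GetDescPlayerByName constructs a BP_Language object on each call and switches on the character name to return the description text for Thunderstorm or Blazeheart.
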(fn FormatTimestamp
  (params (timestamp :type Integer64))
  (bind _returnvalue (Class|KismetMathLibrary|FromUnixTimestamp timestamp))
  (bind _returnvalue_2 (Class|KismetMathLibrary|GetHour _returnvalue))
  (bind _returnvalue_3 (Class|KismetMathLibrary|GetMinute _returnvalue))
  (bind _returnvalue_4 (Class|KismetMathLibrary|GetSecond _returnvalue))
  (if (Math|Boolean|ANDBoolean (== _returnvalue_2 0) (== _returnvalue_3 0) (== _returnvalue_4 0))
    (return (Utilities|String|Append "--" "h:" "--" "m:" "--" "s"))
    (else
      (return (Utilities|String|Append (Utilities|String|ToString(Integer) _returnvalue_2) "h:" (Utilities|String|ToString(Integer) _returnvalue_3) "m:" (Utilities|String|ToString(Integer) _returnvalue_4) "s")))))

(fn GetDescPlayerbyName
  (params (CharacterName :type E_CharacterName%20Enum :default "NewEnumerator0"))
  (bind _returnvalue (Game|ConstructObjectfromClass "/Game/Blueprints/Constant/BP_Language.BP_Language_C"))
  (switch Utilities|FlowControl|Switch|SwitchonE_CharacterName CharacterName
    (:NewEnumerator17
      (return (Default|GetTextDescThunderstorm _returnvalue)))
    (:NewEnumerator18
      (return (Default|GetTextDescBlazeheart _returnvalue)))))