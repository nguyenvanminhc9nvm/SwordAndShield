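; BP_TextureExtensions is a utility that maps display names of weapons, avatars and characters to their textures.
; GetTextureByName checks the name for "Sword" or "Axe" and forwards it to that category's lookup, sending every other name to the shield lookup.
; Each lookup is a hard-coded switch on the name.
; Avatars and character thumbnails have separate lookups, and several character names share one thumbnail, such as Nightshade with Grimstone.
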(fn GetSwordTexturebyName
  (params (Selection :type String))
  (switch string Selection
    (:AbyssalSword
      (return "/Game/Assets/Image/WeaponThum/Axe/Abyssal_Sword.Abyssal_Sword"))
    (:Radiant%20Sword
      (return "/Game/Assets/Image/WeaponThum/Sword/Radiant_Sword.Radiant_Sword"))
    (:Eclipse%20Sword
      (return "/Game/Assets/Image/WeaponThum/Sword/Eclipse_Sword.Eclipse_Sword"))
    (:Warcry%20Sword
      (return "/Game/Assets/Image/WeaponThum/Sword/Warcry_Sword.Warcry_Sword"))
    (:Tempest%20Sword
      (return "/Game/Assets/Image/WeaponThum/Sword/Tempest_Sword.Tempest_Sword"))
    (:Sunblade%20Sword
      (return "/Game/Assets/Image/WeaponThum/Sword/Sunblade_Sword.Sunblade_Sword"))
    (:Stormrage%20Sword
      (return "/Game/Assets/Image/WeaponThum/Sword/Stormrage_Sword.Stormrage_Sword"))
    (:Mystic%20Sword
      (return "/Game/Assets/Image/WeaponThum/Sword/Mystic_Sword.Mystic_Sword"))
    (:Blackfire%20Sword
      (return "/Game/Assets/Image/WeaponThum/Axe/Blackfire_Sword.Blackfire_Sword"))
    (:Grim%20Reaper%20Sword
      (return "/Game/Assets/Image/WeaponThum/Sword/Grim_Reaper_Sword.Grim_Reaper_Sword"))
    (:Silverlight%20Sword
      (return "/Game/Assets/Image/WeaponThum/Sword/Silverlight_Sword.Silverlight_Sword"))
    (:Ice%20Sword
      (return "/Game/Assets/Image/WeaponThum/Sword/Ice_Sword.Ice_Sword"))
    (:Aurora%20Sword
      (return "/Game/Assets/Image/WeaponThum/Axe/Aurora_Sword.Aurora_Sword"))
    (:Dragonheart%20Sword
      (return "/Game/Assets/Image/WeaponThum/Axe/Dragonheart_Sword.Dragonheart_Sword"))
    (:Shadowbane%20Sword
      (return "/Game/Assets/Image/WeaponThum/Sword/Shadowbane_Sword.Shadowbane_Sword"))
    (:Vortex%20Sword
      (return "/Game/Assets/Image/WeaponThum/Sword/Vortex_Sword.Vortex_Sword"))
    (:Thundercry%20Sword
      (return "/Game/Assets/Image/WeaponThum/Sword/Thundercry_Sword.Thundercry_Sword"))
    (:Seraphim%20Sword
      (return "/Game/Assets/Image/WeaponThum/Sword/Seraphim_Sword.Seraphim_Sword"))
    (:Magic%20Sword
      (return "/Game/Assets/Image/WeaponThum/Sword/Magic_Sword.Magic_Sword"))
    (:ThunderstormSword
      (return "/Game/Assets/Image/WeaponThum/Sword/ThunderstormSword.ThunderstormSword"))
    (:FostbiteSword
      (return "/Game/Assets/Image/WeaponThum/Sword/Fostbite_Sword.Fostbite_Sword"))))

(fn GetAxeTexturebyName
  (params (Selection :type String))
  (switch string Selection
    (:Bloodiron%20Axe
      (return "/Game/Assets/Image/WeaponThum/Axe/Bloodiron_Axe.Bloodiron_Axe"))
    (:Sunflare%20Axe
      (return "/Game/Assets/Image/WeaponThum/Axe/Sunflare_Axe.Sunflare_Axe"))
    (:Blackfire%20Axe
      (return "/Game/Assets/Image/WeaponThum/Axe/Blackfire_Axe.Blackfire_Axe"))
    (:Nightshard%20Axe
      (return "/Game/Assets/Image/WeaponThum/Axe/Nightshard_Axe.Nightshard_Axe"))
    (:Froststeel%20Axe
      (return "/Game/Assets/Image/WeaponThum/Axe/Froststeel_Axe.Froststeel_Axe"))
    (:Voidblade%20Axe
      (return "/Game/Assets/Image/WeaponThum/Axe/Voidblade_Axe.Voidblade_Axe"))
    (:Thunderclaw%20Axe
      (return "/Game/Assets/Image/WeaponThum/Axe/Thunderclaw_Axe.Thunderclaw_Axe"))
    (:Shadowthorn%20Axe
      (return "/Game/Assets/Image/WeaponThum/Axe/Shadowthorn_Axe.Shadowthorn_Axe"))
    (:Hellforged%20Axe
      (return "/Game/Assets/Image/WeaponThum/Axe/Hellforged_Axe.Hellforged_Axe"))
    (:Ironheart%20Axe
      (return "/Game/Assets/Image/WeaponThum/Axe/Ironheart_Axe.Ironheart_Axe"))
    (:Icebreaker%20Axe
      (return "/Game/Assets/Image/WeaponThum/Axe/Icebreaker_Axe.Icebreaker_Axe"))
    (:Duskstrike%20Axe
      (return "/Game/Assets/Image/WeaponThum/Axe/Duskstrike_Axe.Duskstrike_Axe"))
    (:Emberforge%20Axe
      (return "/Game/Assets/Image/WeaponThum/Axe/Emberforge_Axe.Emberforge_Axe"))
    (:Stormwrath%20Axe
      (return "/Game/Assets/Image/WeaponThum/Axe/Stormwrath_Axe.Stormwrath_Axe"))
    (:Soulrender%20Axe
      (return "/Game/Assets/Image/WeaponThum/Axe/Soulrender_Axe.Soulrender_Axe"))
    (:Frost%20Axe
      (return "/Game/Assets/Image/WeaponThum/Axe/Frostbite_Axe.Frostbite_Axe"))
    (:Doomcrusher%20Axe
      (return "/Game/Assets/Image/WeaponThum/Axe/Doomcrusher_Axe.Doomcrusher_Axe"))
    (:Grimfury%20Axe
      (return "/Game/Assets/Image/WeaponThum/Axe/Grimfury_Axe.Grimfury_Axe"))
    (:Dragonbone%20Axe
      (return "/Game/Assets/Image/WeaponThum/Axe/Dragonbone_Axe.Dragonbone_Axe"))
    (:Phoenixflame%20Axe
      (return "/Game/Assets/Image/WeaponThum/Axe/Phoenixflame_Axe.Phoenixflame_Axe"))
    (:BlazeheartAxe
      (return "/Game/Assets/Image/WeaponThum/Axe/BlazeheartAxe.BlazeheartAxe"))))

(fn GetShieldTexturebyName
  (params (Selection :type String))
  (switch string Selection
    (:Nightbane%20Shield
      (return "/Game/Assets/Image/WeaponThum/Shield/Nightbane_Shield.Nightbane_Shield"))
    (:Ironfist%20Shield
      (return "/Game/Assets/Image/WeaponThum/Shield/Ironfist_Shield.Ironfist_Shield"))
    (:Earthshaker%20Shield
      (return "/Game/Assets/Image/WeaponThum/Shield/Earthshaker_Shield.Earthshaker_Shield"))
    (:Emberguard%20Shield
      (return "/Game/Assets/Image/WeaponThum/Shield/Emberguard_Shield.Emberguard_Shield"))
    (:Sunburst%20Shield
      (return "/Game/Assets/Image/WeaponThum/Shield/Sunburst_Shield.Sunburst_Shield"))
    (:Thunderclap%20Shield
      (return "/Game/Assets/Image/WeaponThum/Shield/Thunderclap_Shield.Thunderclap_Shield"))
    (:Bloodthorn%20Shield
      (return "/Game/Assets/Image/WeaponThum/Shield/Bloodthorn_Shield.Bloodthorn_Shield"))
    (:Mystic%20Shield
      (return "/Game/Assets/Image/WeaponThum/Shield/Mystic_Shield.Mystic_Shield"))
    (:Windwhisper%20Shield
      (return "/Game/Assets/Image/WeaponThum/Shield/Windwhisper_Shield.Windwhisper_Shield"))
    (:Frostveil%20Shield
      (return "/Game/Assets/Image/WeaponThum/Shield/Frostveil_Shield.Frostveil_Shield"))
    (:Radiance%20Shield
      (return "/Game/Assets/Image/WeaponThum/Shield/Radiance_Shield.Radiance_Shield"))
    (:Firestorm%20Shield
      (return "/Game/Assets/Image/WeaponThum/Shield/Firestorm_Shield.Firestorm_Shield"))
    (:Blackstone%20Shield
      (return "/Game/Assets/Image/WeaponThum/Shield/Blackstone_Shield.Blackstone_Shield"))
    (:Moonshadow%20Shield
      (return "/Game/Assets/Image/WeaponThum/Shield/Moonshadow_Shield.Moonshadow_Shield"))
    (:Starbright%20Shield
      (return "/Game/Assets/Image/WeaponThum/Shield/Starbright_Shield.Starbright_Shield"))
    (:Grimward%20Shield
      (return "/Game/Assets/Image/WeaponThum/Shield/Grimward_Shield.Grimward_Shield"))
    (:Everglow%20Shield
      (return "/Game/Assets/Image/WeaponThum/Shield/Everglow_Shield.Everglow_Shield"))
    (:Brimstone%20Shield
      (return "/Game/Assets/Image/WeaponThum/Shield/Brimstone_Shield.Brimstone_Shield"))
    (:Titanforge%20Shield
      (return "/Game/Assets/Image/WeaponThum/Shield/Titanforge_Shield.Titanforge_Shield"))
    (:Aegis%20Shield
      (return "/Game/Assets/Image/WeaponThum/Shield/Aegis_Shield.Aegis_Shield"))
    (:BuffaloShield
      (return "/Game/Assets/Image/WeaponThum/Shield/Buffalo_Shield.Buffalo_Shield"))
    (:FostbiteShield
      (return "/Game/Assets/Image/WeaponThum/Shield/Fostbite_Shield.Fostbite_Shield"))))

(fn GetTexturebyName
  (params (WeaponName :type String))
  (if (Utilities|String|Contains WeaponName "Sword")
    (return (CallFunction|GetSwordTexturebyName WeaponName))
    (elif (Utilities|String|Contains WeaponName "Axe")
      (return (CallFunction|GetAxeTexturebyName WeaponName))
      (else
        (return (CallFunction|GetShieldTexturebyName WeaponName))))))

(fn GetAvatarbyName
  (params (Avatar :type E_Avatar%20Enum :default "NewEnumerator0"))
  (switch Utilities|FlowControl|Switch|SwitchonE_Avatar Avatar
    (:NewEnumerator0
      (return "/Game/Assets/Image/Avatar/avatar_1.avatar_1"))
    (:NewEnumerator18
      (return "/Game/Assets/Image/Avatar/avatar_2.avatar_2"))
    (:NewEnumerator19
      (return "/Game/Assets/Image/Avatar/avatar_3.avatar_3"))
    (:NewEnumerator20
      (return "/Game/Assets/Image/Avatar/avatar_4.avatar_4"))
    (:NewEnumerator21
      (return "/Game/Assets/Image/Avatar/avatar_5.avatar_5"))
    (:NewEnumerator22
      (return "/Game/Assets/Image/Avatar/avatar_6.avatar_6"))
    (:NewEnumerator23
      (return "/Game/Assets/Image/Avatar/avatar_7.avatar_7"))
    (:NewEnumerator24
      (return "/Game/Assets/Image/Avatar/avatar_8.avatar_8"))
    (:NewEnumerator25
      (return "/Game/Assets/Image/Avatar/avatar_9.avatar_9"))
    (:NewEnumerator26
      (return "/Game/Assets/Image/Avatar/avatar_10.avatar_10"))
    (:NewEnumerator27
      (return "/Game/Assets/Image/Avatar/avatar_11.avatar_11"))
    (:NewEnumerator28
      (return "/Game/Assets/Image/Avatar/avatar_12.avatar_12"))
    (:NewEnumerator29
      (return "/Game/Assets/Image/Avatar/avatar_13.avatar_13"))
    (:NewEnumerator30
      (return "/Game/Assets/Image/Avatar/avatar_14.avatar_14"))
    (:NewEnumerator31
      (return "/Game/Assets/Image/Avatar/avatar_15.avatar_15"))
    (:NewEnumerator32
      (return "/Game/Assets/Image/Avatar/avatar_16.avatar_16"))))

(fn GetCharacterThumbyName
  (params (CharacterName :type E_CharacterName%20Enum :default "NewEnumerator0"))
  (switch Utilities|FlowControl|Switch|SwitchonE_CharacterName CharacterName
    (:NewEnumerator0
      (return "/Game/Assets/Image/CharacterThum/Hauntseeker.Hauntseeker"))
    (:NewEnumerator20
      _)
    (:NewEnumerator1
      _)
    (:NewEnumerator2
      (return "/Game/Assets/Image/CharacterThum/Grimstone.Grimstone"))
    (:NewEnumerator3
      (return "/Game/Assets/Image/CharacterThum/Grimstone.Grimstone"))
    (:NewEnumerator4
      (return "/Game/Assets/Image/CharacterThum/Starwind.Starwind"))
    (:NewEnumerator5
      (return "/Game/Assets/Image/CharacterThum/Frostwalker.Frostwalker"))
    (:NewEnumerator6
      (return "/Game/Assets/Image/CharacterThum/Frostwalker.Frostwalker"))
    (:NewEnumerator7
      (return "/Game/Assets/Image/CharacterThum/ThunderstormLegender.ThunderstormLegender"))
    (:NewEnumerator8
      (return "/Game/Assets/Image/CharacterThum/Lotus.Lotus"))
    (:NewEnumerator9
      (return "/Game/Assets/Image/CharacterThum/Lotus.Lotus"))
    (:NewEnumerator10
      (return "/Game/Assets/Image/CharacterThum/Sunfire.Sunfire"))
    (:NewEnumerator11
      (return "/Game/Assets/Image/CharacterThum/Emberblade.Emberblade"))
    (:NewEnumerator12
      (return "/Game/Assets/Image/CharacterThum/Dawnbreaker.Dawnbreaker"))
    (:NewEnumerator13
      (return "/Game/Assets/Image/CharacterThum/Dawnbreaker.Dawnbreaker"))
    (:NewEnumerator14
      (return "/Game/Assets/Image/CharacterThum/Voidwalker.Voidwalker"))
    (:NewEnumerator15
      (return "/Game/Assets/Image/CharacterThum/KingAuthur.KingAuthur"))
    (:NewEnumerator17
      (return "/Game/Assets/Image/CharacterThum/Thunderstorm.Thunderstorm")))
  (return "/Game/Assets/Image/CharacterThum/Alaric.Alaric"))