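; BP_StaticMeshExtension is a utility that resolves a weapon or shield name to its static mesh.
; Separate switch-based lookups cover swords, axes and shields, with maces and hammers included in the sword lookup.
; GetStaticMeshByName routes by substring: "sword", then "axe", otherwise shields.
; Mace and hammer names therefore fall through to the shield lookup, which has no cases for them.
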(fn GetSwordStaticMeshbyName
  (params (WeaponName :type String))
  (switch string WeaponName
    (:AbyssalSword
      (return "/Game/Assets/Weapons/Swords/AbyssalSword/AbyssalSword.AbyssalSword"))
    (:Radiant%20Sword
      (return "/Game/Assets/Weapons/Swords/RadianSword/RadiantSword.RadiantSword"))
    (:Eclipse%20Sword
      (return "/Game/Assets/Weapons/Swords/EclipseSword/EclipseSword.EclipseSword"))
    (:Warcry%20Sword
      (return "/Game/Assets/Weapons/Swords/WarcrySword/WarcrySword.WarcrySword"))
    (:Tempest%20Sword
      (return "/Game/Assets/Weapons/Swords/TempestSword/TempestSword.TempestSword"))
    (:Sunblade%20Sword
      (return "/Game/Assets/Weapons/Swords/SubbladeSword/SunbladeSword.SunbladeSword"))
    (:Stormrage%20Sword
      (return "/Game/Assets/Weapons/Swords/StormrageSword/StormrageSword.StormrageSword"))
    (:Mystic%20Sword
      (return "/Game/Assets/Weapons/Swords/MysticSword/MysticSword.MysticSword"))
    (:Blackfire%20Sword
      (return "/Game/Assets/Weapons/Swords/BlackfireSword/BlackfireSword.BlackfireSword"))
    (:Grim%20Reaper%20Sword
      (return "/Game/Assets/Weapons/Swords/GrimReaperSword/GrimReaperSword.GrimReaperSword"))
    (:Silverlight%20Sword
      (return "/Game/Assets/Weapons/Swords/SilverlightSword/SilverlightSword.SilverlightSword"))
    (:Ice%20Sword
      (return "/Game/Assets/Weapons/Swords/IceSword/IceSword.IceSword"))
    (:Aurora%20Sword
      (return "/Game/Assets/Weapons/Swords/AuroraSword/AuroraSword.AuroraSword"))
    (:Dragonheart%20Sword
      (return "/Game/Assets/Weapons/Swords/DragonHeartSword/DragonheartSword.DragonheartSword"))
    (:Shadowbane%20Sword
      (return "/Game/Assets/Weapons/Swords/ShadowbaneSword/ShadowbaneSword.ShadowbaneSword"))
    (:Vortex%20Sword
      (return "/Game/Assets/Weapons/Swords/VortexSword/VortexSword.VortexSword"))
    (:Thundercry%20Sword
      (return "/Game/Assets/Weapons/Swords/ThundercrySword/ThundercrySword.ThundercrySword"))
    (:Seraphim%20Sword
      (return "/Game/Assets/Weapons/Swords/SeraphimSword/SeraphimSword.SeraphimSword"))
    (:Magic%20Sword
      (return "/Game/Assets/Weapons/Swords/MagicSword/MagicSword.MagicSword"))
    (:ThunderstormSword
      (return "/Game/Assets/Weapons/Swords/ThunderstormSword/ThunderstormSword.ThunderstormSword"))
    (:FostbiteSword
      (return "/Game/Assets/Weapons/Swords/FostbiteSword/FostbiteSword.FostbiteSword"))
    (:NightshadeSword
      (return "/Game/Assets/Weapons/Swords/NightshadeSword/NightshadeSword.NightshadeSword"))
    (:IroncladSword
      (return "/Game/Assets/Weapons/Swords/IroncladSword/IroncladSword.IroncladSword"))
    (:SunfireMace
      (return "/Game/Assets/Weapons/Others/MaceSunfire/SunfireMace.SunfireMace"))
    (:EmberbladeMace
      (return "/Game/Assets/Weapons/Axe/EmberbladeAxe/EmberbladeMace.EmberbladeMace"))
    (:DawnbreakerHammer
      (return "/Game/Assets/Weapons/Axe/DawnbreakerHammer/DawnbreakerHammer.DawnbreakerHammer"))
    (:BloodfangHammer
      (return "/Game/Assets/Weapons/Axe/BloodfangHammer/BloodfangHammer.BloodfangHammer"))
    (:VoidWalkerSword
      (return "/Game/Assets/Weapons/Swords/VoidWalkerSword/VoidWalkerSword.VoidWalkerSword"))
    (:KingAuthurSword
      (return "/Game/Assets/Weapons/Swords/KingAuthurSword/KingAuthurSword.KingAuthurSword"))))

(fn GetAxeStaticMeshbyName
  (params (Selection :type String))
  (switch string Selection
    (:Bloodiron%20Axe
      (return "/Game/Assets/Weapons/Axe/BloodironAxe/BloodironAxe.BloodironAxe"))
    (:Sunflare%20Axe
      (return "/Game/Assets/Weapons/Axe/SunflareAxe/SunflareAxe.SunflareAxe"))
    (:Blackfire%20Axe
      (return "/Game/Assets/Weapons/Axe/BlackIceAxe/BlackfireAxe.BlackfireAxe"))
    (:Nightshard%20Axe
      (return "/Game/Assets/Weapons/Axe/NightshardAxe/NightshardAxe.NightshardAxe"))
    (:Froststeel%20Axe
      (return "/Game/Assets/Weapons/Axe/FrostSteelAxe/FroststeelAxe.FroststeelAxe"))
    (:Voidblade%20Axe
      (return "/Game/Assets/Weapons/Axe/VoidbladeAxe/VoidbladeAxe.VoidbladeAxe"))
    (:Thunderclaw%20Axe
      (return "/Game/Assets/Weapons/Axe/ThunderclawAxe/ThunderclawAxe.ThunderclawAxe"))
    (:Shadowthorn%20Axe
      (return "/Game/Assets/Weapons/Axe/ShadowThornAxe/ShadowthornAxe.ShadowthornAxe"))
    (:Hellforged%20Axe
      (return "/Game/Assets/Weapons/Axe/HellForgedAxe/HellforgedAxe.HellforgedAxe"))
    (:Ironheart%20Axe
      (return "/Game/Assets/Weapons/Axe/IronheartAxe/IronheartAxe.IronheartAxe"))
    (:Icebreaker%20Axe
      (return "/Game/Assets/Weapons/Axe/IceBreakerAxe/IcebreakerAxe.IcebreakerAxe"))
    (:Duskstrike%20Axe
      (return "/Game/Assets/Weapons/Axe/DuskstrikeAxe/DuskstrikeAxe.DuskstrikeAxe"))
    (:Emberforge%20Axe
      (return "/Game/Assets/Weapons/Axe/EmberForgeAxe/EmberforgeAxe.EmberforgeAxe"))
    (:Stormwrath%20Axe
      (return "/Game/Assets/Weapons/Axe/StormWrathAxe/StormwrathAxe.StormwrathAxe"))
    (:Soulrender%20Axe
      (return "/Game/Assets/Weapons/Axe/SoulRenderAxe/SoulrenderAxe.SoulrenderAxe"))
    (:Frost%20Axe
      (return "/Game/Assets/Weapons/Axe/FrostAxe/FrostAxe.FrostAxe"))
    (:Doomcrusher%20Axe
      (return "/Game/Assets/Weapons/Axe/DomcrusherAxe/DoomcrusherAxe.DoomcrusherAxe"))
    (:Grimfury%20Axe
      (return "/Game/Assets/Weapons/Axe/GrimfuryAxe/GrimfuryAxe.GrimfuryAxe"))
    (:Dragonbone%20Axe
      (return "/Game/Assets/Weapons/Axe/DragonboneAxe/DragonboneAxe.DragonboneAxe"))
    (:Phoenixflame%20Axe
      (return "/Game/Assets/Weapons/Axe/PhoenixflameAxe/PhoenixflameAxe.PhoenixflameAxe"))
    (:BlazeheartAxe
      (return "/Game/Assets/Weapons/Axe/BlazeheartAxe/BlazeheartAxe.BlazeheartAxe"))))

(fn GetShieldStaticMeshbyName
  (params (Selection :type String))
  (switch string Selection
    (:Nightbane%20Shield
      (return "/Game/Assets/Weapons/Shield/NightbaneShield/NightbaneShield.NightbaneShield"))
    (:Ironfist%20Shield
      (return "/Game/Assets/Weapons/Shield/IronfistShield/IronfistShield.IronfistShield"))
    (:Earthshaker%20Shield
      (return "/Game/Assets/Weapons/Shield/EarthshakerShield/EarthshakerShield.EarthshakerShield"))
    (:Emberguard%20Shield
      (return "/Game/Assets/Weapons/Shield/EmberguardShield/EmberguardShield.EmberguardShield"))
    (:Sunburst%20Shield
      (return "/Game/Assets/Weapons/Shield/SunburstShield/SunburstShield.SunburstShield"))
    (:Thunderclap%20Shield
      (return "/Game/Assets/Weapons/Shield/ThunderclapShield/ThunderclapShield.ThunderclapShield"))
    (:Bloodthorn%20Shield
      (return "/Game/Assets/Weapons/Shield/BloodthornShield/BloodthornShield.BloodthornShield"))
    (:Mystic%20Shield
      (return "/Game/Assets/Weapons/Shield/MysticShield/MysticShield.MysticShield"))
    (:Windwhisper%20Shield
      (return "/Game/Assets/Weapons/Shield/WindwhisperShield/WindwhisperShield.WindwhisperShield"))
    (:Frostveil%20Shield
      (return "/Game/Assets/Weapons/Shield/FrostveilShield/FrostveilShield.FrostveilShield"))
    (:Radiance%20Shield
      (return "/Game/Assets/Weapons/Shield/RadianceShield/RadianceShield.RadianceShield"))
    (:Firestorm%20Shield
      (return "/Game/Assets/Weapons/Shield/FirestormShield/FirestormShield.FirestormShield"))
    (:Blackstone%20Shield
      (return "/Game/Assets/Weapons/Shield/BlackstoneShield/BlackstoneShield.BlackstoneShield"))
    (:Moonshadow%20Shield
      (return "/Game/Assets/Weapons/Shield/MoonshadowShield/MoonshadowShield.MoonshadowShield"))
    (:Starbright%20Shield
      (return "/Game/Assets/Weapons/Shield/StarbrightShield/StarbrightShield.StarbrightShield"))
    (:Grimward%20Shield
      (return "/Game/Assets/Weapons/Shield/GrimwardShield/GrimwardShield.GrimwardShield"))
    (:Everglow%20Shield
      (return "/Game/Assets/Weapons/Shield/EverglowShield/EverglowShield.EverglowShield"))
    (:Brimstone%20Shield
      (return "/Game/Assets/Weapons/Shield/BrimstoneShield/BrimstoneShield.BrimstoneShield"))
    (:Titanforge%20Shield
      (return "/Game/Assets/Weapons/Shield/TitanForgeShield/TitanforgeShield.TitanforgeShield"))
    (:Aegis%20Shield
      (return "/Game/Assets/Weapons/Shield/AegisShield/AegisShield.AegisShield"))
    (:BuffaloShield
      (return "/Game/Assets/Weapons/Shield/BuffaloShield/BuffaloShield.BuffaloShield"))
    (:FostbiteShield
      (return "/Game/Assets/Weapons/Shield/FostbiteShield/FostbiteShield.FostbiteShield"))
    (:IroncladShield
      (return "/Game/Assets/Weapons/Shield/IroncladShield/IroncladShield.IroncladShield"))
    (:KingAuthurShield
      (return "/Game/Assets/Weapons/Shield/KingAuthurShield/KingAuthurShield.KingAuthurShield"))))

(fn GetStaticMeshbyName
  (params (Name :type String))
  (if (Utilities|String|Contains Name "sword")
    (return (CallFunction|GetSwordStaticMeshbyName Name))
    (elif (Utilities|String|Contains Name "axe")
      (return (CallFunction|GetAxeStaticMeshbyName Name))
      (else
        (return (CallFunction|GetShieldStaticMeshbyName Name))))))