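; Launch menu HUD that manages the front-end screens, showing a splash widget at BeginPlay.
; The splash's navigate-to-home event swaps it for the Home widget, whose character and weapon spawn request is re-broadcast through the HUD's own SpawnActorsFromClass dispatcher.
; Background blur events are empty stubs, and the Home and SignUp init functions go uncalled here, with SignUp never added to the viewport.
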(event Custom|OnNavigateToHome_Event
  (Widget|RemovefromParent (stale EventBeginPlay _returnvalue))
  (bind _returnvalue (UserInterface|CreateWidget "/Game/UI/Screen/WBP_Home.WBP_Home_C"))
  (EventDispatchers|AssignSpawnActorsfromClass _returnvalue (delegate Custom|SpawnActorsFromClass_Event))
  (UserInterface|Viewport|AddtoViewport _returnvalue 0))

(event Custom|SpawnActorsFromClass_Event
  (params (Character :type Base%20Character%20Class%20Reference) (WeaponObj :type BP%20STR%20Weapon%20Structure))
  (Default|CallSpawnActorsfromClass Character WeaponObj))

(event EventBeginPlay
  (bind _returnvalue (UserInterface|CreateWidget "/Game/UI/Screen/WBP_Splash.WBP_Splash_C"))
  (UserInterface|Viewport|AddtoViewport _returnvalue 0)
  (EventDispatchers|AssignOnNavigatetoHome _returnvalue (delegate Custom|OnNavigateToHome_Event)))

(event EventShowBackgroundBlur)

(event EventHideBackgroundBlur)

(fn ConstructionScript)

(fn InitScreenHome
  (Widget|RemovefromParent (Variables|Default|GetWBP_Start))
  (bind _returnvalue (UserInterface|CreateWidget "/Game/UI/Screen/WBP_Home.WBP_Home_C"))
  (UserInterface|Viewport|AddtoViewport _returnvalue 0)
  (return _returnvalue))

(fn InitScreenSignUp
  (UserInterface|CreateWidget "/Game/UI/Screen/WBP_SignUp.WBP_SignUp_C"))