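; Player controller for gameplay that times a match and tallies damage dealt and taken through the possessed Base_Character's delegates.
; On death it saves character and match analytics to player and ranking data via SG_GameData, then syncs through BP_AuthRepository.
; It then broadcasts OnPlayerPawnDeath with totals and formatted duration, which is packed into a DateTime on today's date.
; CalculatorBossData, which rescales boss and soldier saves, is an unwired test hook.
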(event Custom|OnDeath_Event
  (bind _returnvalue (CallFunction|CalculatorCompletionTime))
  (bind _output_get (Variables|CompletionTime|SetEndCompletionTime (Class|KismetMathLibrary|ToUnixTimestamp (Math|DateTime|Now))))
  (Development|PrintString (Utilities|String|Append "PlayControl: End: " (Utilities|String|ToString(Integer) _output_get)))
  (Utilities|FlowControl|Delay 0.5)
  (Variables|MatchResult|SetMatchResult "NewEnumerator1")
  (Variables|Default|SetGameStatus "NewEnumerator4")
  (bind _returnvalue_2 (Game|ConstructObjectfromClass "/Game/Blueprints/Data/SaveGame/SG_GameData.SG_GameData_C"))
  (Default|UpdatePlayerData _returnvalue_2 (Utilities|Struct|MakeBP_STR_PlayerCharacter (.charactername (Variables|/Game/Blueprints/Characters/Base_Character.Base_Character_C|GetCurrentPlayerCharacter (stale EventBeginPlay _asbase_character))) (.level (Variables|/Game/Blueprints/Characters/Base_Character.Base_Character_C|GetCurrentPlayerCharacter (stale EventBeginPlay _asbase_character))) (.health (Variables|/Game/Blueprints/Characters/Base_Character.Base_Character_C|GetCurrentPlayerCharacter (stale EventBeginPlay _asbase_character))) (.staminareducewhenattackpercent (Variables|/Game/Blueprints/Characters/Base_Character.Base_Character_C|GetCurrentPlayerCharacter (stale EventBeginPlay _asbase_character))) (.stamina (Variables|/Game/Blueprints/Characters/Base_Character.Base_Character_C|GetCurrentPlayerCharacter (stale EventBeginPlay _asbase_character))) (.activatesword (Variables|/Game/Blueprints/Characters/Base_Character.Base_Character_C|GetCurrentPlayerCharacter (stale EventBeginPlay _asbase_character))) (.activateaxe (Variables|/Game/Blueprints/Characters/Base_Character.Base_Character_C|GetCurrentPlayerCharacter (stale EventBeginPlay _asbase_character))) (.activateshield (Variables|/Game/Blueprints/Characters/Base_Character.Base_Character_C|GetCurrentPlayerCharacter (stale EventBeginPlay _asbase_character))) (.credit (Variables|/Game/Blueprints/Characters/Base_Character.Base_Character_C|GetCurrentPlayerCharacter (stale EventBeginPlay _asbase_character))) (.license (Variables|/Game/Blueprints/Characters/Base_Character.Base_Character_C|GetCurrentPlayerCharacter (stale EventBeginPlay _asbase_character))) (Utilities|Struct|MakeBP_STR_MatchAnalytics (Variables|MatchResult|GetMatchResult) (Variables|Damage|GetTotalDamageDealt) (Variables|Damage|GetTotalDamageTaken) (Variables|Phase|GetMaxPhase) (Math|Conversions|ToFloat(Integer) (Class|KismetMathLibrary|ToUnixTimestamp (Math|DateTime|Now))) 0 0 (Class|KismetMathLibrary|ToUnixTimestampDouble (CallFunction|CalculatorCompletionTime))) (.isactive (Variables|/Game/Blueprints/Characters/Base_Character.Base_Character_C|GetCurrentPlayerCharacter (stale EventBeginPlay _asbase_character))) (.maxlevel (Variables|/Game/Blueprints/Characters/Base_Character.Base_Character_C|GetCurrentPlayerCharacter (stale EventBeginPlay _asbase_character))) (.maxhealth (Variables|/Game/Blueprints/Characters/Base_Character.Base_Character_C|GetCurrentPlayerCharacter (stale EventBeginPlay _asbase_character))) (.maxstamina (Variables|/Game/Blueprints/Characters/Base_Character.Base_Character_C|GetCurrentPlayerCharacter (stale EventBeginPlay _asbase_character))) (.typeequip (Variables|/Game/Blueprints/Characters/Base_Character.Base_Character_C|GetCurrentPlayerCharacter (stale EventBeginPlay _asbase_character)))))
  (Default|UpdateRankingData _returnvalue_2 (Utilities|Struct|MakeBP_STR_MatchAnalytics (Variables|MatchResult|GetMatchResult) (Variables|Damage|GetTotalDamageDealt) (Variables|Damage|GetTotalDamageTaken) (Variables|Phase|GetMaxPhase) (Math|Conversions|ToFloat(Integer) (Class|KismetMathLibrary|ToUnixTimestamp (Math|DateTime|Now))) 0 0 (Class|KismetMathLibrary|ToUnixTimestampDouble (CallFunction|CalculatorCompletionTime))))
  (Utilities|FlowControl|Delay 1.0)
  (bind _returnvalue_3 (Game|ConstructObjectfromClass "/Game/Blueprints/Data/Repository/BP_AuthRepository.BP_AuthRepository_C"))
  (Default|SyncUserData _returnvalue_3)
  (bind _returnvalue_4 (Game|ConstructObjectfromClass "/Game/Blueprints/Utils/BP_StringExtensions.BP_StringExtensions_C"))
  (Development|PrintString (Utilities|String|Append "Hour: " (Utilities|String|ToString(Integer) (Class|KismetMathLibrary|GetHour _returnvalue)) " Minute: " (Utilities|String|ToString(Integer) (Class|KismetMathLibrary|GetMinute _returnvalue)) " Second: " (Utilities|String|ToString(Integer) (Class|KismetMathLibrary|GetSecond _returnvalue))))
  (Default|CallOnPlayerPawnDeath (Variables|Damage|GetTotalDamageTaken) (Variables|Damage|GetTotalDamageDealt) (Default|FormatTimestamp _returnvalue_4 _returnvalue)))

(event Custom|OnDamageDealt_Event
  (params (Damage :type Float%20%28double-precision%29))
  (Variables|Damage|SetTotalDamageDealt (+ (Variables|Damage|GetTotalDamageDealt) Damage)))

(event Custom|OnDamageTaken_Event
  (params (Damage :type Float%20%28double-precision%29))
  (Variables|Damage|SetTotalDamageTaken (+ (Variables|Damage|GetTotalDamageTaken) Damage)))

(event EventBeginPlay
  (Variables|Default|SetGameStatus "NewEnumerator0")
  (bind _output_get (Variables|CompletionTime|SetStartCompletionTime (Class|KismetMathLibrary|ToUnixTimestamp (Math|DateTime|Now))))
  (Development|PrintString (Utilities|String|Append "PlayControl Start: " (Utilities|String|ToString(Integer) _output_get)))
  (Class|PlayerController|ActivateTouchInterface self "/Game/Input/TIS_Play.TIS_Play")
  (bind _asbase_character (Utilities|Casting|CastToBase_Character (Game|Player|GetPlayerPawn 0)))
  (EventDispatchers|AssignOnDeath _asbase_character (delegate Custom|OnDeath_Event))
  (EventDispatchers|AssignOnDamageDealt _asbase_character (delegate Custom|OnDamageDealt_Event))
  (EventDispatchers|AssignOnDamageTaken _asbase_character (delegate Custom|OnDamageTaken_Event)))

(fn ConstructionScript)

(fn CalculatorCompletionTime
  (bind _returnvalue (Math|DateTime|Now))
  (bind _endcompletiontime (Variables|CompletionTime|GetEndCompletionTime))
  (bind _startcompletiontime (Variables|CompletionTime|GetStartCompletionTime))
  (bind _returnvalue_2 (Class|KismetMathLibrary|FromUnixTimestamp _startcompletiontime))
  (bind _returnvalue_3 (Class|KismetMathLibrary|FromUnixTimestamp _endcompletiontime))
  (bind _returnvalue_4 (- _returnvalue_3 _returnvalue_2))
  (bind (_days _hours _minutes _seconds) (Class|KismetMathLibrary|BreakTimespan2 _returnvalue_4))
  (return (Math|DateTime|MakeDateTime (Class|KismetMathLibrary|GetYear _returnvalue) (Class|KismetMathLibrary|GetMonth _returnvalue) (Class|KismetMathLibrary|GetDay _returnvalue) _hours _minutes _seconds)))

(fn CalculatorBossData
  (bind _returnvalue (Game|ConstructObjectfromClass "/Game/Blueprints/Data/SaveGame/SG_GameData.SG_GameData_C"))
  (bind _sg_gamedata (Default|LoadLocalGameData _returnvalue))
  (bind _characteractive1 (Default|GetCharacterActive _returnvalue))
  (Default|UpdateAllBossData _returnvalue _sg_gamedata _characteractive1)
  (Default|UpdateAllSoliderData _returnvalue _sg_gamedata _characteractive1)
  (Default|SaveLocalGameData _returnvalue _sg_gamedata))