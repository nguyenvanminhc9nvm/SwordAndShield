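; BP_DR_Magma_explosion is a projectile-folder actor that deals damage and plays impact effects when its Box collision hits something.
; On BeginPlay, the Box ignores the Instigator while moving, falling back to the Owner if no valid Instigator exists.
; A hit spawns an emitter and sound, applies point damage to the hit actor with the Owner as causer, then destroys itself.
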(event OnComponentHit(Box)
  (params (HitComponent :type Primitive%20Component%20Object%20Reference) (OtherActor :type Actor%20Object%20Reference) (OtherComp :type Primitive%20Component%20Object%20Reference) (NormalImpulse :type Vector :default "0, 0, 0") (Hit :type Hit%20Result%20Structure%20%28by%20ref%29))
  (bind (_bblockinghit _binitialoverlap _time _distance _location _impactpoint _normal _impactnormal _physmat _hitactor) (Collision|BreakHitResult Hit))
  (Effects|SpawnEmitteratLocation (Variables|Default|GetImpactEmitter) _impactpoint)
  (Audio|PlaySoundatLocation (Variables|Default|GetImpactSound) _location "0, 0, 0" 1.0 1.0 0.0 0 0 0 0)
  (Game|Damage|ApplyPointDamage _hitactor (Variables|Default|GetDamage) _location Hit 0 (Components|GetOwner))
  (Actor|DestroyActor))

(event EventBeginPlay
  (bind _returnvalue (Game|GetInstigator))
  (Collision|IgnoreActorwhenMoving (Variables|Default|GetBox) (select (Utilities|IsValid _returnvalue) _returnvalue (Components|GetOwner)) true))

(event Collision|EventActorBeginOverlap
  (params (OtherActor :type Actor%20Object%20Reference)))

(fn ConstructionScript)