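; Shuriken trap projectile that spins, whirs and deals point damage to what it hits.
; Tick adds a fixed yaw step to the mesh each frame, not scaled by delta time, and replays the flight sound using a flag reset by a short Delay.
; Mesh overlap prints a debug string, spawns impact effects and sound, applies damage with the owner as causer, then destroys the actor.
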(event OnComponentBeginOverlap(StaticMesh)
  (params (OverlappedComponent :type Primitive%20Component%20Object%20Reference) (OtherActor :type Actor%20Object%20Reference) (OtherComp :type Primitive%20Component%20Object%20Reference) (OtherBodyIndex :type Integer) (bFromSweep :type Boolean) (SweepResult :type Hit%20Result%20Structure%20%28by%20ref%29))
  (bind (_bblockinghit _binitialoverlap _time _distance _location _impactpoint _normal _impactnormal _physmat _hitactor) (Collision|BreakHitResult SweepResult))
  (Development|PrintString "overlap")
  (Effects|SpawnEmitteratLocation (Variables|Default|GetImpactEmitter) _impactpoint)
  (Audio|PlaySoundatLocation (Variables|Default|GetImpactSound) _location "0, 0, 0" 1.0 1.0 0.0 0 0 0 0)
  (Game|Damage|ApplyPointDamage _hitactor (Variables|Default|GetDamage) _location SweepResult 0 (Components|GetOwner))
  (Actor|DestroyActor))

(event EventTick
  (params (DeltaSeconds :type Float%20%28single-precision%29))
  (Transformation|SetWorldRotation (Variables|Default|GetStaticMesh) (Math|Rotator|MakeRotator 0.0 0.0 (+ (.yaw (Transformation|GetWorldRotation (Variables|Default|GetStaticMesh))) 2e+02)) false false)
  (if (Variables|Default|GetIsAudioFinished)
    (Utilities|FlowControl|Delay 0.2)
    (Variables|Default|SetIsAudioFinished false)
    (else
      (Audio|PlaySoundatLocation (Variables|Default|GetSound) (Transformation|GetActorLocation) "0, 0, 0" 1.0 1.0 0.0 0 0 0 0)
      (Variables|Default|SetIsAudioFinished true))))

(fn ConstructionScript)