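; Starwind variant of the gate base Blueprint that spawns a Starwind encounter when a character enters it.
; On the first valid overlap by a Base_Character, it records a Unix start timestamp and spawns a StarwindBeetle and a StarwindMolten at their marker components.
; An IsSpawnEnemy flag keeps the spawn from repeating, while construction defers to the parent gate.
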(event EventBeginPlay
  (|CallParentFunction) ; This node is disabled and will not be called.\nDrag off pins to build functionality.
)

(event Collision|EventActorBeginOverlap
  (params (OtherActor :type Actor%20Object%20Reference))
  ;[1 1 1] Spawn Enemy
  (Utilities|IsValid OtherActor
    (:Is%20Valid
      (Utilities|Casting|CastToBase_Character OtherActor)
      (if (not (Variables|Default|GetIsSpawnEnemy))
        (Variables|Default|SetStartTime (Class|KismetMathLibrary|ToUnixTimestamp (Math|DateTime|Now)))
        (Game|SpawnActorfromClass "/Game/Blueprints/Characters/EnemyCharacter/StarwindBeetle.StarwindBeetle_C" (Math|Transform|MakeTransform (Transformation|GetWorldLocation (Variables|Default|GetPointStarwindBeetle)) "0, 0, 0" "1.000000,1.000000,1.000000") "AlwaysSpawn" "MultiplyWithRoot" 0 0)
        (Game|SpawnActorfromClass "/Game/Blueprints/Characters/EnemyCharacter/StarwindMolten.StarwindMolten_C" (Math|Transform|MakeTransform (Transformation|GetWorldLocation (Variables|Default|GetPointStarwindMolten)) "0, 0, 0" "1.000000,1.000000,1.000000") "AlwaysSpawn" "MultiplyWithRoot" 0 0)
        (Variables|Default|SetIsSpawnEnemy true)))))

(fn ConstructionScript
  (|CallParentFunction))