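; Grimstone gate, a child gate Blueprint that spawns an enemy when a character of a specific player type enters it.
; On overlap it checks the character's PlayerType, records a Unix start time and spawns the Enemy class at the PointDawnbreaker location.
; The IsSpawnEnemy flag limits the spawn to one time.
; Leftover nodes for changing the game phase and spawning Nightshade at PointSpawnZombie are unwired and never run.
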(event Collision|EventActorBeginOverlap
  (params (OtherActor :type Actor%20Object%20Reference))
  (Utilities|IsValid OtherActor
    (:Is%20Valid
      (bind _asbase_character (Utilities|Casting|CastToBase_Character OtherActor))
      (if (Utilities|Enum|Equal(Enum) (Variables|/Game/Blueprints/Characters/Base_Character.Base_Character_C|GetPlayerType _asbase_character) "NewEnumerator0")
        (if (not (Variables|Default|GetIsSpawnEnemy))
          (Variables|Default|SetStartTime (Class|KismetMathLibrary|ToUnixTimestamp (Math|DateTime|Now)))
          (Game|SpawnActorfromClass (Variables|Default|GetEnemy) (Math|Transform|MakeTransform (Transformation|GetWorldLocation (Variables|Default|GetPointDawnbreaker)) "0, 0, 0" "1.000000,1.000000,1.000000") "AlwaysSpawn" "MultiplyWithRoot" self 0)
          (Variables|Default|SetIsSpawnEnemy true))))))

(fn ConstructionScript
  (|CallParentFunction))