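; Gate actor, a child of the gate base, that spawns the Dawnbreaker and Bloodfang enemies when a Base_Character first overlaps it.
; The overlap records a Unix-timestamp StartTime, then spawns each enemy at its own spawn point, ignoring collisions.
; An IsSpawnEnemy flag keeps the spawn from repeating, and the construction script only runs the parent's.
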(event Collision|EventActorBeginOverlap
  (params (OtherActor :type Actor%20Object%20Reference))
  (Utilities|IsValid OtherActor
    (:Is%20Valid
      (Utilities|Casting|CastToBase_Character OtherActor)
      (if (not (Variables|Default|GetIsSpawnEnemy))
        (Variables|Default|SetStartTime (Class|KismetMathLibrary|ToUnixTimestamp (Math|DateTime|Now)))
        (Game|SpawnActorfromClass "/Game/Blueprints/Characters/EnemyCharacter/Dawnbreaker.Dawnbreaker_C" (Math|Transform|MakeTransform (Transformation|GetWorldLocation (Variables|Default|GetPointSpawnZombie)) "0, 0, 0" "1.000000,1.000000,1.000000") "AlwaysSpawn" "MultiplyWithRoot" 0 0)
        (Game|SpawnActorfromClass "/Game/Blueprints/Characters/EnemyCharacter/Bloodfang.Bloodfang_C" (Math|Transform|MakeTransform (Transformation|GetWorldLocation (Variables|Default|GetPointSpawnZombie1)) "0, 0, 0" "1.000000,1.000000,1.000000") "AlwaysSpawn" "MultiplyWithRoot" 0 0)
        (Variables|Default|SetIsSpawnEnemy true)))))

(fn ConstructionScript
  (|CallParentFunction))