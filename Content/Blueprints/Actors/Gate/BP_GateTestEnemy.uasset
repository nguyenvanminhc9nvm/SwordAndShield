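; Test gate actor that spawns a sequence of enemies, one at a time, once a Base_Character of the first PlayerType overlaps it.
; Each enemy comes from the Enemy class array at the current Index and appears at the PointDawnbreaker location.
; Its OnDeath event increments Index and spawns the next, with IsSpawnEnemy blocking repeat spawns while one is active.
; The bounds check only rejects an Index greater than the array length, so Index equal to Length passes.
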(event Custom|OnDeath_Event
  ;[1 1 1] Spawn Enemy
  (bind _output_get (Variables|Default|SetIndex (+ (Variables|Default|GetIndex) 1)))
  (Variables|Default|SetIsSpawnEnemy false)
  (CallFunction|SpawEnemy _output_get))

(event Custom|SpawEnemy
  (params (Index :type Integer))
  ;[1 1 1] Spawn Enemy
  (if (not (Variables|Default|GetIsSpawnEnemy))
    (if (not (> Index (Utilities|Array|Length (Variables|Default|GetEnemy))))
      (bind _returnvalue (Game|SpawnActorfromClass (Utilities|Array|Get(acopy) (Variables|Default|GetEnemy) Index) (Math|Transform|MakeTransform (Transformation|GetWorldLocation (Variables|Default|GetPointDawnbreaker)) "0, 0, 0" "1.000000,1.000000,1.000000") "AlwaysSpawn" "MultiplyWithRoot" self 0))
      (Variables|Default|SetIsSpawnEnemy true)
      (Utilities|IsValid _returnvalue
        (:Is%20Valid
          (EventDispatchers|AssignOnDeath _returnvalue (delegate Custom|OnDeath_Event)))))))

(event Collision|EventActorBeginOverlap
  (params (OtherActor :type Actor%20Object%20Reference))
  ;[1 1 1] Spawn Enemy
  (Utilities|IsValid OtherActor
    (:Is%20Valid
      (bind _asbase_character (Utilities|Casting|CastToBase_Character OtherActor))
      (if (Utilities|Enum|Equal(Enum) (Variables|/Game/Blueprints/Characters/Base_Character.Base_Character_C|GetPlayerType _asbase_character) "NewEnumerator0")
        (CallFunction|SpawEnemy (Variables|Default|GetIndex))))))

(fn ConstructionScript)