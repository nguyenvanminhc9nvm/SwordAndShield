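; Meteor rain projectile actor that damages what its box collision hits, then destroys itself after a short delay.
; On BeginPlay the box ignores the instigator, or the owner as fallback, while moving.
; Tick steps the ProjectileMovement initial and max speed up to a cap through SetSpeedMove, which also sets partial gravity.
; Hits apply point damage with the owner as causer, and debug strings print speed and hits.
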(event OnComponentHit(Box)
  (params (HitComponent :type Primitive%20Component%20Object%20Reference) (OtherActor :type Actor%20Object%20Reference) (OtherComp :type Primitive%20Component%20Object%20Reference) (NormalImpulse :type Vector :default "0, 0, 0") (Hit :type Hit%20Result%20Structure%20%28by%20ref%29))
  (bind (_bblockinghit _binitialoverlap _time _distance _location _impactpoint _normal _impactnormal _physmat _hitactor) (Collision|BreakHitResult Hit))
  (Development|PrintString "Hit")
  (Game|Damage|ApplyPointDamage _hitactor (Variables|Default|GetDamage) _location Hit 0 (Components|GetOwner))
  (Utilities|FlowControl|Delay 2.0)
  (Actor|DestroyActor))

(event EventBeginPlay
  (bind _returnvalue (Game|GetInstigator))
  (Collision|IgnoreActorwhenMoving (Variables|Default|GetBox) (select (Utilities|IsValid _returnvalue) _returnvalue (Components|GetOwner)) true))

(event EventTick
  (params (DeltaSeconds :type Float%20%28single-precision%29))
  (bind _projectilemovement (Variables|Default|GetProjectileMovement))
  (bind _returnvalue (Class|MovementComponent|GetMaxSpeed _projectilemovement))
  (if (not (>= _returnvalue 1e+03))
    (CallFunction|SetSpeedMove (+ _returnvalue 1e+02))
    (Development|PrintString (Utilities|String|Append "Speed: " (Utilities|String|ToString(Float) _returnvalue) "IntiSpped"))))

(fn ConstructionScript)

(fn SetSpeedMove
  (params (NewSpeed :type Float%20%28double-precision%29))
  (bind _projectilemovement (Variables|Default|GetProjectileMovement))
  (Variables|/Script/Engine.ProjectileMovementComponent|SetInitialSpeed _projectilemovement NewSpeed)
  (Variables|/Script/Engine.ProjectileMovementComponent|SetMaxSpeed _projectilemovement NewSpeed)
  (Variables|/Script/Engine.ProjectileMovementComponent|SetProjectileGravityScale _projectilemovement 0.5))