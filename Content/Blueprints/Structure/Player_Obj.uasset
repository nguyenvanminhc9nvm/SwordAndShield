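; Player data object holding stats, equipped and owned swords, axes and shields, and an English or Vietnamese character description.
; Add and equip functions store Weapon_Obj data as structs, while display getters construct Weapon_Obj instances from those lists, copying only some fields.
; Attack damage per type derives from AttackDamage by fixed percentage cuts, with ratio getters alongside.
; Power-ups raise max health, stamina and damage by a fixed percentage.
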(fn EquipNewAxe
  (params (Weapon :type Weapon%20Obj%20Object%20Reference))
  (bind _weaponstructure (CallFunction|ConvertWeaponObjtoWeaponStructure Weapon))
  (Variables|Default|SetAxeEquip _weaponstructure))

(fn EquipNewShield
  (params (Weapon :type Weapon%20Obj%20Object%20Reference))
  (bind _weaponstructure (CallFunction|ConvertWeaponObjtoWeaponStructure Weapon))
  (Variables|Default|SetShieldEquip _weaponstructure))

(fn EquipNewSword
  (params (Weapon :type Weapon%20Obj%20Object%20Reference))
  (bind _weaponstructure (CallFunction|ConvertWeaponObjtoWeaponStructure Weapon))
  (Variables|Default|SetSwordEquip _weaponstructure))

(fn ConvertListSwordtoObject
  (params (ListStructure :type Array%20of%20Weapon%20Structure%20Structures))
  (for _array_element ListStructure
    (bind _returnvalue (Game|ConstructObjectfromClass "/Game/Blueprints/Structure/Weapon_Obj.Weapon_Obj_C"))
    (Utilities|FlowControl|Sequence
      (:then_0
        (Variables|/Game/Blueprints/Structure/Weapon_Obj.Weapon_Obj_C|SetTexture _returnvalue (.texture _array_element)))
      (:then_1
        (Variables|/Game/Blueprints/Structure/Weapon_Obj.Weapon_Obj_C|SetStaticMesh _returnvalue (.staticmesh _array_element)))
      (:then_2
        (Variables|/Game/Blueprints/Structure/Weapon_Obj.Weapon_Obj_C|SetName _returnvalue (.name _array_element)))
      (:then_3
        (Variables|/Game/Blueprints/Structure/Weapon_Obj.Weapon_Obj_C|SetCredit _returnvalue (.credit _array_element)))
      (:then_4
        (Variables|/Game/Blueprints/Structure/Weapon_Obj.Weapon_Obj_C|SetLicense _returnvalue (.licensing _array_element)))
      (:then_5
        (Variables|/Game/Blueprints/Structure/Weapon_Obj.Weapon_Obj_C|SetPrice _returnvalue (.price _array_element)))
      (:then_6
        (Variables|/Game/Blueprints/Structure/Weapon_Obj.Weapon_Obj_C|SetWeaponType _returnvalue (.weapontype _array_element)))))
  (Utilities|Array|Add (LocalVariables|GetListWeapon) _returnvalue)
  (return (LocalVariables|GetListWeapon)))

(fn UpdateNewPowerUp
  (Utilities|FlowControl|Sequence
    (:then_0
      (bind _newproperties (CallFunction|IncreaseProperties (Variables|Default|GetMaxStamina)))
      (Variables|Default|SetMaxStamina _newproperties))
    (:then_1
      (bind _newproperties_2 (CallFunction|IncreaseProperties (Variables|Default|GetMaxHeath)))
      (Variables|Default|SetMaxHeath _newproperties_2))
    (:then_2
      (bind _newproperties_3 (CallFunction|IncreaseProperties (Variables|Default|GetAttackDamage)))
      (Variables|Default|SetAttackDamage _newproperties_3))
    (:then_3
      (CallFunction|DecreaseProperties (Variables|Default|GetAttackDamage) 2e+01))
    (:then_4
      (CallFunction|DecreaseProperties (Variables|Default|GetAttackDamage) 8e+01))
    (:then_5
      (CallFunction|DecreaseProperties (Variables|Default|GetAttackDamage) 7e+01))
    (:then_6
      (CallFunction|DecreaseProperties (Variables|Default|GetAttackDamage) 1e+01))))

(fn IncreaseProperties
  (params (Properties :type Float%20%28double-precision%29))
  (return (+ Properties (* (/ Properties 1e+02) 2e+01))))

(fn ConstructorData)

(fn DecreaseProperties
  (params (Properties :type Float%20%28double-precision%29) (ReducePercent :type Float%20%28double-precision%29))
  (return (- Properties (* (/ Properties 1e+02) ReducePercent))))

(fn GetListSwordDisplay
  (bind _listobject (CallFunction|ConvertListSwordtoObject (Variables|Default|GetListSword)))
  (return _listobject))

(fn GetListAxeDisplay
  (bind _listobject (CallFunction|ConvertListSwordtoObject (Variables|Default|GetListAxe)))
  (return _listobject))

(fn GetListShieldDisplay
  (bind _listobject (CallFunction|ConvertListSwordtoObject (Variables|Default|GetListShield)))
  (return _listobject))

(fn GetCharacterDescbyLanguage
  (bind _returnvalue (Game|ConstructObjectfromClass "/Game/Blueprints/Constant/BP_Language.BP_Language_C"))
  (switch Utilities|FlowControl|Switch|SwitchonE_Language (Default|GetSettingLanguage _returnvalue)
    (:NewEnumerator1
      (return (Variables|Default|GetDescription_EN)))
    (:NewEnumerator0
      (return (Variables|Default|GetDescription_VI)))))

(fn GetDamageAttackbyWeapon
  (bind _newproperties (CallFunction|DecreaseProperties (Variables|Default|GetAttackDamage) 3e+01))
  (return _newproperties))

(fn GetDamageAttackbyPunch
  (bind _newproperties (CallFunction|DecreaseProperties (Variables|Default|GetAttackDamage) 7e+01))
  (return _newproperties))

(fn GetDamageAttackbyKick
  (bind _newproperties (CallFunction|DecreaseProperties (Variables|Default|GetAttackDamage) 6e+01))
  (return _newproperties))

(fn GetDamageAttackbyMagic
  (bind _newproperties (CallFunction|DecreaseProperties (Variables|Default|GetAttackDamage) 2e+01))
  (return _newproperties))

(fn GetDamageAttackbyWeaponPercent
  (return (/ (CallFunction|GetDamageAttackbyWeapon) (Variables|Default|GetAttackDamage))))

(fn GetDamageAttackbyPunchPercent
  (return (/ (CallFunction|GetDamageAttackbyPunch) (Variables|Default|GetAttackDamage))))

(fn GetDamageAttackbyKickPercent
  (return (/ (CallFunction|GetDamageAttackbyKick) (Variables|Default|GetAttackDamage))))

(fn GetDamageAttackbyMagicPercent
  (return (/ (CallFunction|GetDamageAttackbyMagic) (Variables|Default|GetAttackDamage))))

(fn GetMaxHeathPercent
  (return (/ (Variables|Default|GetMaxHeath) (Variables|Default|GetMaxHealthLevel))))

(fn GetMaxStaminaPercent
  (return (/ (Variables|Default|GetMaxStamina) (Variables|Default|GetMaxStaminaLevel))))

(fn AddNewSword
  (params (WeaponObj :type Weapon%20Obj%20Object%20Reference))
  (bind _weaponstructure (CallFunction|ConvertWeaponObjtoWeaponStructure WeaponObj))
  (Utilities|Array|Add (Variables|Default|GetListSword) _weaponstructure))

(fn ConvertWeaponObjtoWeaponStructure
  (params (WeaponObj :type Weapon%20Obj%20Object%20Reference))
  (return (Utilities|Struct|MakeWeapon_Structure (Variables|/Game/Blueprints/Structure/Weapon_Obj.Weapon_Obj_C|GetName WeaponObj) (Variables|/Game/Blueprints/Structure/Weapon_Obj.Weapon_Obj_C|GetTexture WeaponObj) (Variables|/Game/Blueprints/Structure/Weapon_Obj.Weapon_Obj_C|GetStaticMesh WeaponObj) (Variables|/Game/Blueprints/Structure/Weapon_Obj.Weapon_Obj_C|GetCredit WeaponObj) (Variables|/Game/Blueprints/Structure/Weapon_Obj.Weapon_Obj_C|GetLicense WeaponObj) (Variables|/Game/Blueprints/Structure/Weapon_Obj.Weapon_Obj_C|GetPrice WeaponObj) (Variables|/Game/Blueprints/Structure/Weapon_Obj.Weapon_Obj_C|GetWeaponType WeaponObj) (Variables|/Game/Blueprints/Structure/Weapon_Obj.Weapon_Obj_C|GetIncreaseDamage WeaponObj) (Variables|/Game/Blueprints/Structure/Weapon_Obj.Weapon_Obj_C|GetDecreaseSpeed WeaponObj) (Variables|/Game/Blueprints/Structure/Weapon_Obj.Weapon_Obj_C|GetMagicSkill WeaponObj))))

(fn AddNewAxe
  (params (WeaponObj :type Weapon%20Obj%20Object%20Reference))
  (bind _weaponstructure (CallFunction|ConvertWeaponObjtoWeaponStructure WeaponObj))
  (Utilities|Array|Add (Variables|Default|GetListAxe) _weaponstructure))

(fn AddNewShield
  (params (WeaponObj :type Weapon%20Obj%20Object%20Reference))
  (bind _weaponstructure (CallFunction|ConvertWeaponObjtoWeaponStructure WeaponObj))
  (Utilities|Array|Add (Variables|Default|GetListShield) _weaponstructure))