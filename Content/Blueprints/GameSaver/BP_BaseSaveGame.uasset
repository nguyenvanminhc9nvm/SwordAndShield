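; BP_BaseSaveGame is a save game Blueprint that holds combat stats and scales them by percentage when updated.
; UpdateNewData raises max stamina, max health and attack damage by a fixed percentage through UpdateAllProperties.
; It also lowers the weapon, punch, kick and magic damage-reduce values and attack stamina cost through UpdateAllReduceDamage.
; Each call overwrites the stored values and returns the object, so repeated updates compound.
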(fn UpdateNewData
  (bind _newproperties (CallFunction|UpdateAllProperties (Variables|Default|GetMaxStamina)))
  (Variables|Default|SetMaxStamina _newproperties)
  (bind _newproperties_2 (CallFunction|UpdateAllProperties (Variables|Default|GetMaxHeath)))
  (Variables|Default|SetMaxHeath _newproperties_2)
  (bind _newproperties_3 (CallFunction|UpdateAllProperties (Variables|Default|GetAttackDamage)))
  (Variables|Default|SetAttackDamage _newproperties_3)
  (bind _newdamagereduce (CallFunction|UpdateAllReduceDamage (Variables|Reduce|GetWeaponDamageReduce) 1e+01))
  (Variables|Reduce|SetWeaponDamageReduce _newdamagereduce)
  (bind _newdamagereduce_2 (CallFunction|UpdateAllReduceDamage (Variables|Reduce|GetPunchDamageReduce) 5.0))
  (Variables|Reduce|SetPunchDamageReduce _newdamagereduce_2)
  (bind _newdamagereduce_3 (CallFunction|UpdateAllReduceDamage (Variables|Reduce|GetKickDamageReduce) 5.0))
  (Variables|Reduce|SetKickDamageReduce _newdamagereduce_3)
  (bind _newdamagereduce_4 (CallFunction|UpdateAllReduceDamage (Variables|Reduce|GetMagicDamageReduce) 1e+01))
  (Variables|Reduce|SetMagicDamageReduce _newdamagereduce_4)
  (bind _newdamagereduce_5 (CallFunction|UpdateAllReduceDamage (Variables|Reduce|GetStaminaReduceWhenAttack) 1e+01))
  (Variables|Reduce|SetStaminaReduceWhenAttack _newdamagereduce_5)
  (return self))

(fn UpdateAllReduceDamage
  (params (BaseDamage :type Float%20%28double-precision%29) (ReducePercent :type Float%20%28double-precision%29))
  (return (- BaseDamage (* (/ BaseDamage 1e+02) ReducePercent))))

(fn UpdateAllProperties
  (params (Properties :type Float%20%28double-precision%29))
  (return (+ Properties (* (/ Properties 1e+02) 2e+01))))