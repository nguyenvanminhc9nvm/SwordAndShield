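; Stamina component that tracks a character's current and maximum stamina, clamping losses at a small floor above zero.
; Attacks drain a percentage of current stamina, discounted by action type, while blocked hits drain more than unblocked ones.
; Recovery and passive loss are fixed-step functions with no internal tick.
; At 15% or below, UpStamina can raise the maximum, refill stamina and play a power-up montage through BPI_BaseCharacter.
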(event EventBeginPlay)

(event EventTick
  (params (DeltaSeconds :type Float%20%28single-precision%29)))

(fn ReduceStaminabyPercent
  (params (PercentLoss :type Float%20%28double-precision%29))
  (Variables|Default|SetCurrentStamina (- (Variables|Default|GetCurrentStamina) (* (/ (Variables|Default|GetCurrentStamina) 1e+02) PercentLoss)))
  (if (< (Variables|Default|GetCurrentStamina) 0.01)
    (Variables|Default|SetCurrentStamina 0.01)))

(fn GetStaminaPercent
  (return (/ (Variables|Default|GetCurrentStamina) (Variables|Default|GetMaxStamina))))

(fn InitStamina
  (params (Stamina :type Float%20%28double-precision%29))
  (bind _output_get (Variables|Default|SetCurrentStamina Stamina))
  (Variables|Default|SetMaxStamina _output_get))

(fn UpStamina
  (params (PercentUp :type Float%20%28double-precision%29))
  (bind _returnvalue (Components|GetOwner))
  (if (<= (CallFunction|GetStaminaPercent) 0.15)
    (if (Utilities|DoesObjectImplementInterface _returnvalue "/Game/Blueprints/Interface/BPI_BaseCharacter.BPI_BaseCharacter_C")
      (bind _characterreferences (Class|BPIBaseCharacter|IGetCharacterReferences(Message) _returnvalue))
      (Animation|PlayAnimMontage _characterreferences (Variables|Default|GetAM_PowerUp) 1.0 "None")
      (CallFunction|InitStamina (+ (* (/ (Variables|Default|GetMaxStamina) 1e+02) PercentUp) (Variables|Default|GetMaxStamina))))))

(fn RecoverStamina
  (if (< (Variables|Default|GetCurrentStamina) (Variables|Default|GetMaxStamina))
    (Variables|Default|SetCurrentStamina (+ (Variables|Default|GetCurrentStamina) 0.1))))

(fn LossStamina
  (if (<= (Variables|Default|GetCurrentStamina) 0.01)
    (Variables|Default|SetCurrentStamina 0.01)
    (else
      (Variables|Default|SetCurrentStamina (- (Variables|Default|GetCurrentStamina) 0.01)))))

(fn UpdateStaminabyDamage
  (params (Damage :type Float%20%28double-precision%29) (IsBlock :type Boolean))
  (if IsBlock
    (Variables|Default|SetCurrentStamina (- (Variables|Default|GetCurrentStamina) (+ (* (/ Damage 1e+02) 2e+01) Damage)))
    (else
      (Variables|Default|SetCurrentStamina (- (Variables|Default|GetCurrentStamina) (- Damage (* (/ Damage 1e+02) 2e+01))))))
  (if (< (Variables|Default|GetCurrentStamina) 0.01)
    (Variables|Default|SetCurrentStamina 0.01)))

(fn CalculatorStaminaReducebyAction
  (params (E_Action :type E_Action%20Enum :default "NewEnumerator0"))
  (switch Utilities|FlowControl|Switch|SwitchonE_Action E_Action
    (:NewEnumerator0
      _)
    (:NewEnumerator1
      _)
    (:NewEnumerator2
      _)
    (:NewEnumerator3
      (bind _newstaminaloss (CallFunction|ReduceStaminaLoss 1e+01 :!label _label))
      (return _newstaminaloss))
    (:NewEnumerator4
      (goto _label))
    (:NewEnumerator5
      (goto _label))
    (:NewEnumerator6
      (goto _label))
    (:NewEnumerator7
      (goto _label))
    (:NewEnumerator13
      (bind _newstaminaloss_2 (CallFunction|ReduceStaminaLoss 7e+01 :!label _label_2))
      (return _newstaminaloss_2))
    (:NewEnumerator14
      (goto _label_2))
    (:NewEnumerator15
      (goto _label_2))
    (:NewEnumerator16
      (bind _newstaminaloss_3 (CallFunction|ReduceStaminaLoss 5e+01 :!label _label_3))
      (return _newstaminaloss_3))
    (:NewEnumerator17
      (goto _label_3))
    (:NewEnumerator18
      (goto _label_3))
    (:NewEnumerator19
      (goto _label_3)))
  (bind _newstaminaloss_4 (CallFunction|ReduceStaminaLoss 8e+01))
  (return _newstaminaloss_4))

(fn ReduceStaminaLoss
  (params (DamageReduce :type Float%20%28double-precision%29))
  (return (- (Variables|Default|GetStaminaLossWhenAttack) (* DamageReduce (/ (Variables|Default|GetStaminaLossWhenAttack) 1e+02)))))

(fn ReduceStaminawhenAttack
  (params (Action :type E_Action%20Enum :default "NewEnumerator0"))
  (bind _staminaloss (CallFunction|CalculatorStaminaReducebyAction Action))
  (Variables|Default|SetCurrentStamina (- (Variables|Default|GetCurrentStamina) (* (/ (Variables|Default|GetCurrentStamina) 1e+02) _staminaloss)))
  (if (< (Variables|Default|GetCurrentStamina) 0.01)
    (Variables|Default|SetCurrentStamina 0.01)))