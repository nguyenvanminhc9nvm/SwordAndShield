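; Actor component that runs combat for BPI_BaseCharacter owners, covering punch, kick, weapon and magic attacks plus shield blocking.
; Attack requests play per-action montages, buffering input made mid-attack until ContinueAttack chains the combo.
; Sphere traces between mesh socket pairs apply point damage once per actor per swing, scaled by category reduction percentages.
; Helpers pick random actions and spawn randomly chosen magic actors carrying calculated damage.
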(event EventBeginPlay)

(event EventTick
  (params (DeltaSeconds :type Float%20%28single-precision%29)))

(fn RequestAttack
  (params (Action :type E_Action%20Enum :default "NewEnumerator0"))
  (if (or (not (Variables|Default|GetIsAttacking)) (Variables|Default|GetCanContinue))
    (CallFunction|DoAttack Action)
    (else
      (Variables|Default|SetHasAttack true))))

(fn DoAttack
  (params (Action :type E_Action%20Enum :default "NewEnumerator0"))
  (bind _returnvalue (Components|GetOwner))
  (bind _output_get (Variables|Default|SetCurrentAction Action))
  (if (Utilities|DoesObjectImplementInterface _returnvalue "/Game/Blueprints/Interface/BPI_BaseCharacter.BPI_BaseCharacter_C")
    (bind _characterreferences (Class|BPIBaseCharacter|IGetCharacterReferences(Message) _returnvalue))
    (Animation|PlayAnimMontage _characterreferences (CallFunction|GetCorrectAnimMontage _output_get) 1.0 "None")
    (Variables|Default|SetIsAttacking true)
    (Variables|Default|SetCanContinue false)))

(fn GetCorrectAnimMontage
  (params (Action :type E_Action%20Enum :default "NewEnumerator0"))
  (switch Utilities|FlowControl|Switch|SwitchonE_Action Action
    (:NewEnumerator0
      (return (Variables|Montage|GetAM_Punch)))
    (:NewEnumerator1
      (return (Variables|Montage|GetAM_Punch_2)))
    (:NewEnumerator2
      (return (Variables|Montage|GetAM_Punch_3)))
    (:NewEnumerator3
      (return (Variables|Montage|GetAM_Action_With_Weapon_1)))
    (:NewEnumerator4
      (return (Variables|Montage|GetAM_Action_With_Weapon_2)))
    (:NewEnumerator5
      (return (Variables|Montage|GetAM_Action_With_Weapon_3)))
    (:NewEnumerator6
      (return (Variables|Montage|GetAM_Action_With_Weapon_4)))
    (:NewEnumerator7
      (return (Variables|Montage|GetAM_Action_With_Weapon_5)))
    (:NewEnumerator13
      (return (Variables|Montage|GetAM_Action_With_Kick)))
    (:NewEnumerator14
      (return (Variables|Montage|GetAM_Action_With_Kick_2)))
    (:NewEnumerator15
      (return (Variables|Montage|GetAM_Action_With_Kick_3)))
    (:NewEnumerator16
      (return (Variables|Montage|GetAM_Action_With_Magic)))
    (:NewEnumerator17
      (return (Variables|Montage|GetAM_Action_With_Magic_2)))
    (:NewEnumerator18
      (return (Variables|Montage|GetAM_Action_With_Magic_3)))
    (:NewEnumerator19
      (return (Variables|Montage|GetAM_Action_With_Magic_4)))))

(fn ContinueAttack
  (params (Action :type E_Action%20Enum :default "NewEnumerator0"))
  (Variables|Default|SetCanContinue true)
  (if (Variables|Default|GetHasAttack)
    (CallFunction|RequestAttack Action)
    (Variables|Default|SetHasAttack false)))

(fn TraceHitDoDamage
  (params (Side :type E_SideAttack%20Enum :default "NewEnumerator0"))
  (bind (_startsocket _endsocket) (CallFunction|GetHitSocketLocation Side))
  (bind _returnvalue (Components|GetOwner))
  (bind _outhits (Collision|MultiSphereTraceForObjects _startsocket _endsocket 5e+01 (Variables|Default|GetTraceHitObjectType) false 0 "ForOneFrame"))
  (for _array_element _outhits
    (if (.bBlockingHit (Collision|BreakHitResult _array_element))
      (if (not (Utilities|Array|ContainsItem (Variables|Default|GetAllTraceHitActor) (.HitActor (Collision|BreakHitResult _array_element))))
        (Rendering|Debug|DrawDebugSphere (.ImpactPoint (Collision|BreakHitResult _array_element)) 2e+01 12 "(R=1.000000,G=1.000000,B=1.000000,A=1.000000)" 2.0 1.0)
        (Utilities|Array|Add (Variables|Default|GetAllTraceHitActor) (.HitActor (Collision|BreakHitResult _array_element)))
        (if (Utilities|DoesObjectImplementInterface _returnvalue "/Game/Blueprints/Interface/BPI_BaseCharacter.BPI_BaseCharacter_C")
          (bind _controllerreferences (Class|BPIBaseCharacter|IGetControllerReferences(Message) _returnvalue))
          (bind _newdamage (CallFunction|CalculatorDamagebyAction (Variables|Default|GetCurrentAction)))
          (Game|Damage|ApplyPointDamage (.HitActor (Collision|BreakHitResult _array_element)) _newdamage (Math|Vector|GetUnitDirection(Vector) (Transformation|GetActorLocation _controllerreferences) (Transformation|GetActorLocation (.HitActor (Collision|BreakHitResult _array_element)))) _array_element _controllerreferences _returnvalue))))))

(fn GetHitSocketLocation
  (params (SideAttack :type E_SideAttack%20Enum :default "NewEnumerator0"))
  (bind _returnvalue (Components|GetOwner))
  (if (Utilities|DoesObjectImplementInterface _returnvalue "/Game/Blueprints/Interface/BPI_BaseCharacter.BPI_BaseCharacter_C")
    (bind _meshreferences (Class|BPIBaseCharacter|IGetSkeletonMeshReferences(Message) _returnvalue))
    (switch Utilities|FlowControl|Switch|SwitchonE_SideAttack SideAttack
      (:NewEnumerator0
        (return (Transformation|GetSocketLocation _meshreferences (Variables|Socket|GetFirstSocketStart)) (Transformation|GetSocketLocation _meshreferences (Variables|Socket|GetFirstSocketEnd))))
      (:NewEnumerator1
        (return (Transformation|GetSocketLocation _meshreferences (Variables|Socket|GetSecondSocketStart)) (Transformation|GetSocketLocation _meshreferences (Variables|Socket|GetSecondSocketEnd)))))))

(fn CalculatorDamagebyAction
  (params (Action :type E_Action%20Enum :default "NewEnumerator0"))
  (switch Utilities|FlowControl|Switch|SwitchonE_Action Action
    (:NewEnumerator0
      _)
    (:NewEnumerator1
      _)
    (:NewEnumerator2
      _)
    (:NewEnumerator3
      (bind _newdamage (CallFunction|ReduceDamage (Variables|Damage|GetWeaponDamageReduce) :!label _label))
      (return _newdamage))
    (:NewEnumerator4
      (goto _label))
    (:NewEnumerator5
      (goto _label))
    (:NewEnumerator6
      (goto _label))
    (:NewEnumerator7
      (goto _label))
    (:NewEnumerator13
      (bind _newdamage_2 (CallFunction|ReduceDamage (Variables|Damage|GetKickDamageReduce) :!label _label_2))
      (return _newdamage_2))
    (:NewEnumerator14
      (goto _label_2))
    (:NewEnumerator15
      (goto _label_2))
    (:NewEnumerator16
      (bind _newdamage_3 (CallFunction|ReduceDamage (Variables|Damage|GetMagicDamageReduce) :!label _label_3))
      (return _newdamage_3))
    (:NewEnumerator17
      (goto _label_3))
    (:NewEnumerator18
      (goto _label_3))
    (:NewEnumerator19
      (goto _label_3)))
  (bind _newdamage_4 (CallFunction|ReduceDamage (Variables|Damage|GetPunchDamageReduce)))
  (return _newdamage_4))

(fn ReduceDamage
  (params (DamageReduce :type Float%20%28double-precision%29))
  (return (- (Variables|Damage|GetAttackDamage) (* DamageReduce (/ (Variables|Damage|GetAttackDamage) 1e+02)))))

(fn HandleTickDoDamage
  (params (Side :type E_SideAttack%20Enum :default "NewEnumerator0"))
  (CallFunction|TraceHitDoDamage Side))

(fn HandleBeginDoDamage
  (Utilities|Array|Clear (Variables|Default|GetAllTraceHitActor)))

(fn HandleEndAttack
  (Variables|Default|SetCanContinue false)
  (Variables|Default|SetIsAttacking false)
  (Variables|Default|SetHasAttack false))

(fn GetCorrectActionwithWeapons
  (return (Utilities|Array|Get(acopy) (Variables|Default|GetActionsWithWeapons) (Math|Random|RandomInteger (Math|Random|RandomIntegerinRange 0 (- (Utilities|Array|Length (Variables|Default|GetActionsWithWeapons)) 1))))))

(fn GetCorrectActionKicks
  (return (Utilities|Array|Get(acopy) (Variables|Default|GetActionsWithKicks) (Math|Random|RandomIntegerinRange 0 (- (Utilities|Array|Length (Variables|Default|GetActionsWithKicks)) 1)))))

(fn GetCorrectMagicClassbyAction
  (params (Index :type Integer))
  (switch int Index
    (:0
      (return (Variables|Magic|GetM_Action_Magic)))
    (:1
      (return (Variables|Magic|GetM_Action_Magic_2)))
    (:2
      (return (Variables|Magic|GetM_Action_Magic_3)))
    (:3
      (return (Variables|Magic|GetM_Action_Magic_4)))))

(fn GetCorrectActionMagics
  (bind _actionwithmagics (Variables|Default|GetActionWithMagics))
  (bind _returnvalue (Utilities|Array|Length _actionwithmagics))
  (bind _returnvalue_2 (- _returnvalue 1))
  (bind _returnvalue_3 (Math|Random|RandomIntegerinRange 0 _returnvalue_2))
  (return (Utilities|Array|Get(acopy) (Variables|Default|GetActionWithMagics) _returnvalue_3) _returnvalue_3))

(fn GetCorrectActionPunchs
  (return (Utilities|Array|Get(acopy) (Variables|Default|GetActionWithPunchs) (Math|Random|RandomIntegerinRange 0 (- (Utilities|Array|Length (Variables|Default|GetActionWithPunchs)) 1)))))

(fn SpawnMagicBeam
  (params (SpawnTransform :type Transform))
  (bind (_actions _indexselected) (CallFunction|GetCorrectActionMagics))
  (bind _returnvalue (Components|GetOwner))
  (if (Utilities|DoesObjectImplementInterface _returnvalue "/Game/Blueprints/Interface/BPI_BaseCharacter.BPI_BaseCharacter_C")
    (bind _characterreferences (Class|BPIBaseCharacter|IGetCharacterReferences(Message) _returnvalue))
    (bind _magicclass (CallFunction|GetCorrectMagicClassbyAction _indexselected))
    (bind _returnvalue_2 (Game|SpawnActorfromClass _magicclass SpawnTransform "AlwaysSpawn" "MultiplyWithRoot" _characterreferences 5e+02 0.0 0 _characterreferences))
    (bind _newdamage (CallFunction|CalculatorDamagebyAction _actions))
    (Variables|/Game/Blueprints/Magics/BP_Base_Magic.BP_Base_Magic_C|SetDamage _returnvalue_2 _newdamage)))

(fn InitDamage
  (params (AttackDamage :type Float%20%28double-precision%29) (WeaponReducePercent :type Float%20%28double-precision%29) (PunchReducePercrnt :type Float%20%28double-precision%29) (KickReducePercent :type Float%20%28double-precision%29) (MagicReducePercent :type Float%20%28double-precision%29))
  (Variables|Damage|SetAttackDamage AttackDamage)
  (Variables|Damage|SetWeaponDamageReduce WeaponReducePercent)
  (Variables|Damage|SetPunchDamageReduce PunchReducePercrnt)
  (Variables|Damage|SetKickDamageReduce KickReducePercent)
  (Variables|Damage|SetMagicDamageReduce MagicReducePercent))

(fn IGetRandomActionAttack
  (for _array_element (Variables|Default|GetActionsWithWeapons)
    (Utilities|Array|Add (LocalVariables|GetAllAction) _array_element))
  (for _array_element_2 (Variables|Default|GetActionWithMagics)
    (Utilities|Array|Add (LocalVariables|GetAllAction) _array_element_2))
  (for _array_element_3 (Variables|Default|GetActionWithPunchs)
    (Utilities|Array|Add (LocalVariables|GetAllAction) _array_element_3))
  (return (Utilities|Array|Get(acopy) (LocalVariables|GetAllAction) (Math|Random|RandomIntegerinRange 0 (- (Utilities|Array|Length (LocalVariables|GetAllAction)) 1)))))

(fn RequestBlock
  (bind _returnvalue (Components|GetOwner))
  (if (Utilities|DoesObjectImplementInterface _returnvalue "/Game/Blueprints/Interface/BPI_BaseCharacter.BPI_BaseCharacter_C")
    (bind _characterreferences (Class|BPIBaseCharacter|IGetCharacterReferences(Message) _returnvalue))
    (Animation|PlayAnimMontage _characterreferences (Variables|Montage|GetAM_ShieldBlock) 1.0 "None")))