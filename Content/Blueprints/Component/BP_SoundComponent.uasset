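; BP_SoundComponent is a component that plays pain and hit sounds on its owner when a character damages it.
; PlaySoundByAction casts the damage causer to Base_Character and gets the owner's skeletal mesh through the BPI_BaseCharacter interface.
; It plays a pain sound at the pain socket, then switches on the attacker's current action to play a punch, weapon, kick or magic impact sound at the body socket.
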(fn PlaySoundbyAction
  (params (Damage%20Causer :type Actor%20Object%20Reference))
  (bind _returnvalue (Components|GetOwner))
  (bind _asbase_character (Utilities|Casting|CastToBase_Character Damage%20Causer))
  (if (Utilities|DoesObjectImplementInterface _returnvalue "/Game/Blueprints/Interface/BPI_BaseCharacter.BPI_BaseCharacter_C")
    (bind _meshreferences (Class|BPIBaseCharacter|IGetSkeletonMeshReferences(Message) _returnvalue))
    (Audio|PlaySoundatLocation (Variables|Default|GetPainSound) (Transformation|GetSocketLocation _meshreferences (Variables|Default|GetPainSocket)) "0, 0, 0" 1.0 1.0 0.0 0 0 0 0)
    (switch Utilities|FlowControl|Switch|SwitchonE_Action (Variables|/Game/Blueprints/Component/BP_AttackComponent.BP_AttackComponent_C|GetCurrentAction (Variables|/Game/Blueprints/Characters/Base_Character.Base_Character_C|GetBP_AttackComponent _asbase_character))
      (:NewEnumerator0
        (Audio|PlaySoundatLocation (Variables|Default|GetDamageByPunch) (Transformation|GetSocketLocation _meshreferences (Variables|Default|GetBodySocket)) "0, 0, 0" 1.0 1.0 0.0 0 0 0 0 :!label _label))
      (:NewEnumerator1
        (goto _label))
      (:NewEnumerator2
        (goto _label))
      (:NewEnumerator3
        (Audio|PlaySoundatLocation (Variables|Default|GetDamageByWeapon) (Transformation|GetSocketLocation _meshreferences (Variables|Default|GetBodySocket)) "0, 0, 0" 1.0 1.0 0.0 0 0 0 0 :!label _label_2))
      (:NewEnumerator4
        (goto _label_2))
      (:NewEnumerator5
        (goto _label_2))
      (:NewEnumerator6
        (goto _label_2))
      (:NewEnumerator7
        (goto _label_2))
      (:NewEnumerator13
        (Audio|PlaySoundatLocation (Variables|Default|GetDamageByKick) (Transformation|GetSocketLocation _meshreferences (Variables|Default|GetBodySocket)) "0, 0, 0" 1.0 1.0 0.0 0 0 0 0 :!label _label_3))
      (:NewEnumerator14
        (goto _label_3))
      (:NewEnumerator15
        (goto _label_3))
      (:NewEnumerator16
        (Audio|PlaySoundatLocation (Variables|Default|GetDamageByMagic) (Transformation|GetSocketLocation _meshreferences (Variables|Default|GetBodySocket)) "0, 0, 0" 1.0 1.0 0.0 0 0 0 0 :!label _label_4))
      (:NewEnumerator17
        (goto _label_4))
      (:NewEnumerator18
        (goto _label_4))
      (:NewEnumerator19
        (goto _label_4)))))