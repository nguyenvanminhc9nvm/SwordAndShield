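; Hit component that plays hit reaction montages and impact particles on characters implementing BPI_BaseCharacter.
; HandleHitImpact spawns a shield-block effect at the damage causer's shield socket on blocks, otherwise plays a montage and spawns an effect at the hit location.
; GetCorrectHitReactMontage picks front, back or side reactions from the dot product of facing and hit direction.
; Left and right hits share one side montage, despite a cross-product check.
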(event EventBeginPlay)

(event EventTick
  (params (DeltaSeconds :type Float%20%28single-precision%29)))

(fn GetCorrectHitReactMontage
  (params (HitDirection :type Vector))
  (bind _returnvalue (Components|GetOwner))
  (if (Utilities|DoesObjectImplementInterface _returnvalue "/Game/Blueprints/Interface/BPI_BaseCharacter.BPI_BaseCharacter_C")
    (bind _characterreferences (Class|BPIBaseCharacter|IGetCharacterReferences(Message) _returnvalue))
    (if (> (Math|Float|Absolute(Float) (Math|Vector|DotProduct (Transformation|GetActorForwardVector _characterreferences) HitDirection)) 0.5)
      (if (> (Math|Vector|DotProduct (Transformation|GetActorForwardVector _characterreferences) HitDirection) 0.0)
        (return (Variables|Default|GetAM_HIt_ReactBack))
        (else
          (return (Variables|Default|GetAM_Hit_ReactFront))))
      (else
        (if (> (.z (Math|Vector|CrossProduct HitDirection (Transformation|GetActorForwardVector _characterreferences))) 0.0)
          _
          (else
            _))
        (return (Variables|Default|GetAM_Hit_ReactSide))))))

(fn HandleHitImpact
  (params (HitDirection :type Vector) (HitLocation :type Vector) (IsBlock :type Boolean) (DamageCauser :type Actor%20Object%20Reference))
  (bind _returnvalue (Components|GetOwner))
  (if IsBlock
    (bind _asbase_character (Utilities|Casting|CastToBase_Character DamageCauser))
    (Effects|SpawnEmitteratLocation (Variables|Default|GetShieldBlockImpact) (Transformation|GetSocketLocation (Variables|/Script/Engine.Character|GetMesh _asbase_character) (Default|GetCorrectShieldSocketName _asbase_character)))
    (elif (Utilities|DoesObjectImplementInterface _returnvalue "/Game/Blueprints/Interface/BPI_BaseCharacter.BPI_BaseCharacter_C")
      (bind _characterreferences (Class|BPIBaseCharacter|IGetCharacterReferences(Message) _returnvalue))
      (Animation|PlayAnimMontage _characterreferences (CallFunction|GetCorrectHitReactMontage HitDirection) 1.0 "None")
      (Effects|SpawnEmitteratLocation (Variables|Default|GetHitImpact) HitLocation))))