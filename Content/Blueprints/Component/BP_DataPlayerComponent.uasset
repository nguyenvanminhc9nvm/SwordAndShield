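; BP_DataPlayerComponent is an actor component that manages the player's saved data and power-up progression.
; On BeginPlay it loads the save slot, or creates a new save object, and pushes it to the owner through BPI_BaseCharacter.
; PowerUp plays a sound and montage, updates the save data, resends it to the owner and writes it to the slot.
; A separate function deletes the save slot.
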(event EventBeginPlay
  (CallFunction|LoadInfoPlayerfromSaveGame))

(event EventTick
  (params (DeltaSeconds :type Float%20%28single-precision%29)))

(fn LoadInfoPlayerfromSaveGame
  (bind _returnvalue (Components|GetOwner))
  (bind _returnvalue_2 (SaveGame|DoesSaveGameExist (Variables|Default|GetSlotname) (Variables|Default|GetUser%20Index)))
  (if _returnvalue_2
    (bind _returnvalue_3 (SaveGame|LoadGamefromSlot (Variables|Default|GetSlotname) (Variables|Default|GetUser%20Index)))
    (bind _asbp_base_save_game (Utilities|Casting|CastToBP_BaseSaveGame _returnvalue_3))
    (Variables|Default|SetSG_SaveGameObject _asbp_base_save_game)
    (else
      (bind _returnvalue_4 (SaveGame|CreateSaveGameObject (Variables|Default|GetSG_SaveGame)))
      (Variables|Default|SetSG_SaveGameObject _returnvalue_4)))
  (if (Utilities|DoesObjectImplementInterface _returnvalue "/Game/Blueprints/Interface/BPI_BaseCharacter.BPI_BaseCharacter_C")
    (bind _sg_savegameobject (Variables|Default|GetSG_SaveGameObject)
      (:then
        (Class|BPIBaseCharacter|ISetComponentData(Message) _returnvalue _sg_savegameobject))
      (:else))))

(fn DeleteGameinSlot
  (SaveGame|DeleteGameinSlot (Variables|Default|GetSlotname) (Variables|Default|GetUser%20Index)))

(fn PowerUp
  (bind _returnvalue (Components|GetOwner))
  (if (Utilities|DoesObjectImplementInterface _returnvalue "/Game/Blueprints/Interface/BPI_BaseCharacter.BPI_BaseCharacter_C")
    (bind _characterreferences (Class|BPIBaseCharacter|IGetCharacterReferences(Message) _returnvalue))
    (Audio|PlaySoundatLocation (Variables|Default|GetSC_PowerUp) (Transformation|GetActorLocation _characterreferences) "0, 0, 0" 1.0 1.0 0.0 0 0 0 0)
    (Animation|PlayAnimMontage _characterreferences (Variables|Default|GetAM_PowerUP) 1.0 "None")
    (bind _sg_savegameobject (Variables|Default|GetSG_SaveGameObject)
      (:then
        (bind _savegame (Default|UpdateNewData _sg_savegameobject))
        (bind _output_get (Variables|Default|SetSG_SaveGameObject _savegame))
        (Class|BPIBaseCharacter|ISetComponentData(Message) _returnvalue _output_get)
        (SaveGame|SaveGametoSlot _output_get (Variables|Default|GetSlotname) (Variables|Default|GetUser%20Index)))
      (:else))))