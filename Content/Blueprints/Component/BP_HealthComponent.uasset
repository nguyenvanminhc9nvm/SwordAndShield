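; Actor component that tracks a character's health, applying damage and healing and exposing percent, alive and low-health checks.
; Damage is halved when blocked, and both paths fire the OnLossHeath dispatcher; unblocked hits also print debug text.
; Healing and death reach the owner through BPI_BaseCharacter, adding a percentage of max health (unclamped) with particle and sound effects, or playing the death montage.
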(event EventBeginPlay)

(event EventTick
  (params (DeltaSeconds :type Float%20%28single-precision%29)))

(fn GetHealthPercent
  (return (/ (Variables|Default|GetCurrentHealth) (Variables|Default|GetMaxHealth))))

(fn DoesStillAlive
  (return (> (CallFunction|GetHealthPercent) 0.0)))

(fn UpdateHealthbyDamage
  (params (Damage%20Receiver :type Float%20%28double-precision%29) (IsBlock :type Boolean))
  (if IsBlock
    (Variables|Default|SetCurrentHealth (- (Variables|Default|GetCurrentHealth) (- Damage%20Receiver (* (/ Damage%20Receiver 1e+02) 5e+01))))
    (Default|CallOnLossHeath)
    (else
      (bind _output_get (Variables|Default|SetCurrentHealth (- (Variables|Default|GetCurrentHealth) Damage%20Receiver)))
      (Development|PrintString (Utilities|String|Append "Actor: " (Utilities|GetDisplayName (Components|GetOwner)) " Receiver Damage: " (Utilities|String|ToString(Float) (- (Variables|Default|GetCurrentHealth) Damage%20Receiver)) " Currenthealth After: " (Utilities|String|ToString(Float) _output_get)) true true "(R=0.000000,G=0.660000,B=1.000000,A=1.000000)" 5.0)
      (Default|CallOnLossHeath))))

(fn ChechNeedHeal
  (return (< (CallFunction|GetHealthPercent) 0.15)))

(fn Heal
  (params (UpToPercent :type Float%20%28double-precision%29))
  (bind _returnvalue (Components|GetOwner))
  (if (Utilities|DoesObjectImplementInterface _returnvalue "/Game/Blueprints/Interface/BPI_BaseCharacter.BPI_BaseCharacter_C")
    (bind _point_emitter (Class|BPIBaseCharacter|IGetLocationEmitterHealEffect(Message) _returnvalue))
    (Effects|SpawnEmitteratLocation (Variables|Default|GetEM_Heal) _point_emitter "0, 0, 0" "1.000000,1.000000,1.000000" true "AutoRelease")
    (Audio|PlaySoundatLocation (Variables|Default|GetSC_Heal) _point_emitter "0, 0, 0" 1.0 1.0 0.0 0 0 0 0)
    (if (< (Variables|Default|GetCurrentHealth) (Variables|Default|GetMaxHealth))
      (Variables|Default|SetCurrentHealth (+ (Variables|Default|GetCurrentHealth) (* (/ (Variables|Default|GetMaxHealth) 1e+02) UpToPercent))))))

(fn InitHealth
  (params (Health :type Float%20%28double-precision%29))
  (bind _output_get (Variables|Default|SetCurrentHealth Health))
  (Variables|Default|SetMaxHealth _output_get))

(fn HandleDeath
  (bind _returnvalue (Components|GetOwner))
  (if (Utilities|DoesObjectImplementInterface _returnvalue "/Game/Blueprints/Interface/BPI_BaseCharacter.BPI_BaseCharacter_C")
    (bind _characterreferences (Class|BPIBaseCharacter|IGetCharacterReferences(Message) _returnvalue))
    (Animation|PlayAnimMontage _characterreferences (Variables|Default|GetAM_Death) 1.0 "None")))