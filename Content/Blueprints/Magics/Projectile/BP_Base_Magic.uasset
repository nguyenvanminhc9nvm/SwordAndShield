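; Base magic projectile actor that flies by projectile movement, optionally toward or homing on a target.
; The construction script sets speed and gravity from variables and enables homing on the target's root component when flagged.
; At BeginPlay it ignores its instigator (or owner) for collision and aims velocity at any valid target.
; On box hit it signals impact, spawns effect and sound, applies point damage and destroys itself.
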(event OnComponentHit(Box)
  (params (HitComponent :type Primitive%20Component%20Object%20Reference) (OtherActor :type Actor%20Object%20Reference) (OtherComp :type Primitive%20Component%20Object%20Reference) (NormalImpulse :type Vector :default "0, 0, 0") (Hit :type Hit%20Result%20Structure%20%28by%20ref%29))
  (bind (_bblockinghit _binitialoverlap _time _distance _location _impactpoint _normal _impactnormal _physmat _hitactor) (Collision|BreakHitResult Hit))
  (Default|CallOnProjectileImpact OtherActor Hit)
  (Effects|SpawnEmitteratLocation (Variables|Effect|GetImpactEmitter) _impactpoint)
  (Audio|PlaySoundatLocation (Variables|Sound|GetImpactSound) _location "0, 0, 0" 1.0 1.0 0.0 0 0 0 0)
  (Game|Damage|ApplyPointDamage _hitactor (Variables|Default|GetDamage) _location Hit 0 (Components|GetOwner))
  (Actor|DestroyActor))

(event Custom|RotateToTarget
  (Variables|/Script/Engine.MovementComponent|SetVelocity (Variables|Default|GetProjectileMovement) (* (Math|Vector|GetUnitDirection(Vector) (Transformation|GetActorLocation) (Transformation|GetActorLocation (Variables|Default|GetTarget))) (Variables|ProjectileSetting|GetSpeed))))

(event EventBeginPlay
  (bind _returnvalue (Game|GetInstigator))
  (Collision|IgnoreActorwhenMoving (Variables|Default|GetBox) (select (Utilities|IsValid _returnvalue) _returnvalue (Components|GetOwner)) true)
  (Variables|Default|GetTarget
    (:then
      (CallFunction|RotatetoTarget))
    (:else)))

(fn ConstructionScript
  (bind _projectilemovement (Variables|Default|GetProjectileMovement))
  (bind _speed (Variables|ProjectileSetting|GetSpeed))
  (Variables|/Script/Engine.ProjectileMovementComponent|SetInitialSpeed _projectilemovement _speed)
  (Variables|/Script/Engine.ProjectileMovementComponent|SetMaxSpeed _projectilemovement _speed)
  (Variables|/Script/Engine.ProjectileMovementComponent|SetProjectileGravityScale _projectilemovement (Variables|ProjectileSetting|GetGravity))
  (bind _target (Variables|Default|GetTarget)
    (:then
      (if (Variables|Default|GetisHoming)
        (Variables|/Script/Engine.ProjectileMovementComponent|SetbIsHomingProjectile _projectilemovement true)
        (Variables|/Script/Engine.ProjectileMovementComponent|SetHomingTargetComponent _projectilemovement (Variables|/Script/Engine.Actor|GetRootComponent _target))))
    (:else)))