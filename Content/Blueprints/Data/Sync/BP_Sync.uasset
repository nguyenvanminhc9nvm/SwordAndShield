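; BP_Sync converts game data between Firebase Firestore JSON and Blueprint structs for users, characters, weapons, matches and rankings.
; VaRest decodes responses, and nested parsers unwrap typed fields into structs and enums, including master weapon lists.
; Converters build Firestore JSON by string concatenation, storing booleans as doubles.
; SyncFirebaseToSaveGame writes the first returned user into SG_GameData's local save, and GetDocumentID finds a document ID by email.
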(fn ToContent
  (params (VaRestRequest :type Va%20Rest%20Request%20JSON%20Object%20Reference))
  (bind _returnvalue (Class|VaRestRequestJSON|GetResponseContentasString VaRestRequest true))
  (bind _returnvalue_2 (Class|VaRestSubsystem|DecodeJsonObject (|VaRestSubsystem) (Utilities|String|Append "{ 
\"data\" :" _returnvalue "}")))
  (if (Utilities|Array|IsNotEmpty (Class|VaRestJsonObject|GetObjectArrayField _returnvalue_2 "data"))
    (return (Class|VaRestJsonObject|GetObjectField (Class|VaRestJsonObject|GetObjectField (Utilities|Array|Get(acopy) (Class|VaRestJsonObject|GetObjectArrayField _returnvalue_2 "data")) "document") "fields"))
    (else
      (return 0))))

(fn ToStringField
  (params (JsonObject :type Va%20Rest%20Json%20Object%20Object%20Reference) (objectName :type String) (fields :type String))
  (bind _returnvalue (Class|VaRestJsonObject|GetObjectField JsonObject objectName))
  (if (Class|VaRestJsonObject|HasField JsonObject objectName)
    (if (Class|VaRestJsonObject|HasField _returnvalue fields)
      (return (Class|VaRestJsonObject|GetStringField _returnvalue fields))
      (else
        (return "")))
    (else
      (return ""))))

(fn IsActive
  (params (Value :type Float%20%28double-precision%29))
  (if (== Value 1.0)
    (return true)
    (else
      (return false))))

(fn ToResultMatch
  (params (String :type String))
  (switch string String
    (:Win
      (return "NewEnumerator0"))
    (:Loss
      (return "NewEnumerator1"))
    (:Disconnected
      (return "NewEnumerator2"))))

(fn ToPhaseGame
  (params (Phase :type String))
  (bind _enumvalue (|ForEachE_PhaseGame)
    (:LoopBody
      (if (Utilities|Enum|Equal(Enum) Phase (Utilities|String|EnumtoString _enumvalue))
        (LocalVariables|SetPhaseSelected _enumvalue)))
    (:then
      (return (LocalVariables|GetPhaseSelected)))))

(fn ToActive
  (params (IsActive :type Boolean))
  (if IsActive
    (return 1.0)
    (else
      (return 0.0))))

(fn ToNumberField
  (params (JsonObject :type Va%20Rest%20Json%20Object%20Object%20Reference) (objectName :type String))
  (return (Class|VaRestJsonObject|GetNumberField (Class|VaRestJsonObject|GetObjectField JsonObject objectName) "doubleValue")))

(fn ParseJsonArrayWeapontoListStruct
  (params (JsonObject :type Va%20Rest%20Json%20Object%20Object%20Reference))
  (bind _returnvalue (Class|VaRestJsonObject|GetObjectField JsonObject "weapon_purchased"))
  (bind _returnvalue_2 (Class|VaRestJsonObject|GetObjectField _returnvalue "arrayValue"))
  (if (Class|VaRestJsonObject|HasField _returnvalue_2 "values")
    (for _array_element (Class|VaRestJsonObject|GetObjectArrayField _returnvalue_2 "values")
      (Utilities|Array|Add (LocalVariables|GetListWeaponLocal) (JsonToStruct|ParseJsonObjtoWeaponStruct (Class|VaRestJsonObject|GetObjectField (Class|VaRestJsonObject|GetObjectField _array_element "mapValue") "fields"))))
    (return (LocalVariables|GetListWeaponLocal))
    (else
      (return 0))))

(fn ParseJsonObjtoMatchStruct
  (params (JsonObject :type Va%20Rest%20Json%20Object%20Object%20Reference))
  (return (Utilities|Struct|MakeBP_STR_MatchAnalytics (Extension|ToResultMatch (Extension|ToStringField JsonObject "result" "stringValue")) (Extension|ToNumberField JsonObject "damage_dealt") (Extension|ToNumberField JsonObject "damage_taken") (Extension|ToPhaseGame (Extension|ToStringField JsonObject "max_phase" "stringValue")) (Extension|ToNumberField JsonObject "match_date") (Math|Float|Truncate (Extension|ToNumberField JsonObject "death")) (Math|Float|Truncate (Extension|ToNumberField JsonObject "boss_defeated")) (Extension|ToNumberField JsonObject "complete_time"))))

(fn ParseJsonObjtoPlayerStruct
  (params (JsonObject :type Va%20Rest%20Json%20Object%20Object%20Reference))
  (return (Utilities|Struct|MakeBP_STR_PlayerCharacter (Extension|ToCharacterName (Extension|ToStringField JsonObject "character_name" "stringValue")) (Math|Float|Truncate (Extension|ToNumberField JsonObject "level")) (Extension|ToNumberField JsonObject "health") (Extension|ToNumberField JsonObject "stamina_reduce_when_attack") (Extension|ToNumberField JsonObject "stamina") (JsonToStruct|ParseJsonObjtoWeaponStruct (Class|VaRestJsonObject|GetObjectField (Class|VaRestJsonObject|GetObjectField (Class|VaRestJsonObject|GetObjectField JsonObject "activate_sword") "mapValue") "fields")) (JsonToStruct|ParseJsonObjtoWeaponStruct (Class|VaRestJsonObject|GetObjectField (Class|VaRestJsonObject|GetObjectField (Class|VaRestJsonObject|GetObjectField JsonObject "activate_axe") "mapValue") "fields")) (JsonToStruct|ParseJsonObjtoWeaponStruct (Class|VaRestJsonObject|GetObjectField (Class|VaRestJsonObject|GetObjectField (Class|VaRestJsonObject|GetObjectField JsonObject "activate_shield") "mapValue") "fields")) (Extension|ToStringField JsonObject "credit" "stringValue") (Extension|ToStringField JsonObject "license" "stringValue") (JsonToStruct|ParseJsonObjtoMatchStruct (Class|VaRestJsonObject|GetObjectField (Class|VaRestJsonObject|GetObjectField (Class|VaRestJsonObject|GetObjectField JsonObject "match_analytics") "mapValue") "fields")) (Extension|IsActive (Extension|ToNumberField JsonObject "is_active")) (Math|Float|Truncate (Extension|ToNumberField JsonObject "max_level")) (Extension|ToNumberField JsonObject "max_health") (Extension|ToNumberField JsonObject "max_stamina") (Extension|ToTypeEquip (Extension|ToStringField JsonObject "type_equip" "stringValue")))))

(fn ParseJsonObjtoWeaponStruct
  (params (InputPin :type Va%20Rest%20Json%20Object%20Object%20Reference))
  (return (Utilities|Struct|MakeBP_STR_Weapon (Extension|ToStringField InputPin "weapon_name" "stringValue") (Extension|ToStringField InputPin "credit" "stringValue") (Extension|ToStringField InputPin "license" "stringValue") (Extension|ToNumberField InputPin "damage") (Math|Float|Truncate (Extension|ToNumberField InputPin "level")) (Extension|IsActive (Extension|ToNumberField InputPin "is_active")) (Math|Float|Truncate (Extension|ToNumberField InputPin "level_max")) (Extension|ToNumberField InputPin "max_damage"))))

(fn ParseJsonObjtoUserStruct
  (params (JsonObject :type Va%20Rest%20Json%20Object%20Object%20Reference))
  (return (Utilities|Struct|MakeBP_STR_User (Extension|ToStringField JsonObject "username" "stringValue") (Extension|ToStringField JsonObject "password" "stringValue") (Extension|ToStringField JsonObject "email" "stringValue") (Extension|FromAvatar (Extension|ToStringField JsonObject "avatar" "stringValue")) (Math|Float|Truncate (Extension|ToNumberField JsonObject "age")) (JsonToStruct|ParseJsonArrayWeapontoListStruct JsonObject) (JsonToStruct|ParseJsonArrayPlayertoListStruct JsonObject) (Math|Float|Truncate (Extension|ToNumberField JsonObject "g_coin")) (JsonToStruct|PhaseJsontoRankingStruct (Class|VaRestJsonObject|GetObjectField (Class|VaRestJsonObject|GetObjectField (Class|VaRestJsonObject|GetObjectField JsonObject "ranking") "mapValue") "fields")))))

(fn ParseJsonArrayPlayertoListStruct
  (params (JsonObject :type Va%20Rest%20Json%20Object%20Object%20Reference))
  (for _array_element (Class|VaRestJsonObject|GetObjectArrayField (Class|VaRestJsonObject|GetObjectField (Class|VaRestJsonObject|GetObjectField JsonObject "player_purchased") "arrayValue") "values")
    (Utilities|Array|Add (LocalVariables|GetListPlayerLocal) (JsonToStruct|ParseJsonObjtoPlayerStruct (Class|VaRestJsonObject|GetObjectField (Class|VaRestJsonObject|GetObjectField _array_element "mapValue") "fields"))))
  (return (LocalVariables|GetListPlayerLocal)))

(fn ToCharacterName
  (params (Name :type String))
  (bind _enumvalue (|ForEachE_CharacterName)
    (:LoopBody
      (if (Utilities|Enum|Equal(Enum) Name (Utilities|String|EnumtoString _enumvalue))
        (LocalVariables|SetCharacterName _enumvalue)))
    (:then
      (return (LocalVariables|GetCharacterName)))))

(fn FromAvatar
  (params (Name :type String))
  (bind _enumvalue (|ForEachE_Avatar)
    (:LoopBody
      (if (Utilities|Enum|Equal(Enum) Name (Utilities|String|EnumtoString _enumvalue))
        (LocalVariables|SetAvatarSelected _enumvalue)))
    (:then
      (return (LocalVariables|GetAvatarSelected)))))

(fn PhaseJsontoRankingStruct
  (params (JsonObject :type Va%20Rest%20Json%20Object%20Object%20Reference))
  (return (Utilities|Struct|MakeBP_STR_Ranking (Math|Float|Truncate (Extension|ToNumberField JsonObject "total_match")) (Math|Float|Truncate (Extension|ToNumberField JsonObject "win")) (Math|Float|Truncate (Extension|ToNumberField JsonObject "loss")) (Math|Float|Truncate (Extension|ToNumberField JsonObject "best_completion_time")) (Math|Float|Truncate (Extension|ToNumberField JsonObject "total_boss_defeated")) (Math|Float|Truncate (Extension|ToNumberField JsonObject "total_damage_taken")) (Math|Float|Truncate (Extension|ToNumberField JsonObject "total_damage_dealt")))))

(fn ConvertUserStructtoJsonString
  (params (User :type BP%20STR%20User%20Structure))
  (bind (_username _password _email _avatar _age _weaponpurchased _characterpurchased _gcoin _ranking _createdat) (Utilities|Struct|BreakBP_STR_User User))
  (return (Utilities|String|Append "{
  \"fields\": {
    \"email\": { \"stringValue\": \"" _email "\" },
    \"password\": { \"stringValue\": \"" _password "\" },
    \"username\": { \"stringValue\": \"" _username "\" },
    \"age\": { \"doubleValue\": " (Utilities|String|ToString(Integer) _age) " },
    \"g_coin\": { \"doubleValue\": " (Utilities|String|ToString(Integer) _gcoin) " },
    \"created_at\": { \"doubleValue\": " (Utilities|String|ToString(Float) _createdat) " },
    \"avatar\": { \"stringValue\": \"" (Utilities|String|EnumtoString _avatar) "\" },
    \"ranking\": { 
      \"mapValue\": {
        
      " (StructToJson|ConvertRankingStructtoJsonString _ranking) "}
    },
    \"weapon_purchased\": {
      \"arrayValue\": {
        \"values\": [" (StructToJson|ConvertListWeaponStructtoJsonString _weaponpurchased) "]
      }
    },
    \"player_purchased\": {
      \"arrayValue\": {
        \"values\": [
          
       " (StructToJson|ConvertListPlayerStructtoJsonString _characterpurchased) " ]
      }
    }
  }
}")))

(fn ConvertWeaponStructtoJsonString
  (params (Weapon :type BP%20STR%20Weapon%20Structure))
  (bind (_weaponname _credit _license _damage _level _isactive _levelmax _maxdamage) (Utilities|Struct|BreakBP_STR_Weapon Weapon))
  (return (Utilities|String|Append "\"fields\": {" (Utilities|String|Append "\"weapon_name\": { \"stringValue\": \"" _weaponname "\" },
    \"credit\": { \"stringValue\": \"" _credit "\" },
    \"license\": { \"stringValue\":  \"" _license "\"},
    \"damage\": { \"doubleValue\": " (Utilities|String|ToString(Float) _damage) " },
    \"level\": { \"doubleValue\":  " (Utilities|String|ToString(Integer) _level) "},
    \"is_active\": { \"doubleValue\":  " (Utilities|String|ToString(Float) (Extension|ToActive _isactive)) "},
    \"level_max\": { \"doubleValue\":  " (Utilities|String|ToString(Integer) _levelmax) "},
    \"max_damage\": { \"doubleValue\":  " (Utilities|String|ToString(Float) _maxdamage) "}") "}")))

(fn ConvertPlayerStructtoJsonString
  (params (Player :type BP%20STR%20Player%20Character%20Structure))
  (bind (_charactername _level _health _staminareducewhenattackpercent _stamina _activatesword _activateaxe _activateshield _credit _license _matchanalytics _isactive _maxlevel _maxhealth _maxstamina _typeequip) (Utilities|Struct|BreakBP_STR_PlayerCharacter Player))
  (return (Utilities|String|Append (Utilities|String|Append "\"fields\": {
    \"character_name\": { \"stringValue\": \"" (Utilities|String|EnumtoString _charactername) "\"},
    \"level\": { \"doubleValue\": " (Utilities|String|ToString(Integer) _level) " },
    \"health\": { \"doubleValue\":  " (Utilities|String|ToString(Float) _health) "},
    \"stamina_reduce_when_attack\": { \"doubleValue\":  " (Utilities|String|ToString(Float) _staminareducewhenattackpercent) "},
    \"stamina\": { \"doubleValue\": " (Utilities|String|ToString(Float) _stamina) " },
    \"credit\": { \"stringValue\": \"" _credit "\"},
    \"license\": { \"stringValue\": \"" _license "\"},
    \"match_analytics\": {
      \"mapValue\": {
        
      " (StructToJson|ConvertMatchStructtoJsonString _matchanalytics) "}
    },
    \"is_active\": { \"doubleValue\":" (Utilities|String|ToString(Float) (Extension|ToActive _isactive)) " },
    \"activate_sword\": { 
      \"mapValue\": {
        
      " (StructToJson|ConvertWeaponStructtoJsonString _activatesword) "}
    },
    \"activate_axe\": { 
      \"mapValue\": {
        
      " (StructToJson|ConvertWeaponStructtoJsonString _activateaxe) "}
    },
    \"activate_shield\": { 
      \"mapValue\": {
        
      " (StructToJson|ConvertWeaponStructtoJsonString _activateshield) "}") (Utilities|String|Append "" " },
    \"max_level\": { \"doubleValue\": 
   
  " (Utilities|String|ToString(Integer) _maxlevel) "},
    \"max_health\": { \"doubleValue\": 
   
  " (Utilities|String|ToString(Float) _maxhealth) "},
    \"max_stamina\": { \"doubleValue\": 
   
  " (Utilities|String|ToString(Float) _maxstamina) "},
    \"type_equip\": { \"stringValue\": \"" (Utilities|String|EnumtoString _typeequip) "\"}}"))))

(fn ConvertMatchStructtoJsonString
  (params (Match :type BP%20STR%20Match%20Analytics%20Structure))
  (bind (_result _damagedealt _damagetaken _maxphase _matchdate _deathcount _bossdefeated _completetime) (Utilities|Struct|BreakBP_STR_MatchAnalytics Match))
  (return (Utilities|String|Append "\"fields\": {" (Utilities|String|Append " \"result\": { \"stringValue\": \"" (Utilities|String|EnumtoString _result) "\" },
                                                \"damage_dealt\": { \"doubleValue\": " (Utilities|String|ToString(Float) _damagedealt) " },
                                                \"damage_taken\": { \"doubleValue\": " (Utilities|String|ToString(Float) _damagetaken) " },
                                                \"max_phase\": { \"stringValue\": \"" (Utilities|String|EnumtoString _maxphase) "\" },
                                                \"match_date\": { \"doubleValue\":" (Utilities|String|ToString(Float) _matchdate) "  },
                                                \"death\" : { \"doubleValue\": " (Utilities|String|ToString(Integer) _deathcount) " },
                                                \"boss_defeated\" : { \"doubleValue\": " (Utilities|String|ToString(Integer) _bossdefeated) " },
                                                \"complete_time\": { \"doubleValue\": " (Utilities|String|ToString(Float) _completetime) " } ") "}")))

(fn ConvertListWeaponStructtoJsonString
  (params (ListWeapon :type Array%20of%20BP%20STR%20Weapon%20Structures))
  (bind _returnvalue (Utilities|Array|LastIndex ListWeapon))
  (if (Utilities|Array|IsNotEmpty ListWeapon)
    (for (_array_element _array_index) ListWeapon
      (Development|PrintString 0 (Utilities|String|Append "Length: " "" "  LastIndex: " (Utilities|String|ToString(Integer) _returnvalue) "  CurrentIndex: " (Utilities|String|ToString(Integer) _array_index)))
      (if (== _array_index _returnvalue)
        (LocalVariables|SetResult (Utilities|String|Append (LocalVariables|GetResult) (Utilities|String|Append "{" (Utilities|String|Append "\"mapValue\": {" (StructToJson|ConvertWeaponStructtoJsonString _array_element) "}") "}")))
        (else
          (LocalVariables|SetResult (Utilities|String|Append (LocalVariables|GetResult) (Utilities|String|Append "{" (Utilities|String|Append "\"mapValue\": {" (StructToJson|ConvertWeaponStructtoJsonString _array_element) "}") "},"))))))
    (return (LocalVariables|GetResult))
    (else
      (return ""))))

(fn ConvertListPlayerStructtoJsonString
  (params (ListPlayer :type Array%20of%20BP%20STR%20Player%20Character%20Structures))
  (if (Utilities|Array|IsNotEmpty ListPlayer)
    (for (_array_element _array_index) ListPlayer
      (if (== _array_index (Utilities|Array|LastIndex ListPlayer))
        (LocalVariables|SetResult (Utilities|String|Append (LocalVariables|GetResult) (Utilities|String|Append "{" (Utilities|String|Append "\"mapValue\": {" (StructToJson|ConvertPlayerStructtoJsonString _array_element) "}") "}")))
        (else
          (LocalVariables|SetResult (Utilities|String|Append (LocalVariables|GetResult) (Utilities|String|Append "{" (Utilities|String|Append "\"mapValue\": {" (StructToJson|ConvertPlayerStructtoJsonString _array_element) "}") "},"))))))
    (return (LocalVariables|GetResult))
    (else
      (return ""))))

(fn SyncFirebasetoSaveGame
  (params (JsonObject :type Va%20Rest%20Request%20JSON%20Object%20Reference))
  (bind _returnvalue (Extension|ToContent JsonObject))
  (bind _userstruct (JsonToStruct|ParseJsonObjtoUserStruct _returnvalue))
  (bind _returnvalue_2 (SaveGame|CreateSaveGameObject "/Game/Blueprints/Data/SaveGame/SG_GameData.SG_GameData_C"))
  (bind _sg_gamedata (Default|LoadLocalGameData _returnvalue_2))
  (Variables|/Game/Blueprints/Data/SaveGame/SG_GameData.SG_GameData_C|SetUser _sg_gamedata _userstruct)
  (Default|SaveLocalGameData _returnvalue_2 _sg_gamedata))

(fn ConvertRankingStructtoJsonString
  (params (Ranking :type BP%20STR%20Ranking%20Structure))
  (bind (_totalmatch _win _loss _bestcompletiontime _totalbossdefeated _totaldamagetaken _totaldamagedealt) (Utilities|Struct|BreakBP_STR_Ranking Ranking))
  (return (Utilities|String|Append "
  \"fields\": {
    \"total_match\": { \"doubleValue\":  " (Utilities|String|ToString(Integer) _totalmatch) "},
    \"win\": { \"doubleValue\": " (Utilities|String|ToString(Integer) _win) " },
    \"loss\": { \"doubleValue\":  " (Utilities|String|ToString(Integer) _loss) "},
    \"best_completion_time\": { \"doubleValue\": " (Utilities|String|ToString(Integer) _bestcompletiontime) " },
    \"total_boss_defeated\": { \"doubleValue\": " (Utilities|String|ToString(Integer) _totalbossdefeated) " },
    \"total_damage_taken\": { \"doubleValue\": " (Utilities|String|ToString(Integer) _totaldamagetaken) " },
    \"total_damage_dealt\": { \"doubleValue\": " (Utilities|String|ToString(Integer) _totaldamagedealt) " }
  }

")))

(fn ToListContent
  (params (VaRestRequest :type Va%20Rest%20Request%20JSON%20Object%20Reference))
  (bind _returnvalue (Class|VaRestRequestJSON|GetResponseContentasString VaRestRequest true))
  (bind _returnvalue_2 (Class|VaRestSubsystem|DecodeJsonObject (|VaRestSubsystem) (Utilities|String|Append "{ 
\"data\" :" _returnvalue "}")))
  (return (Class|VaRestJsonObject|GetObjectArrayField _returnvalue_2 "data")))

(fn ParseJsonMasterWeapontoWeapon
  (params (JsonObject :type Va%20Rest%20Json%20Object%20Object%20Reference))
  (return (Utilities|Struct|MakeBP_STR_MasterWeapon (Extension|ToStringField JsonObject "credit" "stringValue") (Extension|ToStringField JsonObject "license" "stringValue") (Extension|ToStringField JsonObject "name" "stringValue") (Math|Conversions|ToInteger(Byte) (Extension|ToStringField JsonObject "price" "integerValue")) (Math|Conversions|ToInteger(Byte) (Extension|ToStringField JsonObject "max_level" "integerValue")) (Math|Conversions|ToFloat(Integer) (Extension|ToStringField JsonObject "damage" "integerValue")) (Math|Conversions|ToFloat(Integer) (Extension|ToStringField JsonObject "max_damage" "integerValue")))))

(fn FromJsontoWeaponType
  (params (JsonObj :type Va%20Rest%20Json%20Object%20Object%20Reference))
  (switch string (Class|VaRestJsonObject|GetStringField (Class|VaRestJsonObject|GetObjectField JsonObj "type") "stringValue")
    (:axe
      (return "NewEnumerator1"))
    (:sword
      (return "NewEnumerator0"))
    (:shield
      (return "NewEnumerator2"))))

(fn ParseJsonArraytoListMasterWeaponStruct
  (params (JsonObj :type Va%20Rest%20Request%20JSON%20Object%20Reference))
  (bind _returnvalue (Class|VaRestRequestJSON|GetResponseContentasString JsonObj true))
  (bind _returnvalue_2 (Class|VaRestSubsystem|DecodeJsonObject (|VaRestSubsystem) (Utilities|String|Append "{ 
\"data\" :" _returnvalue "}")))
  (for _array_element (Class|VaRestJsonObject|GetObjectArrayField (Class|VaRestJsonObject|GetObjectField _returnvalue_2 "data") "documents")
    (bind _weaponmaster (JsonToStruct|ParseJsonMasterWeapontoWeapon (Class|VaRestJsonObject|GetObjectField _array_element "fields")))
    (Utilities|Array|Add (LocalVariables|GetListMasterWeaponLocal) _weaponmaster))
  (return (LocalVariables|GetListMasterWeaponLocal)))

(fn GetDocumentID
  (params (Request :type Va%20Rest%20Request%20JSON%20Object%20Reference) (Email :type String))
  (bind _returnvalue (Class|VaRestRequestJSON|GetResponseContentasString Request true))
  (bind _returnvalue_2 (Class|VaRestSubsystem|DecodeJsonObject (|VaRestSubsystem) (Utilities|String|Append "{ 
\"data\" :" _returnvalue "}")))
  (for _array_element (Class|VaRestJsonObject|GetObjectArrayField _returnvalue_2 "data")
    (if (Utilities|Enum|Equal(Enum) (Class|VaRestJsonObject|GetStringField (Class|VaRestJsonObject|GetObjectField (Class|VaRestJsonObject|GetObjectField (Class|VaRestJsonObject|GetObjectField _array_element "document") "fields") "email") "stringValue") Email)
      (bind _output_get (LocalVariables|SetDocumentFounded _array_element))
      (Development|PrintString 0 (Utilities|String|Append "DocumentFounded: " (Class|VaRestJsonObject|GetStringField (Class|VaRestJsonObject|GetObjectField _output_get "document") "name")))))
  (Development|PrintString 0 (Utilities|String|Append "DocumentID: " (Utilities|Array|Get(acopy) (Utilities|String|ParseIntoArray (Class|VaRestJsonObject|GetStringField (Class|VaRestJsonObject|GetObjectField (LocalVariables|GetDocumentFounded) "document") "name") "/") (- (Utilities|Array|Length (Utilities|String|ParseIntoArray (Class|VaRestJsonObject|GetStringField (Class|VaRestJsonObject|GetObjectField (LocalVariables|GetDocumentFounded) "document") "name") "/")) 1))))
  (return (Utilities|Array|Get(acopy) (Utilities|String|ParseIntoArray (Class|VaRestJsonObject|GetStringField (Class|VaRestJsonObject|GetObjectField (LocalVariables|GetDocumentFounded) "document") "name") "/") (- (Utilities|Array|Length (Utilities|String|ParseIntoArray (Class|VaRestJsonObject|GetStringField (Class|VaRestJsonObject|GetObjectField (LocalVariables|GetDocumentFounded) "document") "name") "/")) 1))))

(fn ToTypeEquip
  (params (TypeEquip :type String))
  (bind _enumvalue (|ForEachE_EquipType)
    (:LoopBody
      (if (Utilities|String|Contains (Utilities|String|EnumtoString _enumvalue) TypeEquip)
        (LocalVariables|SetNewLocalVar _enumvalue)))
    (:then
      (return (LocalVariables|GetNewLocalVar)))))