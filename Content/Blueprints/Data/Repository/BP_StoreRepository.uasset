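; Store repository Blueprint that fetches master lists of swords, axes and shields from an API.
; Each getter constructs a BP_ApiService, makes the matching request and binds to its completion event.
; On completion, a new BP_Sync parses the JSON array into master weapon structs, which a per-category success dispatcher broadcasts.
; All three categories share the same parser, and no failure handling appears here.
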(event Custom|GetListMasterSword
  (bind _returnvalue (Game|ConstructObjectfromClass "/Game/Blueprints/Data/Service/BP_ApiService.BP_ApiService_C"))
  (bind _outputpin (Default|MakeRequestGetListMasterSword _returnvalue))
  (EventDispatchers|AssignOnRequestComplete _outputpin (delegate Custom|OnRequestComplete_Event)))

(event Custom|OnRequestComplete_Event
  (params (Request :type Va%20Rest%20Request%20JSON%20Object%20Reference))
  (bind _returnvalue (Game|ConstructObjectfromClass "/Game/Blueprints/Data/Sync/BP_Sync.BP_Sync_C"))
  (bind _listmasterweaponlocal1 (Default|ParseJsonArraytoListMasterWeaponStruct _returnvalue Request))
  (Default|CallOnGetListMasterSwordSuccess _listmasterweaponlocal1))

(event Custom|GetListMasterWeaponAxe
  (bind _returnvalue (Game|ConstructObjectfromClass "/Game/Blueprints/Data/Service/BP_ApiService.BP_ApiService_C"))
  (bind _outputpin (Default|MakeRequestGetListMasterAxe _returnvalue))
  (EventDispatchers|AssignOnRequestComplete _outputpin (delegate Custom|OnRequestComplete_Event_0)))

(event Custom|OnRequestComplete_Event_0
  (params (Request :type Va%20Rest%20Request%20JSON%20Object%20Reference))
  (bind _returnvalue (Game|ConstructObjectfromClass "/Game/Blueprints/Data/Sync/BP_Sync.BP_Sync_C"))
  (bind _listmasterweaponlocal1 (Default|ParseJsonArraytoListMasterWeaponStruct _returnvalue Request))
  (Default|CallOnGetListMasterAxeSuccess _listmasterweaponlocal1))

(event Custom|GetListMasterShield
  (bind _returnvalue (Game|ConstructObjectfromClass "/Game/Blueprints/Data/Service/BP_ApiService.BP_ApiService_C"))
  (bind _outputpin (Default|MakeRequestGetListMasterShield _returnvalue))
  (EventDispatchers|AssignOnRequestComplete _outputpin (delegate Custom|OnRequestComplete_Event_1)))

(event Custom|OnRequestComplete_Event_1
  (params (Request :type Va%20Rest%20Request%20JSON%20Object%20Reference))
  (bind _returnvalue (Game|ConstructObjectfromClass "/Game/Blueprints/Data/Sync/BP_Sync.BP_Sync_C"))
  (bind _listmasterweaponlocal1 (Default|ParseJsonArraytoListMasterWeaponStruct _returnvalue Request))
  (Default|CallOnGetListMasterShieldSuccess _listmasterweaponlocal1))