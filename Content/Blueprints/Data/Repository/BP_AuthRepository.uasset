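; Repository for Firebase user accounts: sign-up, login, email existence checks, user rankings and pushing local save data to the database.
; Each operation sends async requests through BP_ApiService and fires a dispatcher from the completion callback.
; Sign-up and login chain a user query by email, then BP_Sync writes the result to the save game.
; User sync looks up the document ID by saved email, then updates it from SG_GameData.
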(event Custom|SignUp
  (params (Username :type String) (Password :type String) (Email :type String) (Avatar :type E_Avatar%20Enum :default "NewEnumerator0") (Age :type Integer))
  (bind _returnvalue (Game|ConstructObjectfromClass "/Game/Blueprints/Data/Service/BP_ApiService.BP_ApiService_C"))
  (bind _outputpin (Default|MakeRequestSignUp _returnvalue Username Password Email Avatar Age))
  (EventDispatchers|AssignOnRequestComplete _outputpin (delegate Custom|OnRequestComplete_Event)))

(event Custom|OnRequestComplete_Event
  (params (Request :type Va%20Rest%20Request%20JSON%20Object%20Reference))
  (bind _returnvalue (Game|ConstructObjectfromClass "/Game/Blueprints/Data/Service/BP_ApiService.BP_ApiService_C"))
  (bind _outputpin (Default|MakeRequestQueryDatabase _returnvalue "user" "email" (stale Custom|SignUp Email)))
  (EventDispatchers|AssignOnRequestComplete _outputpin (delegate Custom|OnRequestComplete_Event_0)))

(event Custom|OnRequestComplete_Event_0
  (params (Request :type Va%20Rest%20Request%20JSON%20Object%20Reference))
  (bind _returnvalue (Game|ConstructObjectfromClass "/Game/Blueprints/Data/Sync/BP_Sync.BP_Sync_C"))
  (Default|SyncFirebasetoSaveGame _returnvalue Request)
  (Default|CallOnSignUpSuccess))

(event Custom|Login
  (params (Email :type String) (Password :type String))
  (bind _returnvalue (Game|ConstructObjectfromClass "/Game/Blueprints/Data/Service/BP_ApiService.BP_ApiService_C"))
  (bind _outputpin (Default|MakeRequestSignin _returnvalue Email Password))
  (EventDispatchers|AssignOnRequestComplete _outputpin (delegate Custom|OnRequestComplete_Event_1)))

(event Custom|OnRequestComplete_Event_1
  (params (Request :type Va%20Rest%20Request%20JSON%20Object%20Reference))
  (bind _returnvalue (Game|ConstructObjectfromClass "/Game/Blueprints/Data/Service/BP_ApiService.BP_ApiService_C"))
  (bind _outputpin (Default|MakeRequestQueryDatabase _returnvalue "user" "email" (stale Custom|Login Email)))
  (EventDispatchers|AssignOnRequestComplete _outputpin (delegate Custom|OnRequestComplete_Event_2)))

(event Custom|OnRequestComplete_Event_2
  (params (Request :type Va%20Rest%20Request%20JSON%20Object%20Reference))
  (bind _returnvalue (Game|ConstructObjectfromClass "/Game/Blueprints/Data/Sync/BP_Sync.BP_Sync_C"))
  (Default|SyncFirebasetoSaveGame _returnvalue Request)
  (Default|CallOnSigninSuccess))

(event Custom|EventCheckMailExists
  (params (Email :type String))
  (bind _returnvalue (Game|ConstructObjectfromClass "/Game/Blueprints/Data/Service/BP_ApiService.BP_ApiService_C"))
  (bind _outputpin (Default|MakeRequestCheckMailExists _returnvalue Email))
  (EventDispatchers|AssignOnRequestComplete _outputpin (delegate Custom|OnRequestComplete_Event_3)))

(event Custom|OnRequestComplete_Event_3
  (params (Request :type Va%20Rest%20Request%20JSON%20Object%20Reference))
  (bind _returnvalue (Class|VaRestRequestJSON|GetResponseContentasString Request true))
  (bind _returnvalue_2 (Class|VaRestSubsystem|DecodeJsonObject (|VaRestSubsystem) (Utilities|String|Append "{ 
\"data\" :" _returnvalue "}")))
  (if (Utilities|Array|IsNotEmpty (Class|VaRestJsonObject|GetObjectArrayField _returnvalue_2 "data"))
    (Default|CallOnCheckEmailExists (Class|VaRestJsonObject|HasField (Utilities|Array|Get(acopy) (Class|VaRestJsonObject|GetObjectArrayField _returnvalue_2 "data")) "document"))
    (else
      (Default|CallOnCheckEmailExists false))))

(event Custom|GetListRankingUser
  (params (E_Sort :type E_SortSelected%20Enum :default "NewEnumerator0"))
  (bind _returnvalue (Game|ConstructObjectfromClass "/Game/Blueprints/Data/Service/BP_ApiService.BP_ApiService_C"))
  (bind _outputpin (Default|MakeRequestGetUserRanking _returnvalue E_Sort))
  (EventDispatchers|AssignOnRequestComplete _outputpin (delegate Custom|OnRequestComplete_Event_4)))

(event Custom|OnRequestComplete_Event_4
  (params (Request :type Va%20Rest%20Request%20JSON%20Object%20Reference))
  (bind _returnvalue (Game|ConstructObjectfromClass "/Game/Blueprints/Data/Sync/BP_Sync.BP_Sync_C"))
  (bind _returnvalue_2 (Default|ToListContent _returnvalue Request))
  (for _array_element _returnvalue_2
    (bind _userstruct (Default|ParseJsonObjtoUserStruct _returnvalue (Class|VaRestJsonObject|GetObjectField (Class|VaRestJsonObject|GetObjectField _array_element "document") "fields")))
    (Utilities|Array|Add (Variables|Default|GetListUser) _userstruct))
  (Default|CallOnGetUserRankingComplete (Variables|Default|GetListUser)))

(event Custom|SyncUserData
  (bind _returnvalue (Game|ConstructObjectfromClass "/Game/Blueprints/Data/SaveGame/SG_GameData.SG_GameData_C"))
  (bind _sg_gamedata (Default|LoadLocalGameData _returnvalue))
  (bind _returnvalue_2 (Game|ConstructObjectfromClass "/Game/Blueprints/Data/Service/BP_ApiService.BP_ApiService_C"))
  (bind _outputpin (Default|MakeRequestQueryDatabase _returnvalue_2 "user" "email" (.email (Variables|/Game/Blueprints/Data/SaveGame/SG_GameData.SG_GameData_C|GetUser _sg_gamedata))))
  (EventDispatchers|AssignOnRequestComplete _outputpin (delegate Custom|OnRequestComplete_Event_5)))

(event Custom|OnRequestComplete_Event_5
  (params (Request :type Va%20Rest%20Request%20JSON%20Object%20Reference))
  (bind _returnvalue (Game|ConstructObjectfromClass "/Game/Blueprints/Data/Sync/BP_Sync.BP_Sync_C"))
  (bind _documentid (Default|GetDocumentID _returnvalue Request (.email (Variables|/Game/Blueprints/Data/SaveGame/SG_GameData.SG_GameData_C|GetUser (stale Custom|SyncUserData _sg_gamedata)))))
  (bind _returnvalue_2 (Game|ConstructObjectfromClass "/Game/Blueprints/Data/Service/BP_ApiService.BP_ApiService_C"))
  (bind _outputpin (Default|MakeRequestUpdateUser _returnvalue_2 (Default|ConvertUserStructtoJsonString _returnvalue (Variables|/Game/Blueprints/Data/SaveGame/SG_GameData.SG_GameData_C|GetUser (stale Custom|SyncUserData _sg_gamedata))) _documentid))
  (EventDispatchers|AssignOnRequestComplete _outputpin (delegate Custom|OnRequestComplete_Event_6)))

(event Custom|OnRequestComplete_Event_6
  (params (Request :type Va%20Rest%20Request%20JSON%20Object%20Reference))
  (Default|CallOnUpdateUserComplete))