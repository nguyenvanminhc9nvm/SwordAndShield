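; BP_ApiService is the game's Firebase REST client for sign-up, sign-in, email lookup, user updates, leaderboards and master weapon lists.
; A shared MakeRequest helper fires VaRest JSON calls and returns the request object; user updates build their own PATCH request.
; Sign-up posts a user document seeded with starter weapons, character and coins via BP_Sync.
; Email lookup and rankings use hand-built Firestore structured queries; sign-in uses Identity Toolkit.
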(fn MakeRequestSignUp
  (params (Username :type String) (Password :type String) (Email :type String) (Avatar :type E_Avatar%20Enum :default "NewEnumerator0") (Age :type Integer))
  (bind _bp_st_weapon (Utilities|Struct|MakeBP_ST_Weapon "ThunderstormShield" "Spear_11MB by Mehdi Shahsavan is licensed under Creative Commons Attribution" " Creative Commons Attribution" 0.0 1 true 1))
  (bind _bp_st_weapon_2 (Utilities|Struct|MakeBP_ST_Weapon "ThunderstormSword" "Fantasy Sword Devil May Cry by Maxim Lukyanov is licensed under Creative Commons Attribution" " Creative Commons Attribution" 1e+02 1 true 200 1e+04))
  (bind _returnvalue (Game|ConstructObjectfromClass "/Game/Blueprints/Data/Sync/BP_Sync.BP_Sync_C"))
  (bind _outputpin (CallFunction|MakeRequest (Utilities|String|Append (Variables|Default|GetBaseUrl) (Variables|Default|GetdUser) (Variables|Default|GetapiKey)) (Default|ConvertUserStructtoJsonString _returnvalue (Utilities|Struct|MakeBP_ST_User Username Password Email Avatar Age (Utilities|Array|MakeArray _bp_st_weapon_2 (Utilities|Struct|MakeBP_ST_Weapon "ThunderstormDualSword" "Assassin Sword by Shriker1 is licensed under Creative Commons Attribution" " Creative Commons Attribution" 1e+02 1 false 200 1e+04) (Utilities|Struct|MakeBP_ST_Weapon "ThunderstormAxe" "Infernal Crescent Axe by GarrettBaker is licensed under Creative Commons Attribution" " Creative Commons Attribution" 1e+02 1 false 200 1e+04) (Utilities|Struct|MakeBP_ST_Weapon "ThunderstormSpear" "Spear_11MB by Mehdi Shahsavan is licensed under Creative Commons Attribution" " Creative Commons Attribution" 1e+02 1 false 200 1e+04) _bp_st_weapon (Utilities|Struct|MakeBP_ST_Weapon "GreatThunderstormSword" "Credit the Creator
Stylized Big Sword by Agata Wilczek is licensed under Creative Commons Attribution" " Creative Commons Attribution" 1e+02 1 true 200 1e+04)) (Utilities|Array|MakeArray (Utilities|Struct|MakeBP_ST_PlayerCharacter "NewEnumerator17" 1 1e+03 1e+01 1e+03 _bp_st_weapon_2 "(WeaponName_7_E7338DA37C4433F9A0FC518698EB0A73=\"\",Credit_9_FEAC04340A4AC74CD829DF93AE651CA8=\"\",License_11_138E930AAB459C4E2069FA974076998C=\"\",Damage_13_508B3EBCD941997233B905A6E3A5B31C=0.000000,Level_15_36FDE48E3A40883D88D7CDADCAB8D8FB=0,IsActive_16_0C63B07EDF45E56086DA6797E6B016AF=False,LevelMax_21_605063CF09446D03784B90B3F58DC057=0,MaxDamage_33_4E07351F084259DC497505AFD33B853D=0.000000)" _bp_st_weapon "Mixamo" " Creative Commons Attribution" (Utilities|Struct|MakeBP_ST_MatchAnalytics "NewEnumerator2" 0.0 0.0 "NewEnumerator13") true 999 9.99e+05 9.99e+05 "NewEnumerator1")) 10000 (Utilities|Struct|MakeBP_ST_Ranking) (Math|Conversions|ToFloat(Integer) (Class|KismetMathLibrary|ToUnixTimestamp (Math|DateTime|Now))))) "POST"))
  (return _outputpin))

(fn MakeRequest
  (params (Url :type String) (param :type String) (Verb :type EVaRestRequestVerb%20Enum :default "GET"))
  (bind _returnvalue (|VaRestSubsystem))
  (Development|PrintString 0 (Utilities|String|Append "url: " Url "   params: " param) false true "(R=1.000000,G=1.000000,B=1.000000,A=1.000000)" 1e+01)
  (bind _returnvalue_2 (Class|VaRestSubsystem|DecodeJsonObject _returnvalue param))
  (bind _returnvalue_3 (Class|VaRestSubsystem|ConstructVaRestRequestExt _returnvalue Verb "json"))
  (if (Utilities|Array|IsEmpty param)
    _
    (else
      (Class|VaRestRequestJSON|SetRequestObject _returnvalue_3 _returnvalue_2)))
  (Class|VaRestRequestJSON|SetURL _returnvalue_3 Url)
  (Class|VaRestRequestJSON|ExecuteProcessRequest _returnvalue_3)
  (return _returnvalue_3))

(fn MakeRequestQueryDatabase
  (params (collectionId :type String) (fields :type String) (queryParams :type String))
  (bind _outputpin (CallFunction|MakeRequest (Utilities|String|Append "https://firestore.googleapis.com/v1/projects/sword-and-shield-5aabd/databases/(default)/documents:runQuery" (Variables|Default|GetapiKey)) (Utilities|String|Append "{
  \"structuredQuery\": {
    \"from\": [
      {
        \"collectionId\": \"" collectionId "\"
      }
    ],
    \"where\": {
      \"fieldFilter\": {
        \"field\": {
          \"fieldPath\": \"" fields "\"
        },
        \"op\": \"EQUAL\",
        \"value\": {
          \"stringValue\": \"" queryParams "\"
        }
      }
    },
    \"limit\": 1
  }
}") "POST"))
  (return _outputpin))

(fn MakeRequestSignin
  (params (Email :type String) (Password :type String))
  (bind _outputpin (CallFunction|MakeRequest (Utilities|String|Append "https://identitytoolkit.googleapis.com/v1/accounts:signInWithPassword" (Variables|Default|GetapiKey)) (Utilities|String|Append "{
    \"email\": \"" Email "\",
    \"password\": \"" Password "\",
    \"returnSecureToken\": true
}") "POST"))
  (return _outputpin))

(fn MakeRequestCheckMailExists
  (params (Email :type String))
  (bind _outputpin (CallFunction|MakeRequestQueryDatabase "user" "email" Email))
  (return _outputpin))

(fn MakeRequestGetUserRanking
  (params (E_SortSelected :type E_SortSelected%20Enum :default "NewEnumerator0"))
  (switch Utilities|FlowControl|Switch|SwitchonE_SortSelected E_SortSelected
    (:NewEnumerator0
      (bind _outputpin (CallFunction|MakeRequest (Utilities|String|Append "https://firestore.googleapis.com/v1/projects/sword-and-shield-5aabd/databases/(default)/documents:runQuery" (Variables|Default|GetapiKey)) (Utilities|String|Append "{
    \"structuredQuery\": {
        \"from\": [{
            \"collectionId\": \"user\"
        }],
        \"orderBy\": [{
            \"field\": {
                \"fieldPath\": \"ranking.win\"
            },
            \"direction\": \"DESCENDING\"
        }],
        \"limit\": 50
    }
}" "") "POST"))
      (return _outputpin))
    (:NewEnumerator1
      (bind _outputpin_2 (CallFunction|MakeRequest (Utilities|String|Append "https://firestore.googleapis.com/v1/projects/sword-and-shield-5aabd/databases/(default)/documents:runQuery" (Variables|Default|GetapiKey)) (Utilities|String|Append "{
    \"structuredQuery\": {
        \"from\": [{
            \"collectionId\": \"user\"
        }],
        \"orderBy\": [{
            \"field\": {
                \"fieldPath\": \"ranking.loss\"
            },
            \"direction\": \"ASCENDING\"
        }],
        \"limit\": 50
    }
}" "") "POST"))
      (return _outputpin_2))
    (:NewEnumerator2
      (bind _outputpin_3 (CallFunction|MakeRequest (Utilities|String|Append "https://firestore.googleapis.com/v1/projects/sword-and-shield-5aabd/databases/(default)/documents:runQuery" (Variables|Default|GetapiKey)) (Utilities|String|Append "{
    \"structuredQuery\": {
        \"from\": [{
            \"collectionId\": \"user\"
        }],
        \"orderBy\": [{
            \"field\": {
                \"fieldPath\": \"ranking.total_damage_dealt\"
            },
            \"direction\": \"DESCENDING\"
        }],
        \"limit\": 50
    }
}" "") "POST"))
      (return _outputpin_3))
    (:NewEnumerator3
      (bind _outputpin_4 (CallFunction|MakeRequest (Utilities|String|Append "https://firestore.googleapis.com/v1/projects/sword-and-shield-5aabd/databases/(default)/documents:runQuery" (Variables|Default|GetapiKey)) (Utilities|String|Append "{
    \"structuredQuery\": {
        \"from\": [{
            \"collectionId\": \"user\"
        }],
        \"orderBy\": [{
            \"field\": {
                \"fieldPath\": \"ranking.total_damage_taken\"
            },
            \"direction\": \"ASCENDING\"
        }],
        \"limit\": 50
    }
}" "") "POST"))
      (return _outputpin_4))
    (:NewEnumerator4
      (bind _outputpin_5 (CallFunction|MakeRequest (Utilities|String|Append "https://firestore.googleapis.com/v1/projects/sword-and-shield-5aabd/databases/(default)/documents:runQuery" (Variables|Default|GetapiKey)) (Utilities|String|Append "{
    \"structuredQuery\": {
        \"from\": [{
            \"collectionId\": \"user\"
        }],
        \"orderBy\": [{
            \"field\": {
                \"fieldPath\": \"ranking.best_completion_time\"
            },
            \"direction\": \"ASCENDING\"
        }],
        \"limit\": 50
    }
}" "") "POST"))
      (return _outputpin_5))))

(fn MakeRequestGetListMasterSword
  (bind _outputpin (CallFunction|MakeRequest (Utilities|String|Append (Variables|Default|GetBaseUrl) (Variables|Default|GetdMW_sword) (Variables|Default|GetapiKey)) "" "GET"))
  (return _outputpin))

(fn MakeRequestGetListMasterAxe
  (bind _outputpin (CallFunction|MakeRequest (Utilities|String|Append (Variables|Default|GetBaseUrl) (Variables|Default|GetdMW_axe) (Variables|Default|GetapiKey)) "" "GET"))
  (return _outputpin))

(fn MakeRequestGetListMasterShield
  (bind _outputpin (CallFunction|MakeRequest (Utilities|String|Append (Variables|Default|GetBaseUrl) (Variables|Default|GetdMW_shield) (Variables|Default|GetapiKey)) "" "GET"))
  (return _outputpin))

(fn MakeRequestUpdateUser
  (params (param :type String) (doucumentID :type String))
  (bind _returnvalue (|VaRestSubsystem))
  (Development|PrintString 0 param)
  (bind _returnvalue_2 (Class|VaRestSubsystem|ConstructVaRestRequestExt _returnvalue "CUSTOM" "json"))
  (bind _returnvalue_3 (Class|VaRestSubsystem|DecodeJsonObject _returnvalue param))
  (Class|VaRestRequestJSON|SetRequestObject _returnvalue_2 _returnvalue_3)
  (Class|VaRestRequestJSON|SetURL _returnvalue_2 (Utilities|String|Append (Variables|Default|GetBaseUrl) (Variables|Default|GetdUser) "/" doucumentID (Variables|Default|GetapiKey)))
  (Class|VaRestRequestJSON|SetCustomVerb _returnvalue_2 "PATCH")
  (Class|VaRestRequestJSON|ExecuteProcessRequest _returnvalue_2)
  (return _returnvalue_2))