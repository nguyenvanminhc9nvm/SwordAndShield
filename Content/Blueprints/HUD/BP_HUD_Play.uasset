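; BP_HUD_Play is the gameplay HUD that creates the WBP_PlayMain widget and acts as the bridge between game logic and UI.
; On BeginPlay it adds the widget to the viewport and binds to BP_GM_Play's phase-change dispatcher to forward phase updates.
; Exposed functions pass player health and stamina, game status, and typed notices (Warning, Error, Message) to the widget or its nested WBPPlay.
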(event Custom|OnChangePhaseGame_Event
  (params (PhaseGame :type E_PhaseGame%20Enum :default "NewEnumerator0"))
  (Default|SetPhaseGameUpdate (Variables|Default|GetWBP_PlayMain) PhaseGame))

(event EventBeginPlay
  (CallFunction|InitScreenPlay)
  (bind _asbp_gm_play (Utilities|Casting|CastToBP_GM_Play (Game|GetGameMode)))
  (bind _output_get (Variables|Default|SetAs%20BP%20GM%20Play _asbp_gm_play))
  (EventDispatchers|AssignOnChangePhaseGame _output_get (delegate Custom|OnChangePhaseGame_Event)))

(fn ConstructionScript)

(fn InitScreenPlay
  (bind _returnvalue (UserInterface|CreateWidget "/Game/UI/Screen/WBP_PlayMain.WBP_PlayMain_C"))
  (bind _output_get (Variables|Default|SetWBP_PlayMain _returnvalue))
  (Default|InitGameStatus _output_get (Variables|Default|GetGameState))
  (UserInterface|Viewport|AddtoViewport _output_get 0))

(fn LoadInfoPlayer
  (params (Health :type Float%20%28double-precision%29) (Stamina :type Float%20%28double-precision%29))
  (bind _wbp_playmain (Variables|Default|GetWBP_PlayMain)
    (:then
      (Default|LoadInfoPlayer (Variables|/Game/UI/Screen/WBP_PlayMain.WBP_PlayMain_C|GetWBP_Play _wbp_playmain) Health Stamina))
    (:else)))

(fn InitGameStatus
  (params (GameStatus :type E_GamePlayState%20Enum :default "NewEnumerator0"))
  (bind _wbp_playmain (Variables|Default|GetWBP_PlayMain)
    (:then
      (Default|InitGameStatus _wbp_playmain GameStatus))
    (:else)))

(fn DisplayNotice
  (params (AlertType :type E_AlertType%20Enum :default "NewEnumerator0") (Message :type String))
  (bind _wbp_playmain (Variables|Default|GetWBP_PlayMain))
  (bind _wbp_play (Variables|/Game/UI/Screen/WBP_PlayMain.WBP_PlayMain_C|GetWBP_Play _wbp_playmain))
  (switch Utilities|FlowControl|Switch|SwitchonE_AlertType AlertType
    (:NewEnumerator0
      (Default|NoticeNotEnoughStamina _wbp_play Message))
    (:NewEnumerator1
      (Default|NoticeReceiverDamaged _wbp_play Message))
    (:NewEnumerator3
      (Default|NoticeMessage _wbp_play Message))))