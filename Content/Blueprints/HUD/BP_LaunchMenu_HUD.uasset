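; Launch menu HUD Blueprint that runs the startup screen sequence: MinhLo Studio intro, UE5 intro, splash, then home menu.
; BeginPlay shows the first widget, and each screen's event dispatcher triggers the next: ready-to-next-screen for both intros, Play pressed for the splash.
; Each later init function removes the previous widget only if valid, then creates, stores and adds its own to the viewport.
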(event Custom|OnAnimationComplete_Event
  (CallFunction|InitScreenIntroUE5)
  (EventDispatchers|AssignOnReadytoNextScreen (Variables|Default|GetWBP_IntroUE5) (delegate Custom|OnReadyToNextScreen_Event)))

(event Custom|OnReadyToNextScreen_Event
  (CallFunction|InitScreenSplash)
  (EventDispatchers|AssignOnButtonPlayPressed (Variables|Default|GetWBP_Splash) (delegate Custom|OnButtonPlayPressed_Event)))

(event Custom|OnButtonPlayPressed_Event
  (CallFunction|InitScreenHome))

(event EventBeginPlay
  (CallFunction|InitScreenIntroMinhLoStudio)
  (EventDispatchers|AssignOnReadytoNextScreen (Variables|Default|GetWBP_MinhLoStudioScreen) (delegate Custom|OnAnimationComplete_Event)))

(event Collision|EventActorBeginOverlap
  (params (OtherActor :type Actor%20Object%20Reference)))

(event EventTick
  (params (DeltaSeconds :type Float%20%28single-precision%29)))

(fn ConstructionScript)

(fn InitScreenIntroMinhLoStudio
  (bind _returnvalue (UserInterface|CreateWidget "/Game/UI/Screen/WBP_Intro_MinhLoStudio.WBP_Intro_MinhLoStudio_C"))
  (bind _output_get (Variables|Default|SetWBP_MinhLoStudioScreen _returnvalue))
  (UserInterface|Viewport|AddtoViewport _output_get 0))

(fn InitScreenIntroUE5
  (bind _wbp_minhlostudioscreen (Variables|Default|GetWBP_MinhLoStudioScreen)
    (:then
      (Widget|RemovefromParent _wbp_minhlostudioscreen)
      (bind _returnvalue (UserInterface|CreateWidget "/Game/UI/Screen/WBP_Intro_UE5.WBP_Intro_UE5_C"))
      (bind _output_get (Variables|Default|SetWBP_IntroUE5 _returnvalue))
      (UserInterface|Viewport|AddtoViewport _output_get 0))
    (:else)))

(fn InitScreenSplash
  (bind _wbp_introue5 (Variables|Default|GetWBP_IntroUE5)
    (:then
      (Widget|RemovefromParent _wbp_introue5)
      (bind _returnvalue (UserInterface|CreateWidget "/Game/UI/Screen/WBP_Splash.WBP_Splash_C"))
      (bind _output_get (Variables|Default|SetWBP_Splash _returnvalue))
      (UserInterface|Viewport|AddtoViewport _output_get 0))
    (:else)))

(fn InitScreenHome
  (bind _wbp_splash (Variables|Default|GetWBP_Splash)
    (:then
      (Widget|RemovefromParent _wbp_splash)
      (bind _returnvalue (UserInterface|CreateWidget "/Game/UI/Screen/WBP_Home.WBP_Home_C"))
      (bind _output_get (Variables|Default|SetWBP_Home _returnvalue))
      (UserInterface|Viewport|AddtoViewport _output_get 0))
    (:else)))